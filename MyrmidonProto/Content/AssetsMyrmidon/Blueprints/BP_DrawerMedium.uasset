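; Medium drawer interactable that slides between its start location and a rotation-relative end position, showing a sphere on hover.
; Authority-side StartB and EndB arm or cancel a delay timer that Tick counts down before movement starts.
; Tick derives alpha from current distance to the end, then lerps location.
; It either toggles to each limit or, in follow-mouse mode, takes direction from the player controller's screen-projected handle and look values.
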(event Custom|Direction
  (bind _returnvalue (Game|GetGameMode))
  (bind _asbp_game_mode (Utilities|Casting|CastToBP_GameMode _returnvalue))
  (bind _playercontroller (Default|GetPlayerController _asbp_game_mode false))
  (bind _lookatvalue (Variables|/Game/AssetsMyrmidon/Blueprints/BP_PlayerController.BP_PlayerController_C|GetLookAtValue _playercontroller))
  (bind _lookatvalue2 (Variables|/Game/AssetsMyrmidon/Blueprints/BP_PlayerController.BP_PlayerController_C|GetLookAtValue2 _playercontroller))
  (bind _returnvalue_2 (- _lookatvalue _lookatvalue2))
  (bind _returnvalue_3 (* _lookatvalue _returnvalue_2))
  (bind (_x _y) (Math|Vector2D|BreakVector2D _returnvalue_3))
  (bind _returnvalue_4 (+ _x _y))
  ;[1 1 1] Direction
  (Networking|SwitchHasAuthority
    (:Authority
      (Default|GetWorldtoScreenPos _playercontroller (+ (Math|Vector|RotateVector (Variables|Settings|GetHandlePosition) (Transformation|GetActorRotation)) (Transformation|GetActorLocation)) (Transformation|GetActorLocation))
      (if (not (Variables|/Game/AssetsMyrmidon/Blueprints/BP_PlayerController.BP_PlayerController_C|GetisPantin _playercontroller))
        (Variables|Default|SetGoingBack (> _returnvalue_4 0.0))
        (Variables|Default|SetMoveAllowed (> (Math|Float|Absolute(Float) _returnvalue_4) (Variables|Settings|GetMinimalPercentDistance)))))))

(event Custom|CheckTimerToStartMoving
  (params (DetaTime :type Float%20%28double-precision%29))
  ;[1 1 1] CheckTimerToStartMoving
  (if (and (not (Variables|Default|GetIsMoving)) (>= (Variables|Default|GetTimer) 0.0))
    (Variables|Default|SetTimer (- (Variables|Default|GetTimer) DetaTime))
    (if (<= (Variables|Default|GetTimer) 0.0)
      (Variables|Default|SetTimer -1.0)
      (Variables|Default|SetIsMoving true)
      (if (not (Variables|Settings|GetModeFollowMouse))
        (Variables|Default|SetGoingBack (not (Variables|Default|GetGoingBack)))))))

(event Custom|CustomEvent
  (params (DeltaSeconds :type Float%20%28single-precision%29))
  ;[1 1 1] EventTick
)

(event EventBeginPlay
  ;[1 1 1] BeginPlay
  (Networking|SwitchHasAuthority
    (:Authority
      (Variables|Default|SetInitialPosition (Transformation|GetActorLocation))
      (Variables|Default|SetWorldEndPos (+ (Math|Vector|RotateVector (Variables|Settings|GetEndPosition) (Transformation|GetActorRotation)) (Transformation|GetActorLocation))))))

(event EventStartHover
  ;[1 1 1] Hover
  (Rendering|SetVisibility (Variables|Default|GetSphere) true false))

(event EventEndHover
  ;[1 1 1] Hover
  (Rendering|SetVisibility (Variables|Default|GetSphere) false false))

(event EventTick
  (params (DeltaSeconds :type Float%20%28single-precision%29))
  (bind _returnvalue (Transformation|GetActorLocation))
  (bind _returnvalue_2 (* DeltaSeconds -1.0))
  (bind _worldendpos (Variables|Default|GetWorldEndPos))
  (bind _goingback (Variables|Default|GetGoingBack))
  (bind _initialposition (Variables|Default|GetInitialPosition))
  (bind _speed (Variables|Settings|GetSpeed))
  (bind _worldendpos_2 (Variables|Default|GetWorldEndPos))
  (bind _returnvalue_3 (Math|Vector|Distance(Vector) _returnvalue _worldendpos))
  (bind _returnvalue_4 (Math|Vector|Distance(Vector) _initialposition _worldendpos_2))
  (bind _returnvalue_5 (select _goingback _returnvalue_2 DeltaSeconds))
  (bind _returnvalue_6 (/ _returnvalue_3 _returnvalue_4))
  (bind _returnvalue_7 (* _returnvalue_5 _speed))
  (bind _returnvalue_8 (- 1.0 _returnvalue_6))
  (bind _returnvalue_9 (+ _returnvalue_7 _returnvalue_8))
  (bind _returnvalue_10 (Math|Float|Clamp(Float) _returnvalue_9))
  ;[1 1 1] EventTick
  (CallFunction|CheckTimertoStartMoving DeltaSeconds)
  (if (Variables|Default|GetIsMoving)
    (if (Variables|Settings|GetModeFollowMouse)
      (CallFunction|Direction))
    (if (Variables|Default|GetMoveAllowed)
      (Transformation|SetActorLocation (Math|Vector|Lerp(Vector) (Variables|Default|GetInitialPosition) (Variables|Default|GetWorldEndPos) _returnvalue_10) false false)
      (if (and (not (Variables|Settings|GetModeFollowMouse)) (Math|Float|NearlyEqual(Float) _returnvalue_10 (Math|Float|SelectFloat 0.0 1.0 (Variables|Default|GetGoingBack)) (Variables|Settings|GetMinimalPercentDistance)))
        (Variables|Default|SetIsMoving false)))))

(event EventStartB
  ;[1 1 1] Interaction
  (Networking|SwitchHasAuthority
    (:Authority
      (Variables|Default|SetTimer (Variables|Settings|GetDelayBeforeMovement)))))

(event EventEndB
  ;[1 1 1] Interaction
  (Networking|SwitchHasAuthority
    (:Authority
      (Variables|Default|SetTimer -1.0)
      (if (Variables|Settings|GetModeFollowMouse)
        (Variables|Default|SetIsMoving false)))))

(fn ConstructionScript
  (|CallParentFunction))