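; BP_Button is an interactable button that gives visual feedback on its AnimSphere mesh for hover and press-style events.
; Hover start and end toggle custom depth rendering on the sphere.
; StartB switches the sphere to a red material, and EndB restores the basic shape material and prints an on-screen debug message.
; A separate MulticastEndB event also restores the material, but nothing in this Blueprint calls it.
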(event Custom|MulticastEndB
  (Rendering|Material|SetMaterial (Variables|Default|GetAnimSphere) 0 "/Engine/BasicShapes/BasicShapeMaterial.BasicShapeMaterial"))

(event EventStartHover
  (Rendering|SetRenderCustomDepth (Variables|Default|GetAnimSphere) true))

(event EventEndHover
  (Rendering|SetRenderCustomDepth (Variables|Default|GetAnimSphere) false))

(event EventStartB
  (Rendering|Material|SetMaterial (Variables|Default|GetAnimSphere) 0 "/Game/AssetsMyrmidon/Art/Materials/M_Red.M_Red"))

(event EventEndB
  (Development|PrintString "ENDED" true true "(R=0.000000,G=0.660000,B=1.000000,A=1.000000)" 2e+01)
  (Rendering|Material|SetMaterial (Variables|Default|GetAnimSphere) 0 "/Engine/BasicShapes/BasicShapeMaterial.BasicShapeMaterial"))

(fn ConstructionScript
  (|CallParentFunction))