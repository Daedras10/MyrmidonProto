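; BP_NPC is an interactable, non-pickable level-design NPC that shows and hides floating text through its StartB and EndB events.
; While visible, the text turns every tick to face the local player's camera, using either the Pantin camera or the Animator's first-person camera.
; Aim events toggle the mesh's custom depth stencil as a highlight, only when the local player is not the Pantin.
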(event EventTick
  (params (DeltaSeconds :type Float%20%28single-precision%29))
  (bind _playercontroller (CallFunction|GetBPLocalPlayerController))
  (bind _textrender (Variables|Default|GetTextRender))
  (if (Variables|/Script/Engine.SceneComponent|GetbVisible (Variables|Default|GetTextRender))
    (if (Variables|/Game/AssetsMyrmidon/Blueprints/GameMode/BP_PlayerController.BP_PlayerController_C|GetisPantin _playercontroller)
      (Transformation|SetWorldRotation _textrender (Math|Rotator|FindLookatRotation (Transformation|GetWorldLocation (Variables|Default|GetTextRender)) (Transformation|GetWorldLocation (Variables|/Game/AssetsMyrmidon/Blueprints/Camera/BP_Camera.BP_Camera_C|GetCamera (Variables|/Game/AssetsMyrmidon/Blueprints/GameMode/BP_PlayerController.BP_PlayerController_C|GetCam _playercontroller)))) false false)
      (else
        (Transformation|SetWorldRotation _textrender (Math|Rotator|FindLookatRotation (Transformation|GetWorldLocation (Variables|Default|GetTextRender)) (Transformation|GetWorldLocation (Variables|/Game/AssetsMyrmidon/Blueprints/Character/BP_Animateur.BP_Animateur_C|GetFirstPersonCamera (Variables|/Game/AssetsMyrmidon/Blueprints/GameMode/BP_PlayerController.BP_PlayerController_C|GetBP_Animator _playercontroller)))) false false)))))

(event EventStartB
  (Rendering|SetVisibility (Variables|Default|GetTextRender) true false))

(event EventShowAim
  ;[1 1 1] Aim
  (if (not (Variables|/Game/AssetsMyrmidon/Blueprints/GameMode/BP_PlayerController.BP_PlayerController_C|GetisPantin (.PlayerController (CallFunction|GetBPLocalPlayerController))))
    (Rendering|SetCustomDepthStencilValue (Variables|Character|GetMesh) 1)))

(event EventHideAim
  ;[1 1 1] Aim
  (if (not (Variables|/Game/AssetsMyrmidon/Blueprints/GameMode/BP_PlayerController.BP_PlayerController_C|GetisPantin (.PlayerController (CallFunction|GetBPLocalPlayerController))))
    (Rendering|SetCustomDepthStencilValue (Variables|Character|GetMesh) 0)))

(event EventEndB
  (Rendering|SetVisibility (Variables|Default|GetTextRender) false false))

(fn ConstructionScript)

(fn GetCorkBoardIndex
  (return 0))

(fn GetCorkOffset
  (return 0.0))

(fn GetInputInfos
  (return false ""))

(fn GetInterractOffset
  (return "0, 0, 0"))

(fn GetInterractPoint
  (return (Transformation|GetActorLocation)))

(fn GetRectMargins
  (return "0, 0, 0"))

(fn IsInteractable
  (return true))

(fn IsPickable
  (return false))

(fn IsPicked
  (return false))

(fn PickableShouldLerp
  (return false))