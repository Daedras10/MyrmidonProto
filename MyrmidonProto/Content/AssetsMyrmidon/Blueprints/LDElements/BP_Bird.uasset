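; Level-design bird that resists wind while perched, then flies away along a spline if exposed too long.
; Three upwind line traces from the perch detect shelter; after hovering while the perch is unexposed, it flies back and lands.
; A tick-driven, server-authoritative state machine sets spline distance, applied every tick by Move.
; Timed child-actor height offsets handle takeoff and landing; a multicast material swap signals wind resistance.
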(event Custom|UpdateState
  (params (DetaTime :type Float%20%28double-precision%29))
  ;[1 1 1] UpdateState
  (Networking|SwitchHasAuthority
    (:Authority
      (switch Utilities|FlowControl|Switch|SwitchonEBirdAction (Variables|Default|GetCurrentAction)
        (:Idle
          (CallFunction|IdleUpdateState))
        (:FlyingAway
          (CallFunction|FlyingAwayState DetaTime))
        (:GoingBack
          (CallFunction|GoingBackState DetaTime))
        (:WaitingForSafeSpot
          (CallFunction|WaitingforSafeSpotSate))
        (:Hovering
          (CallFunction|HoveringState DetaTime))
        (:WindResistance
          (CallFunction|WindResistanceUpdateState DetaTime))))
    (:Remote
      _))
  (CallFunction|Move))

(event Custom|IdleUpdateState
  ;[1 1 1] IdleUpdateState
  (if (and (Variables|Default|GetWindIsActive) (Variables|Default|GetBaseIsexposed))
    (Variables|Default|SetCurrentAction "WindResistance")
    (Variables|Default|SetTimer (Variables|Default|GetWindResistanceTime))
    (CallFunction|ChangeApearanceMulticast 1)))

(event Custom|DisplayDebug
  ;[1 1 1] DisplayDebug
  (Rendering|SetVisibility (Variables|Default|GetTextRender) (Variables|Default|GetDebug) false))

(event Custom|ChangeApearanceMulticast
  (params (id :type Integer))
  ;[1 1 1] ChangeApearanceMulticast
  (Rendering|Material|SetMaterial (Variables|Default|GetSkeletalMesh) 0 (Utilities|Array|Get(acopy) (Variables|Default|GetMaterials) id)))

(event Custom|AnimationTick
  (params (DeltaTime :type Float%20%28double-precision%29))
  ;[1 1 1] AnimationTick
  (Variables|Default|SetAnimationTime (+ DeltaTime (Variables|Default|GetAnimationTime))))

(event Custom|UpdateValues
  ;[1 1 1] UpdateValues
  (if (Variables|Default|GetWindIsActive)
    (Variables|Default|SetBaseIsexposed false)
    (CallFunction|WindTrace 2e+02 0.0 "0.000000,90.000000,0.000000")
    (CallFunction|WindTrace 2e+02 -2e+01 "0.000000,90.000000,0.000000")
    (CallFunction|WindTrace 2e+02 2e+01 "0.000000,90.000000,0.000000")
    (else
      (Variables|Default|SetBaseIsexposed false))))

(event Custom|WaitingForSafeSpotSate
  ;[1 1 1] WaitingForSafeSpotSate
  (if (or (and (Variables|Default|GetWindIsActive) (not (Variables|Default|GetBaseIsexposed))) (not (Variables|Default|GetWindIsActive)))
    (Variables|Default|SetCurrentAction "GoingBack")
    (Variables|Default|SetAnimationTime 0.0)))

(event Custom|FlyingAwayState
  (params (DeltaTime :type Float%20%28double-precision%29))
  (bind _spline (Variables|Default|GetSpline))
  (bind _returnvalue (Spline|GetSplineLength _spline))
  ;[1 1 1] FlyingAwayState
  (bind _done (CallFunction|FlyingOffDone))
  (if _done
    (bind _output_get (Variables|Default|SetCurrentPosAlongSpline (Math|Float|Clamp(Float) (+ (* DeltaTime (Variables|Default|GetSpeed)) (Variables|Default|GetCurrentPosAlongSpline)) 0.0 _returnvalue)))
    (if (== _output_get _returnvalue)
      (Variables|Default|SetCurrentAction "Hovering")
      (Variables|Default|SetTimer (Variables|Default|GetHoverTime)))
    (else
      (CallFunction|AnimationTick DeltaTime))))

(event Custom|WindResistanceUpdateState
  (params (DeltaTime :type Float%20%28double-precision%29))
  ;[1 1 1] WindResistanceUpdateState
  (if (and (Variables|Default|GetWindIsActive) (Variables|Default|GetBaseIsexposed))
    (bind _output_get (Variables|Default|SetTimer (- (Variables|Default|GetTimer) DeltaTime)))
    (if (<= _output_get 0.0)
      (Variables|Default|SetCurrentAction "FlyingAway")
      (Variables|Default|SetAnimationTime 0.0)
      (Variables|Default|SetCurrentPosAlongSpline 0.0)
      (CallFunction|ChangeApearanceMulticast))
    (else
      (Variables|Default|SetCurrentAction "Idle")
      (CallFunction|ChangeApearanceMulticast))))

(event Custom|HoveringState
  (params (DeltaTime :type Float%20%28double-precision%29))
  ;[1 1 1] HoveringState
  (if (not (Variables|Default|GetBaseIsexposed))
    (bind _output_get (Variables|Default|SetTimer (- (Variables|Default|GetTimer) DeltaTime)))
    (if (<= _output_get 0.0)
      (Variables|Default|SetCurrentAction "GoingBack"))
    (else
      (Variables|Default|SetTimer (Variables|Default|GetHoverTime)))))

(event Custom|GoingBackState
  (params (DeltaTime :type Float%20%28double-precision%29))
  ;[1 1 1] GoingBackState
  (if (== 0.0 (Variables|Default|GetCurrentPosAlongSpline))
    (bind _done (CallFunction|LandingDone))
    (if _done
      (Variables|Default|SetCurrentAction "Idle")
      (else
        (CallFunction|AnimationTick DeltaTime)))
    (else
      (Variables|Default|SetCurrentPosAlongSpline (Math|Float|Clamp(Float) (- (Variables|Default|GetCurrentPosAlongSpline) (* DeltaTime (Variables|Default|GetSpeed))) 0.0 (Spline|GetSplineLength (Variables|Default|GetSpline)))))))

(event Custom|Move
  ;[1 1 1] Move
  (Transformation|SetWorldLocation (Variables|Default|GetBird) (Spline|GetLocationatDistanceAlongSpline (Variables|Default|GetSpline) (Variables|Default|GetCurrentPosAlongSpline) "World") false false))

(event Custom|CalculateCurrentAlpha
  ;[1 1 1] CalculateCurrentAlpha
  (Networking|SwitchHasAuthority
    (:Authority
      (Variables|Default|SetCurrentPosAlongSpline (Class|SplineComponent|GetDistanceAlongSplineatLocation (Variables|Default|GetSpline) (Transformation|GetWorldLocation (Variables|Default|GetBird)) "World")))))

(event Collision|EventActorBeginOverlap
  (params (OtherActor :type Actor%20Object%20Reference)))

(event EventTick
  (params (DeltaSeconds :type Float%20%28single-precision%29))
  ;[1 1 1] Event Tick
  (CallFunction|UpdateValues)
  (CallFunction|UpdateState DeltaSeconds)
  (Rendering|Components|TextRender|SetText (Variables|Default|GetTextRender) (Class|Bird|GetDebugText)))

(event EventSetActiveWind
  (params (bIsActive :type Boolean))
  ;[1 1 1] Wind
  (Variables|Default|SetWindIsActive bIsActive))

(event EventSetWindDirection
  (params (WindDirection :type Vector :default "0, 0, 0") (WindStrength :type Float%20%28single-precision%29))
  ;[1 1 1] Wind
  (Variables|Default|SetWindDirection (* WindDirection WindStrength)))

(event EventBeginPlay
  ;[1 1 1] BeginPlay
  (Variables|Default|SetIdleLocation (Transformation|GetWorldLocation (Variables|Default|GetBird)))
  (CallFunction|CalculateCurrentAlpha))

(fn ConstructionScript
  (CallFunction|DisplayDebug)
  (CallFunction|ChangeApearanceMulticast))

(fn WindTrace
  (params (Length :type Float%20%28double-precision%29) (DistFromCenter :type Float%20%28double-precision%29) (RotatorFromDistance :type Rotator :default "0.000000,90.000000,0.000000"))
  (bind _idlelocation (Variables|Default|GetIdleLocation))
  (bind _winddirection (Variables|Default|GetWindDirection))
  (bind _returnvalue (Math|Vector|RotateVector _winddirection RotatorFromDistance))
  (bind _returnvalue_2 (* _returnvalue DistFromCenter))
  (bind _returnvalue_3 (+ _idlelocation _returnvalue_2))
  (bind _outactors (Actor|GetAllActorswithInterface "/Script/MyrmidonProto.WindIgnored"))
  (bind _returnvalue_4 (Collision|LineTraceByChannel _returnvalue_3 (- _returnvalue_3 (* (Variables|Default|GetWindDirection) Length)) "TraceTypeQuery1" false _outactors (Variables|Default|GetBaseWindDebug) true "(R=0.000000,G=0.166656,B=1.000000,A=1.000000)" "(R=0.462745,G=0.000000,B=0.003922,A=1.000000)"))
  (if (not _returnvalue_4)
    (Variables|Default|SetBaseIsexposed true)))

(fn GetInterractPoint
  (return (Transformation|GetActorLocation)))

(fn GetInputInfos
  (return false ""))

(fn FlyingOffDone
  (bind _animationtime (Variables|Default|GetAnimationTime))
  (bind _flyingoff (Variables|Default|GetFlyingOff))
  (bind _framerate (Variables|Default|GetFrameRate))
  (bind _returnvalue (/ _flyingoff _framerate))
  (Transformation|SetRelativeLocation (Variables|Default|GetChildActor) (Math|Vector|MakeVector 0.0 0.0 (Math|Float|MapRangeClamped (/ _returnvalue _animationtime) 0.0 1.0 5e+01 1e+02)) false false)
  (return (>= _animationtime _returnvalue)))

(fn LandingDone
  (bind _animationtime (Variables|Default|GetAnimationTime))
  (bind _framerate (Variables|Default|GetFrameRate))
  (bind _landing (Variables|Default|GetLanding))
  (bind _returnvalue (/ _landing _framerate))
  (Transformation|SetRelativeLocation (Variables|Default|GetChildActor) (Math|Vector|MakeVector 0.0 0.0 (Math|Float|MapRangeClamped (- 1.0 (Math|Float|Clamp(Float) (/ _returnvalue _animationtime))) 0.0 1.0 5e+01 1e+02)) false false)
  (return (>= _animationtime _returnvalue)))