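; Networked movable platform that slides between two offsets, A and B, from its placed location.
; The server waits for at least two players, snaps it to its starting end, then passes origin and alpha through ReplicateInitialPos.
; Tick lerps position by a clamped alpha while IsMoving, which is not set here.
; Despite its name, a true TargetPosIsA drives the platform toward B.
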(event Custom|ReplicateInitialPos
  (params (Alpha :type Float%20%28double-precision%29) (InitialPos :type Vector))
  ;[1 1 1] ReplicateInitialPos
  (Variables|Default|SetInitialPos InitialPos)
  (bind _output_get (Variables|Default|SetCurrentPos Alpha))
  (if (Variables|Default|Getprint)
    (Development|PrintString (Utilities|String|ToString(Float) _output_get))
    (Development|PrintString (Utilities|String|ToString(Vector) (Math|Vector|Lerp(Vector) (+ (Variables|Default|GetInitialPos) (Variables|Default|GetPositionA)) (+ (Variables|Default|GetInitialPos) (Variables|Default|GetPositionB)) (Variables|Default|GetCurrentPos))) true true "(R=0.000000,G=0.660000,B=1.000000,A=1.000000)" 1e+01)
    (Development|PrintString (Utilities|String|ToString(Vector) (Variables|Default|GetInitialPos)) true true "(R=0.000000,G=0.660000,B=1.000000,A=1.000000)" 1e+01)
    (Development|PrintString (Utilities|String|ToString(Vector) (Variables|Default|GetPositionA)) true true "(R=0.000000,G=0.660000,B=1.000000,A=1.000000)" 1e+01)
    (Development|PrintString (Utilities|String|ToString(Vector) (Variables|Default|GetPositionB)) true true "(R=0.000000,G=0.660000,B=1.000000,A=1.000000)" 1e+01))
  (Transformation|SetActorLocation (Math|Vector|Lerp(Vector) (+ (Variables|Default|GetInitialPos) (Variables|Default|GetPositionA)) (+ (Variables|Default|GetInitialPos) (Variables|Default|GetPositionB)) (Variables|Default|GetCurrentPos)) false false))

(event EventTick
  (params (DeltaSeconds :type Float%20%28single-precision%29))
  (bind _initialpos (Variables|Default|GetInitialPos))
  (bind _speed (Variables|Default|GetSpeed))
  (bind _returnvalue (* DeltaSeconds _speed))
  ;[1 1 1] EventTick
  (if (Variables|Default|GetIsMoving)
    (if (Variables|Default|GetTargetPosIsA)
      (Variables|Default|SetCurrentPos (Math|Float|Clamp(Float) (+ (Variables|Default|GetCurrentPos) _returnvalue)))
      (else
        (Variables|Default|SetCurrentPos (Math|Float|Clamp(Float) (+ (Variables|Default|GetCurrentPos) (* _returnvalue -1.0))))))
    (if (Variables|Default|Getprint)
      (Development|PrintString (Utilities|String|ToString(Vector) (Math|Vector|Lerp(Vector) (+ _initialpos (Variables|Default|GetPositionA)) (+ _initialpos (Variables|Default|GetPositionB)) (Variables|Default|GetCurrentPos)))))
    (Transformation|SetActorLocation (Math|Vector|Lerp(Vector) (+ _initialpos (Variables|Default|GetPositionA)) (+ _initialpos (Variables|Default|GetPositionB)) (Variables|Default|GetCurrentPos)) false false)
    (if (Variables|Default|Getprint)
      (Development|PrintString (Utilities|String|ToString(Text) (Utilities|Text|FormatText "{alpha} => {deltatime} & {speed} ; {targetPos}" (Variables|Default|GetCurrentPos) DeltaSeconds (Variables|Default|GetSpeed) (Variables|Default|GetTargetPosIsA)))))))

(event EventBeginPlay
  ;[1 1 1] BeginPlay
  (Networking|SwitchHasAuthority
    (:Authority
      (Utilities|FlowControl|Delay 0.2 :!label _label)
      (bind _returnvalue (Class|GameModeBase|GetNumPlayers (Game|GetGameMode)))
      (if (>= _returnvalue 2)
        (Utilities|FlowControl|Delay 0.3)
        (if (not (Variables|Default|GethasInit))
          (Variables|Default|SethasInit true)
          (Variables|Default|SetInitialPos (Transformation|GetActorLocation))
          (if (Variables|Default|GetInitialPosIsA)
            (Transformation|SetActorLocation (+ (Transformation|GetActorLocation) (Variables|Default|GetPositionA)) false false)
            (Variables|Default|SetCurrentPos 0.0)
            (else
              (Transformation|SetActorLocation (+ (Transformation|GetActorLocation) (Variables|Default|GetPositionB)) false false)
              (Variables|Default|SetCurrentPos 1.0)))
          (Variables|Default|SetTargetPosIsA (not (Variables|Default|GetInitialPosIsA)))
          (CallFunction|ReplicateInitialPos (Variables|Default|GetCurrentPos) (Variables|Default|GetInitialPos)))
        (else
          (goto _label))))
    (:Remote
      (Utilities|FlowControl|Delay 0.3))))

(fn ConstructionScript)