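; BP_Mole is a level-design element with a Mole component placed at either a lower Start or a raised End position.
; The construction script scales the Sphere's height by MoleHeightMult, derives Start from that scale and puts End UpHeight above it.
; It then snaps Mole to the end chosen by StrartUp and copies that flag into GoingUp.
; The event graph contains no runtime movement logic.
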(event Custom|MoveToInitialPos
  ;[1 1 1] MoveToInitialPos
  (Transformation|SetRelativeLocation (Variables|Default|GetMole) (Math|Vector|SelectVector (Variables|/Script/Engine.SceneComponent|GetRelativeLocation (Variables|Default|GetEnd)) (Variables|/Script/Engine.SceneComponent|GetRelativeLocation (Variables|Default|GetStart)) (Variables|Default|GetStrartUp)) false false)
  (Variables|Default|SetGoingUp (Variables|Default|GetStrartUp)))

(event Custom|ElementsPosScale
  (bind _moleheightmult (Variables|Default|GetMoleHeightMult))
  (bind _returnvalue (Math|Vector|MakeVector 1.0 1.0 _moleheightmult))
  (bind _returnvalue_2 (* _returnvalue 1e+02))
  ;[1 1 1] ElementsPosScale
  (Transformation|SetRelativeScale3D (Variables|Default|GetSphere) _returnvalue)
  (Transformation|SetRelativeLocation (Variables|Default|GetStart) _returnvalue_2 false false)
  (Transformation|SetRelativeLocation (Variables|Default|GetEnd) (+ _returnvalue_2 (Math|Vector|MakeVector 0.0 0.0 (Variables|Default|GetUpHeight))) false false))

(event EventBeginPlay)

(event Collision|EventActorBeginOverlap
  (params (OtherActor :type Actor%20Object%20Reference)))

(event EventTick
  (params (DeltaSeconds :type Float%20%28single-precision%29)))

(fn ConstructionScript
  (CallFunction|ElementsPosScale)
  (CallFunction|MovetoInitialPos))