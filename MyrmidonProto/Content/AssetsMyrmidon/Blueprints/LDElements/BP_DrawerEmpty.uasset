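; BP_DrawerEmpty is a level-design drawer built from six cubes: bottom, depth panel and four walls, resized parametrically.
; ScaleContent sizes the cubes from DrawerScale and BordersScale, then PlaceContent offsets them to the box edges, with Depth setting the depth panel's height.
; PlaceHandle puts the handle on the front wall's outer face.
; The construction script only calls its parent, and nothing here calls ScaleContent or PlaceHandle.
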(event EventScaleContent
  (bind _drawerscale (Variables|Default|GetDrawerScale))
  (bind _bordersscale (Variables|Settings|GetBordersScale))
  (bind _drawerscale_2 (Variables|Default|GetDrawerScale))
  (bind _bordersscale_2 (Variables|Settings|GetBordersScale))
  (bind _drawerscale_3 (Variables|Default|GetDrawerScale))
  (bind _bordersscale_3 (Variables|Settings|GetBordersScale))
  (bind (_x _y _z) (Math|Vector|BreakVector _drawerscale_2))
  (bind (_x_2 _y_2) (Math|Vector|BreakVector _drawerscale_3))
  (bind (_x_3 _y_3 _z_2) (Math|Vector|BreakVector _drawerscale))
  (bind _returnvalue (Math|Vector|MakeVector _bordersscale_2 _y _z))
  (bind _returnvalue_2 (Math|Vector|MakeVector _x_2 _y_2 _bordersscale_3))
  (bind _returnvalue_3 (Math|Vector|MakeVector _x_3 _bordersscale _z_2))
  ;[1 1 1] Event Scale Content
  (Transformation|SetRelativeScale3D (Variables|Default|GetCubeBot) _returnvalue_2)
  (Transformation|SetRelativeScale3D (Variables|Default|GetCubeDepth) _returnvalue_2)
  (Transformation|SetRelativeScale3D (Variables|Default|GetCubeRight) _returnvalue_3)
  (Transformation|SetRelativeScale3D (Variables|Default|GetCubeLeft) _returnvalue_3)
  (Transformation|SetRelativeScale3D (Variables|Default|GetCubeBack) _returnvalue)
  (Transformation|SetRelativeScale3D (Variables|Default|GetCubeForward) _returnvalue)
  (CallFunction|PlaceContent))

(event EventPlaceHandle
  (bind _cubeforward (Variables|Default|GetCubeForward))
  ;[1 1 1] Place Handle
  (Transformation|SetRelativeLocation (Variables|Default|GetHandleParent) (+ (Variables|/Script/Engine.SceneComponent|GetRelativeLocation _cubeforward) (Math|Vector|MakeVector (* (.X (Math|Vector|BreakVector (Variables|/Script/Engine.SceneComponent|GetRelativeScale3D _cubeforward))) 5e+01) 0.0 0.0)) false false))

(event EventPlaceContent
  (bind _drawerscale (Variables|Default|GetDrawerScale))
  (bind _drawerscale_2 (Variables|Default|GetDrawerScale))
  (bind _drawerscale_3 (Variables|Default|GetDrawerScale))
  (bind _x (Math|Vector|BreakVector _drawerscale))
  (bind _z (Math|Vector|BreakVector _drawerscale_2))
  (bind _y (Math|Vector|BreakVector _drawerscale_3))
  (bind _returnvalue (* _x -5e+01))
  (bind _returnvalue_2 (* _z -5e+01))
  (bind _returnvalue_3 (* _y 5e+01))
  (bind _returnvalue_4 (Math|Vector|MakeVector _returnvalue 0.0 0.0))
  (bind _returnvalue_5 (Math|Vector|MakeVector 0.0 0.0 _returnvalue_2))
  (bind _returnvalue_6 (Math|Vector|MakeVector 0.0 _returnvalue_3 0.0))
  ;[1 1 1] Place Content
  (Transformation|SetRelativeLocation (Variables|Default|GetCubeBot) _returnvalue_5 false false)
  (Transformation|SetRelativeLocation (Variables|Default|GetCubeDepth) (* _returnvalue_5 (- 1.0 (Variables|Settings|GetDepth))) false false)
  (Transformation|SetRelativeLocation (Variables|Default|GetCubeRight) _returnvalue_6 false false)
  (Transformation|SetRelativeLocation (Variables|Default|GetCubeLeft) (* _returnvalue_6 -1.0) false false)
  (Transformation|SetRelativeLocation (Variables|Default|GetCubeBack) _returnvalue_4 false false)
  (Transformation|SetRelativeLocation (Variables|Default|GetCubeForward) (* _returnvalue_4 -1.0) false false))

(fn ConstructionScript
  (|CallParentFunction))