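; BP_WindPump is an interactable pump that blows directional wind through a box volume while a player pumps it.
; While the interaction is held, the server reads mouse or stick vertical input, and each reversal refreshes a short timer that keeps the wind active.
; Overlapping Windable actors receive wind direction and strength.
; Tick animates the handle, updates debug materials and syncs a spawned BP_WindFromPump effect.
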(event OnComponentBeginOverlap(Box)
  (params (OverlappedComponent :type Primitive%20Component%20Object%20Reference) (OtherActor :type Actor%20Object%20Reference) (OtherComp :type Primitive%20Component%20Object%20Reference) (OtherBodyIndex :type Integer) (bFromSweep :type Boolean) (SweepResult :type Hit%20Result%20Structure%20%28by%20ref%29))
  (bind (_aswindable _bsuccess) (Utilities|Casting|CastToWindable OtherActor))
  ;[1 1 1] BeginEndOverlap
  (if _bsuccess
    (Utilities|Array|AddUnique (Variables|Default|GetWindables) _aswindable)
    (if (or (Variables|Default|GetActivatedRep) (Variables|Default|GetActivated))
      (Class|Windable|SetActiveWind _aswindable true)
      (Class|Windable|SetWindDirection _aswindable (Math|Vector|Normalize (Variables|Default|GetWindDirection)) (Variables|Default|GetWindPower)))))

(event OnComponentEndOverlap(Box)
  (params (OverlappedComponent :type Primitive%20Component%20Object%20Reference) (OtherActor :type Actor%20Object%20Reference) (OtherComp :type Primitive%20Component%20Object%20Reference) (OtherBodyIndex :type Integer))
  (bind (_aswindable _bsuccess) (Utilities|Casting|CastToWindable OtherActor))
  ;[1 1 1] BeginEndOverlap
  (if _bsuccess
    (Utilities|Array|RemoveItem (Variables|Default|GetWindables) _aswindable)
    (Class|Windable|SetActiveWind _aswindable false)))

(event Custom|UpdateMouseUp
  (params (mouseUp :type Boolean))
  ;[1 1 1] UpdateMouseUp
  (Variables|Default|SetmouseUp mouseUp))

(event Custom|DebugWindChangeState
  ;[1 1 1] DebugWindChangeState
  (bind _output_get (Variables|Default|SetDebugModeActivated (not (Variables|Default|GetDebugModeActivated))))
  (bind _output_get_2 (Variables|Default|SetActivated _output_get))
  (Variables|Default|SetActivatedRep _output_get_2)
  (if _output_get_2
    (CallFunction|SetActive)
    (else
      (CallFunction|SetInactive))))

(event Custom|SetActive
  ;[1 1 1] SetActive
  (bind _output_get (Variables|Default|SetActivated true))
  (Variables|Default|SetActivatedRep _output_get)
  (for _array_element (Variables|Default|GetWindables)
    (Class|Windable|SetActiveWind _array_element true)
    (Class|Windable|SetWindDirection _array_element (Math|Vector|Normalize (Variables|Default|GetWindDirection)) (Variables|Default|GetWindPower))))

(event Custom|SetInactive
  ;[1 1 1] SetInactive
  (bind _output_get (Variables|Default|SetActivated false))
  (Variables|Default|SetActivatedRep _output_get)
  (for _array_element (Variables|Default|GetWindables)
    (Class|Windable|SetActiveWind _array_element false)))

(event Custom|ChangeActiveState
  ;[1 1 1] ChangeActiveState
  (if (Variables|Default|GetActivated)
    (CallFunction|SetInactive)
    (else
      (CallFunction|SetActive))))

(event Custom|Direction
  (bind _gamemode (CallFunction|GetBPGameMode))
  (bind _playercontroller (Default|GetBPPlayerController _gamemode false))
  (bind _lastinputswasgamepad (Variables|/Game/AssetsMyrmidon/Blueprints/GameMode/BP_PlayerController.BP_PlayerController_C|GetLastInputsWasGamepad _playercontroller))
  (bind _playermoveinputs (Variables|/Game/AssetsMyrmidon/Blueprints/GameMode/BP_PlayerController.BP_PlayerController_C|GetPlayerMoveInputs _playercontroller))
  (bind _playerlookinputs (Variables|/Game/AssetsMyrmidon/Blueprints/GameMode/BP_PlayerController.BP_PlayerController_C|GetPlayerLookInputs _playercontroller))
  (bind _y (Math|Vector2D|BreakVector2D _playerlookinputs))
  (bind _x (Math|Vector2D|BreakVector2D _playermoveinputs))
  (bind _returnvalue (not _lastinputswasgamepad))
  (bind _returnvalue_2 (* _x -1.0))
  (bind _returnvalue_3 (Math|Float|SelectFloat _y _returnvalue_2 _returnvalue))
  ;[1 1 1] Direction
  (Networking|SwitchHasAuthority
    (:Authority
      (if (Variables|Default|GetisPumping)
        (if (and (not (Math|Float|NearlyEqual(Float) _returnvalue_3 0.0 1e-06)) (!= (Variables|Default|GetmouseUp) (> _returnvalue_3 0.0)))
          (bind _output_get (Variables|Default|SetmouseUp (not (Variables|Default|GetmouseUp))))
          (CallFunction|UpdateMouseUp _output_get)
          (Variables|Default|SetWindTimer 1.0)
          (if (not (Variables|Default|GetActivated))
            (CallFunction|SetActive)))))))

(event Custom|DebugWindVisual
  (bind _m1 (Variables|Default|GetM1))
  (bind _m2 (Variables|Default|GetM2))
  (bind _activatedrep (Variables|Default|GetActivatedRep))
  (bind _returnvalue (select _activatedrep _m2 _m1))
  ;[1 1 1] DebugWind
  (Rendering|Material|SetMaterial (Variables|Default|GetCubeBase) 0 _returnvalue)
  (Rendering|Material|SetMaterial (Variables|Default|GetCubeBase1) 0 _returnvalue)
  (Rendering|Material|SetMaterial (Variables|Default|GetCubeBase2) 0 _returnvalue)
  (Rendering|Material|SetMaterial (Variables|Default|GetCubeBase3) 0 _returnvalue))

(event Custom|CheckForPlayer
  ;[1 1 1] CheckForPlayer
  (if (Variables|Default|GetActivated)
    (for _array_element (Variables|Default|GetWindables)
      (bind _asbp_pantin (Utilities|Casting|CastToBP_Pantin _array_element))
      (Class|Windable|SetActiveWind _asbp_pantin true)
      (Class|Windable|SetWindDirection _asbp_pantin (Math|Vector|Normalize (Variables|Default|GetWindDirection)) (Variables|Default|GetWindPower)))))

(event Custom|WindVFXTick
  ;[1 1 1] WindVFXTick
  (if (!= (Variables|Default|GetActivated) (Variables|/Game/AssetsMyrmidon/Blueprints/VFX/BP_WindFromPump.BP_WindFromPump_C|GetIsActive (Variables|Default|GetWindVFX)))
    (CallFunction|VFXClient (Variables|Default|GetActivated))))

(event Custom|VFXClient
  (params (Activated :type Boolean))
  (bind _windvfx (Variables|Default|GetWindVFX))
  (bind _windvfx_2 (Variables|Default|GetWindVFX))
  ;[1 1 1] WindVFXTick
  (Default|SetSize _windvfx (Variables|Default|GetWindBoxScale))
  (Default|SetDirection _windvfx (Variables|Default|GetWindDirection))
  (if Activated
    (Default|Activate _windvfx_2)
    (else
      (Default|Deactivate _windvfx_2))))

(event EventBeginPlay
  ;[1 1 1] BeginPlay
  (bind _returnvalue (Game|SpawnActorfromClass "/Game/AssetsMyrmidon/Blueprints/VFX/BP_WindFromPump.BP_WindFromPump_C" (Math|Transform|MakeTransform (Transformation|GetWorldLocation (Variables|Default|GetBox))) "Undefined" "MultiplyWithRoot" 0 0))
  (Variables|Default|SetWindVFX _returnvalue)
  (Utilities|FlowControl|Delay 0.1)
  (for _array_element (Collision|GetOverlappingActors (Variables|Default|GetBox) 0 :!class /Script/Engine.PrimitiveComponent)
    (bind _aswindable (Utilities|Casting|CastToWindable _array_element))
    (Utilities|Array|AddUnique (Variables|Default|GetWindables) _aswindable))
  (if (Variables|Default|GetActivated)
    (CallFunction|SetActive)
    (else
      (CallFunction|SetInactive))))

(event EventStartB
  ;[1 1 1] StartEnd B
  (Networking|SwitchHasAuthority
    (:Authority
      (Default|DisableMvLookatServer (Default|GetBPPlayerController (.GameMode (CallFunction|GetBPGameMode)) false))
      (Variables|Default|SetisPumping true))))

(event EventEndB
  ;[1 1 1] StartEnd B
  (Networking|SwitchHasAuthority
    (:Authority
      (Default|EnableMvLookatServer (Default|GetBPPlayerController (.GameMode (CallFunction|GetBPGameMode)) false))
      (Variables|Default|SetisPumping false))))

(event EventTick
  (params (DeltaSeconds :type Float%20%28single-precision%29))
  (bind _pivotcylinder (Variables|Default|GetPivotCylinder))
  ;[1 1 1] EventTick
  (CallFunction|DebugWindVisual)
  (Transformation|SetRelativeRotation _pivotcylinder (Math|Rotator|Lerp(Rotator) (Variables|/Script/Engine.SceneComponent|GetRelativeRotation _pivotcylinder) (Math|Rotator|SelectRotator "80.000000,0.000000,90.000000" "40.000000,0.000000,90.000000" (Variables|Default|GetmouseUp)) (* DeltaSeconds 8.0) true) false false)
  (CallFunction|Direction)
  (if (> (Variables|Default|GetWindTimer) 0.0)
    (Variables|Default|SetWindTimer (- (Variables|Default|GetWindTimer) DeltaSeconds))
    (elif (and (Variables|Default|GetActivated) (not (Variables|Default|GetDebugModeActivated)))
      (CallFunction|SetInactive)))
  (CallFunction|WindVFXTick))

(fn ConstructionScript
  (bind _box (Variables|Default|GetBox))
  (Transformation|SetRelativeLocation _box (+ (+ (Variables|/Script/Engine.SceneComponent|GetRelativeLocation (Variables|Default|GetCylinder)) (Variables|Default|GetWindBoxOffset)) (* "1.000000,0.000000,0.000000" (* (.X (Math|Vector|BreakVector (Variables|Default|GetWindBoxScale))) 5e+01))) false false)
  (Components|Box|SetBoxExtent _box (* (Variables|Default|GetWindBoxScale) 5e+01) true)
  (Transformation|SetActorRotation (Math|Rotator|FindLookatRotation (Math|Vector|MakeVector 0.0 0.0 0.0) (Variables|Default|GetWindDirection))))

(fn GetInterractPoint
  (return (Transformation|GetActorLocation)))

(fn GetInputInfos
  (return true (Utilities|Struct|MakeSTRUC_InputInfos true "Hold +" "Up and Down" "/Game/AssetsMyrmidon/Art/Textures/T_ButtonLT.T_ButtonLT" "/Game/AssetsMyrmidon/Art/Textures/T_StickL.T_StickL")))

(fn OnRepMouseUp
  (Development|PrintString "REP"))

(fn OnRepActivatedRep)