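; Wind-driven windmill level element whose four arm slots each carry a platform, a non-pickupable lateral bar, or nothing.
; Tick spins the rotor, easing speed up toward a maximum while wind is active and down to zero otherwise, and refreshes occluders on linked god rays.
; Four pivot points are reset to the actor's yaw so mounted objects stay upright.
; The construction script sizes the blades and sets each slot's visibility, collision and child actor.
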(event Custom|UpdateGodRays
  (for _array_element (Variables|Default|GetGodRaysToUpdate)
    (Default|UpdateOccluders _array_element)))

(event EventBeginPlay)

(event EventSetActiveWind
  (params (bIsActive :type Boolean))
  (Variables|Default|SetwindActive bIsActive))

(event EventTick
  (params (DeltaSeconds :type Float%20%28single-precision%29))
  (Variables|Default|SetAngle (+ (* DeltaSeconds (Variables|Default|GetSpeed)) (Variables|Default|GetAngle)))
  (CallFunction|SetAngles)
  (Variables|Default|SetSpeed (Math|Float|Clamp(Float) (Math|Float|SelectFloat (+ (Variables|Default|GetSpeed) (* DeltaSeconds (Variables|Default|GetAcceleration))) (- (Variables|Default|GetSpeed) (* DeltaSeconds (Variables|Default|GetDeceleration))) (Variables|Default|GetwindActive)) 0.0 (Variables|Default|GetSpeedMax)))
  (CallFunction|UpdateGodRays))

(fn ConstructionScript
  (bind _lenght (Variables|Default|GetLenght))
  (bind _returnvalue (Math|Vector|MakeVector 0.2 _lenght 2.0))
  (Transformation|SetRelativeScale3D (Variables|Default|GetPale) _returnvalue)
  (Transformation|SetRelativeScale3D (Variables|Default|GetPale2) _returnvalue)
  (CallFunction|SetAngles)
  (CallFunction|SetCollisions)
  (CallFunction|SetObjects))

(fn SetAngles
  (bind _returnvalue (Transformation|GetActorRotation))
  (bind _yaw (Math|Rotator|BreakRotator _returnvalue))
  (bind _returnvalue_2 (Math|Rotator|MakeRotator 0.0 0.0 _yaw))
  (Transformation|SetRelativeRotation (Variables|Default|GetCylinder) (Math|Rotator|MakeRotator 9e+01 (Variables|Default|GetAngle) 9e+01) false false)
  (Transformation|SetWorldRotation (Variables|Default|GetPoint1) _returnvalue_2 false false)
  (Transformation|SetWorldRotation (Variables|Default|GetPoint2) _returnvalue_2 false false)
  (Transformation|SetWorldRotation (Variables|Default|GetPoint3) _returnvalue_2 false false)
  (Transformation|SetWorldRotation (Variables|Default|GetPoint4) _returnvalue_2 false false))

(fn OnRepReplicatedAngle)

(fn SetObjects
  (bind _bp_lateralbar (Variables|Default|GetBP_LateralBar))
  (bind _bp_lateralbar1 (Variables|Default|GetBP_LateralBar1))
  (bind _bp_lateralbar2 (Variables|Default|GetBP_LateralBar2))
  (bind _bp_lateralbar3 (Variables|Default|GetBP_LateralBar3))
  (bind _childactor (Variables|/Script/Engine.ChildActorComponent|GetChildActor _bp_lateralbar3))
  (bind _childactor_2 (Variables|/Script/Engine.ChildActorComponent|GetChildActor _bp_lateralbar))
  (bind _childactor_3 (Variables|/Script/Engine.ChildActorComponent|GetChildActor _bp_lateralbar1))
  (bind _childactor_4 (Variables|/Script/Engine.ChildActorComponent|GetChildActor _bp_lateralbar2))
  (bind _asbp_lateral_bar (Utilities|Casting|CastToBP_LateralBar _childactor))
  (bind _asbp_lateral_bar_2 (Utilities|Casting|CastToBP_LateralBar _childactor_2))
  (bind _asbp_lateral_bar_3 (Utilities|Casting|CastToBP_LateralBar _childactor_3))
  (bind _asbp_lateral_bar_4 (Utilities|Casting|CastToBP_LateralBar _childactor_4))
  (Utilities|FlowControl|Sequence
    (:then_0
      (Rendering|SetVisibility (Variables|Default|GetPlatform1) false false)
      (Rendering|SetVisibility (Variables|Default|GetBP_LateralBar) false false)
      (switch Utilities|FlowControl|Switch|SwitchonE_WindmillObjects (Utilities|Array|Get(acopy) (Variables|Default|GetObjects))
        (:NewEnumerator1
          (Rendering|SetVisibility (Variables|Default|GetPlatform1) true false))
        (:NewEnumerator2
          (Rendering|SetVisibility _bp_lateralbar true false)
          (Variables|/Script/MyrmidonProto.InteractableBase|SetIsPickupable _asbp_lateral_bar_2 false)
          (Variables|/Script/MyrmidonProto.InteractableBase|SetbIsInteractable _asbp_lateral_bar_2 false)
          (Variables|/Game/AssetsMyrmidon/Blueprints/LDElements/BP_LateralBar.BP_LateralBar_C|SetUsePantinMesh _asbp_lateral_bar_2 false))))
    (:then_1
      (Rendering|SetVisibility (Variables|Default|GetPlatform2) false false)
      (Rendering|SetVisibility (Variables|Default|GetBP_LateralBar1) false false)
      (switch Utilities|FlowControl|Switch|SwitchonE_WindmillObjects (Utilities|Array|Get(acopy) (Variables|Default|GetObjects) 1)
        (:NewEnumerator1
          (Rendering|SetVisibility (Variables|Default|GetPlatform2) true false))
        (:NewEnumerator2
          (Rendering|SetVisibility _bp_lateralbar1 true false)
          (Variables|/Script/MyrmidonProto.InteractableBase|SetIsPickupable _asbp_lateral_bar_3 false)
          (Variables|/Script/MyrmidonProto.InteractableBase|SetbIsInteractable _asbp_lateral_bar_3 false)
          (Variables|/Game/AssetsMyrmidon/Blueprints/LDElements/BP_LateralBar.BP_LateralBar_C|SetUsePantinMesh _asbp_lateral_bar_3 false))))
    (:then_2
      (Rendering|SetVisibility (Variables|Default|GetPlatform3) false false)
      (Rendering|SetVisibility (Variables|Default|GetBP_LateralBar2) false false)
      (switch Utilities|FlowControl|Switch|SwitchonE_WindmillObjects (Utilities|Array|Get(acopy) (Variables|Default|GetObjects) 2)
        (:NewEnumerator1
          (Rendering|SetVisibility (Variables|Default|GetPlatform3) true false))
        (:NewEnumerator2
          (Rendering|SetVisibility _bp_lateralbar2 true false)
          (Variables|/Script/MyrmidonProto.InteractableBase|SetIsPickupable _asbp_lateral_bar_4 false)
          (Variables|/Script/MyrmidonProto.InteractableBase|SetbIsInteractable _asbp_lateral_bar_4 false)
          (Variables|/Game/AssetsMyrmidon/Blueprints/LDElements/BP_LateralBar.BP_LateralBar_C|SetUsePantinMesh _asbp_lateral_bar_4 false))))
    (:then_3
      (Rendering|SetVisibility (Variables|Default|GetPlatform4) false false)
      (Rendering|SetVisibility (Variables|Default|GetBP_LateralBar3) false false)
      (switch Utilities|FlowControl|Switch|SwitchonE_WindmillObjects (Utilities|Array|Get(acopy) (Variables|Default|GetObjects) 3)
        (:NewEnumerator1
          (Rendering|SetVisibility (Variables|Default|GetPlatform4) true false))
        (:NewEnumerator2
          (Rendering|SetVisibility _bp_lateralbar3 true false)
          (Variables|/Script/MyrmidonProto.InteractableBase|SetIsPickupable _asbp_lateral_bar false)
          (Variables|/Script/MyrmidonProto.InteractableBase|SetbIsInteractable _asbp_lateral_bar false)
          (Variables|/Game/AssetsMyrmidon/Blueprints/LDElements/BP_LateralBar.BP_LateralBar_C|SetUsePantinMesh _asbp_lateral_bar false))))))

(fn SetCollisions
  (Utilities|FlowControl|Sequence
    (:then_0
      (Collision|SetCollisionEnabled (Variables|Default|GetPlatform1) "NoCollision")
      (ChildActorComponent|SetChildActorClass (Variables|Default|GetBP_LateralBar) 0)
      (switch Utilities|FlowControl|Switch|SwitchonE_WindmillObjects (Utilities|Array|Get(acopy) (Variables|Default|GetObjects))
        (:NewEnumerator1
          (Collision|SetCollisionEnabled (Variables|Default|GetPlatform1) "QueryAndPhysics"))
        (:NewEnumerator2
          (ChildActorComponent|SetChildActorClass (Variables|Default|GetBP_LateralBar) "/Game/AssetsMyrmidon/Blueprints/LDElements/BP_LateralBar.BP_LateralBar_C"))))
    (:then_1
      (Collision|SetCollisionEnabled (Variables|Default|GetPlatform2) "NoCollision")
      (ChildActorComponent|SetChildActorClass (Variables|Default|GetBP_LateralBar1) 0)
      (switch Utilities|FlowControl|Switch|SwitchonE_WindmillObjects (Utilities|Array|Get(acopy) (Variables|Default|GetObjects) 1)
        (:NewEnumerator1
          (Collision|SetCollisionEnabled (Variables|Default|GetPlatform2) "QueryAndPhysics"))
        (:NewEnumerator2
          (ChildActorComponent|SetChildActorClass (Variables|Default|GetBP_LateralBar1) "/Game/AssetsMyrmidon/Blueprints/LDElements/BP_LateralBar.BP_LateralBar_C"))))
    (:then_2
      (Collision|SetCollisionEnabled (Variables|Default|GetPlatform3) "NoCollision")
      (ChildActorComponent|SetChildActorClass (Variables|Default|GetBP_LateralBar2) 0)
      (switch Utilities|FlowControl|Switch|SwitchonE_WindmillObjects (Utilities|Array|Get(acopy) (Variables|Default|GetObjects) 2)
        (:NewEnumerator1
          (Collision|SetCollisionEnabled (Variables|Default|GetPlatform3) "QueryAndPhysics"))
        (:NewEnumerator2
          (ChildActorComponent|SetChildActorClass (Variables|Default|GetBP_LateralBar2) "/Game/AssetsMyrmidon/Blueprints/LDElements/BP_LateralBar.BP_LateralBar_C"))))
    (:then_3
      (Collision|SetCollisionEnabled (Variables|Default|GetPlatform4) "NoCollision")
      (ChildActorComponent|SetChildActorClass (Variables|Default|GetBP_LateralBar3) 0)
      (switch Utilities|FlowControl|Switch|SwitchonE_WindmillObjects (Utilities|Array|Get(acopy) (Variables|Default|GetObjects) 3)
        (:NewEnumerator1
          (Collision|SetCollisionEnabled (Variables|Default|GetPlatform4) "QueryAndPhysics"))
        (:NewEnumerator2
          (ChildActorComponent|SetChildActorClass (Variables|Default|GetBP_LateralBar3) "/Game/AssetsMyrmidon/Blueprints/LDElements/BP_LateralBar.BP_LateralBar_C"))))))

(fn SetActiveOutsideTriger
  (return false))