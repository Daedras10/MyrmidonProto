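; BP_MovablePlatformButton is a level-design button that starts and stops a referenced movable platform.
; On activation it passes its GoToA flag to the platform as the travel direction and sets it moving; on deactivation it halts the platform.
; Both handlers act only if the platform reference is valid, and the button only sets state on the platform, containing no movement logic itself.
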(event EventTick
  (params (DeltaSeconds :type Float%20%28single-precision%29))
  (|CallParentFunction DeltaSeconds) ; This node is disabled and will not be called.\nDrag off pins to build functionality.
)

(event EventButtonActive)

(event EventOnButtonActivated
  (bind _movableplatform (Variables|Default|GetMovablePlatform))
  (Utilities|IsValid _movableplatform
    (:Is%20Valid
      (Variables|/Game/AssetsMyrmidon/Blueprints/LDElements/BP_MovablePlatform.BP_MovablePlatform_C|SetTargetPosIsA _movableplatform (Variables|Default|GetGoToA))
      (Variables|/Game/AssetsMyrmidon/Blueprints/LDElements/BP_MovablePlatform.BP_MovablePlatform_C|SetIsMoving (Variables|Default|GetMovablePlatform) true))))

(event EventOnButtonDeactivated
  (Utilities|IsValid (Variables|Default|GetMovablePlatform)
    (:Is%20Valid
      (Variables|/Game/AssetsMyrmidon/Blueprints/LDElements/BP_MovablePlatform.BP_MovablePlatform_C|SetIsMoving (Variables|Default|GetMovablePlatform) false))))

(fn ConstructionScript
  (|CallParentFunction))