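; Pushable item box that BP_Pantin characters push or pull, and that OpenBox replaces with a pickupable lateral bar or destroying platform.
; Four side triggers set the push axis; Tick moves box and Pantin together from input using swept moves.
; A downward trace detects lost ground, enabling physics and removing the triggers.
; Secret boxes register with the game mode, report found upon falling, then self-destroy after a delay.
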(event OnComponentBeginOverlap(YPosBox)
  (params (OverlappedComponent :type Primitive%20Component%20Object%20Reference) (OtherActor :type Actor%20Object%20Reference) (OtherComp :type Primitive%20Component%20Object%20Reference) (OtherBodyIndex :type Integer) (bFromSweep :type Boolean) (SweepResult :type Hit%20Result%20Structure%20%28by%20ref%29))
  ;[1 1 1] Trigger Enter / Exit
  (bind _asbp_pantin (Utilities|Casting|CastToBP_Pantin OtherActor))
  (CallFunction|Setup _asbp_pantin "0.000000,-1.000000,0.000000"))

(event OnComponentBeginOverlap(YNegBox)
  (params (OverlappedComponent :type Primitive%20Component%20Object%20Reference) (OtherActor :type Actor%20Object%20Reference) (OtherComp :type Primitive%20Component%20Object%20Reference) (OtherBodyIndex :type Integer) (bFromSweep :type Boolean) (SweepResult :type Hit%20Result%20Structure%20%28by%20ref%29))
  ;[1 1 1] Trigger Enter / Exit
  (bind _asbp_pantin (Utilities|Casting|CastToBP_Pantin OtherActor))
  (CallFunction|Setup _asbp_pantin "0.000000,1.000000,0.000000"))

(event OnComponentBeginOverlap(XNegBox)
  (params (OverlappedComponent :type Primitive%20Component%20Object%20Reference) (OtherActor :type Actor%20Object%20Reference) (OtherComp :type Primitive%20Component%20Object%20Reference) (OtherBodyIndex :type Integer) (bFromSweep :type Boolean) (SweepResult :type Hit%20Result%20Structure%20%28by%20ref%29))
  ;[1 1 1] Trigger Enter / Exit
  (bind _asbp_pantin (Utilities|Casting|CastToBP_Pantin OtherActor))
  (CallFunction|Setup _asbp_pantin "1.000000,0.000000,0.000000"))

(event OnComponentBeginOverlap(XPosBox)
  (params (OverlappedComponent :type Primitive%20Component%20Object%20Reference) (OtherActor :type Actor%20Object%20Reference) (OtherComp :type Primitive%20Component%20Object%20Reference) (OtherBodyIndex :type Integer) (bFromSweep :type Boolean) (SweepResult :type Hit%20Result%20Structure%20%28by%20ref%29))
  ;[1 1 1] Trigger Enter / Exit
  (bind _asbp_pantin (Utilities|Casting|CastToBP_Pantin OtherActor))
  (CallFunction|Setup _asbp_pantin "-1.000000,0.000000,0.000000"))

(event OnComponentEndOverlap(YPosBox)
  (params (OverlappedComponent :type Primitive%20Component%20Object%20Reference) (OtherActor :type Actor%20Object%20Reference) (OtherComp :type Primitive%20Component%20Object%20Reference) (OtherBodyIndex :type Integer))
  ;[1 1 1] Trigger Enter / Exit
  (bind _asbp_pantin (Utilities|Casting|CastToBP_Pantin OtherActor))
  (Variables|/Game/AssetsMyrmidon/Blueprints/Character/BP_Pantin.BP_Pantin_C|SetPushable _asbp_pantin 0)
  (CallFunction|FinishInteracting))

(event OnComponentEndOverlap(YNegBox)
  (params (OverlappedComponent :type Primitive%20Component%20Object%20Reference) (OtherActor :type Actor%20Object%20Reference) (OtherComp :type Primitive%20Component%20Object%20Reference) (OtherBodyIndex :type Integer))
  ;[1 1 1] Trigger Enter / Exit
  (bind _asbp_pantin (Utilities|Casting|CastToBP_Pantin OtherActor))
  (Variables|/Game/AssetsMyrmidon/Blueprints/Character/BP_Pantin.BP_Pantin_C|SetPushable _asbp_pantin 0)
  (CallFunction|FinishInteracting))

(event OnComponentEndOverlap(XNegBox)
  (params (OverlappedComponent :type Primitive%20Component%20Object%20Reference) (OtherActor :type Actor%20Object%20Reference) (OtherComp :type Primitive%20Component%20Object%20Reference) (OtherBodyIndex :type Integer))
  ;[1 1 1] Trigger Enter / Exit
  (bind _asbp_pantin (Utilities|Casting|CastToBP_Pantin OtherActor))
  (Variables|/Game/AssetsMyrmidon/Blueprints/Character/BP_Pantin.BP_Pantin_C|SetPushable _asbp_pantin 0)
  (CallFunction|FinishInteracting))

(event OnComponentEndOverlap(XPosBox)
  (params (OverlappedComponent :type Primitive%20Component%20Object%20Reference) (OtherActor :type Actor%20Object%20Reference) (OtherComp :type Primitive%20Component%20Object%20Reference) (OtherBodyIndex :type Integer))
  ;[1 1 1] Trigger Enter / Exit
  (bind _asbp_pantin (Utilities|Casting|CastToBP_Pantin OtherActor))
  (Variables|/Game/AssetsMyrmidon/Blueprints/Character/BP_Pantin.BP_Pantin_C|SetPushable _asbp_pantin 0)
  (CallFunction|FinishInteracting))

(event Custom|OpenBox
  (params (corkId :type Integer))
  (bind _returnvalue (Transformation|GetActorTransform))
  (bind (_location _rotation) (Math|Transform|BreakTransform _returnvalue))
  ;[1 1 1] OpenBox
  (Networking|SwitchHasAuthority
    (:Authority
      (bind _returnvalue_2 (Game|SpawnActorfromClass (Variables|Default|GetItemClass) (Math|Transform|MakeTransform _location (Math|Rotator|MakeRotator 0.0 0.0 (.Yaw (Math|Rotator|BreakRotator _rotation)))) "Undefined" "MultiplyWithRoot" 0 0))
      (Utilities|FlowControl|Sequence
        (:then_0
          (bind _asbp_lateral_bar (Utilities|Casting|CastToBP_LateralBar _returnvalue_2))
          (bind _output_get (Variables|/Game/AssetsMyrmidon/Blueprints/LDElements/BP_LateralBar.BP_LateralBar_C|SetBoardIndex _asbp_lateral_bar corkId))
          (Default|ChangeCorkIndex _asbp_lateral_bar _output_get)
          (Variables|/Script/MyrmidonProto.InteractableBase|SetIsPickupable _asbp_lateral_bar true)
          (Default|Spawned _asbp_lateral_bar))
        (:then_1
          (bind _asbp_destroying_platform (Utilities|Casting|CastToBP_DestroyingPlatform _returnvalue_2))
          (bind _output_get_2 (Variables|/Game/AssetsMyrmidon/Blueprints/LDElements/BP_DestroyingPlatform.BP_DestroyingPlatform_C|SetBoardIndex _asbp_destroying_platform corkId))
          (Default|ChangeCorkIndex _asbp_destroying_platform _output_get_2)
          (Variables|/Script/MyrmidonProto.InteractableBase|SetIsPickupable _asbp_destroying_platform true)
          (Default|Spawned _asbp_destroying_platform))
        (:then_2
          (Actor|DestroyActor :!label _label))))
    (:Remote
      (goto _label))))

(event Custom|CheckFalling
  (bind _returnvalue (Transformation|GetActorLocation))
  ;[1 1 1] CheckFalling
  (bind _returnvalue_2 (Collision|LineTraceByChannel _returnvalue (+ _returnvalue "0.000000,0.000000,-120.000000") "TraceTypeQuery1" false 0 "None"))
  (if (not _returnvalue_2)
    (Physics|SetSimulatePhysics (Variables|Default|GetCube) true)
    (Variables|Default|SetisPhysics true)
    (CallFunction|CheckSecret)
    (CallFunction|FinishInteracting)
    (CallFunction|RemoveBoxes)))

(event Custom|FinishInteracting
  ;[1 1 1] FinishInteracting
  (Variables|Default|SetisPhysics true)
  (Variables|Default|SetisPantinInRange false)
  (Variables|Default|SetisPantinInterracting false)
  (Utilities|IsValid (Variables|Default|GetPantin)
    (:Is%20Valid
      (Default|OrientRotationtoMovement (Variables|Default|GetPantin) true)
      (Variables|/Game/AssetsMyrmidon/Blueprints/Character/BP_Pantin.BP_Pantin_C|SetisPushing (Variables|Default|GetPantin) false)
      (Variables|/Game/AssetsMyrmidon/Blueprints/Character/BP_Pantin.BP_Pantin_C|SetisPulling (Variables|Default|GetPantin) false)
      (Variables|Default|SetPantin 0)
      (Development|PrintString "FinishInteracting" false false))))

(event Custom|Setup
  (params (Pantin :type BP%20Pantin%20Object%20Reference) (Direction :type Vector))
  ;[1 1 1] Setup
  (Networking|SwitchHasAuthority
    (:Authority
      _)
    (:Remote
      _))
  (bind _output_get (Variables|Default|SetPantin Pantin))
  (Variables|/Game/AssetsMyrmidon/Blueprints/Character/BP_Pantin.BP_Pantin_C|SetPushable _output_get self)
  (Variables|Default|SetPushDirection Direction)
  (Variables|Default|SetisPantinInRange true)
  (Variables|Default|SetisPantinInterracting (Variables|/Game/AssetsMyrmidon/Blueprints/Character/BP_Pantin.BP_Pantin_C|GetPushInterract (Variables|Default|GetPantin)))
  (Default|OrientRotationtoMovement (Variables|Default|GetPantin) (not (Variables|/Game/AssetsMyrmidon/Blueprints/Character/BP_Pantin.BP_Pantin_C|GetPushInterract (Variables|Default|GetPantin))))
  (if (Variables|/Game/AssetsMyrmidon/Blueprints/Character/BP_Pantin.BP_Pantin_C|GetPushInterract (Variables|Default|GetPantin))
    (Transformation|SetActorRotation (Variables|Default|GetPantin) (Math|Rotator|FindLookatRotation (Math|Vector|MakeVector 0.0 0.0 0.0) (Math|Transform|TransformDirection (Transformation|GetActorTransform) (Variables|Default|GetPushDirection))))
    (Variables|Default|SetcanPull true)
    (Development|PrintString "SETUP" false false)))

(event Custom|CheckSecret
  ;[1 1 1] CheckSecret
  (if (Math|Boolean|ANDBoolean (Ability|HasAuthority) (Variables|Default|GetIsSecret) (not (Variables|Default|GetWasObtained)))
    (Variables|Default|SetWasObtained true)
    (Default|ReportNewSecretFound (.GameMode (CallFunction|GetBPGameMode)))
    (Utilities|FlowControl|Delay (Variables|Default|GetTimeBeforeSecretIsDestroyed))
    (Actor|DestroyActor)))

(event Custom|RemoveBoxes
  ;[1 1 1] RemoveBoxes
  (Utilities|FlowControl|DoOnce false
    (:Completed
      (Components|DestroyComponent (Variables|Default|GetYNegBox))
      (Components|DestroyComponent (Variables|Default|GetXNegBox))
      (Components|DestroyComponent (Variables|Default|GetXPosBox))
      (Components|DestroyComponent (Variables|Default|GetYPosBox)))))

(event EventTick
  (params (DeltaSeconds :type Float%20%28single-precision%29))
  (bind _returnvalue (Transformation|GetActorLocation))
  (bind _returnvalue_2 (Transformation|GetActorTransform))
  (bind _pushdirection (Variables|Default|GetPushDirection))
  (bind _pantin (Variables|Default|GetPantin))
  (bind _pantin_2 (Variables|Default|GetPantin))
  (bind _distancepantin (Variables|Default|GetDistancePantin))
  (bind _pantin_3 (Variables|Default|GetPantin))
  (bind _pushspeed (Variables|Default|GetPushSpeed))
  (bind _pantin_4 (Variables|Default|GetPantin))
  (bind _pushdirection_2 (Variables|Default|GetPushDirection))
  (bind _returnvalue_3 (Math|Transform|TransformDirection _returnvalue_2 _pushdirection_2))
  (bind _returnvalue_4 (* _pushdirection _distancepantin))
  (bind _returnvalue_5 (* _pushspeed DeltaSeconds))
  (bind _inputvector (Variables|/Game/AssetsMyrmidon/Blueprints/Character/BP_Pantin.BP_Pantin_C|GetInputVector _pantin_4))
  (bind _returnvalue_6 (Math|Vector|Normalize _inputvector))
  (bind _returnvalue_7 (Math|Vector|DotProduct _returnvalue_6 _returnvalue_3))
  (bind _returnvalue_8 (> _returnvalue_7 0.0))
  (bind _returnvalue_9 (Math|Float|SelectFloat 1.0 -1.0 _returnvalue_8))
  (bind _returnvalue_10 (* _returnvalue_9 _returnvalue_5))
  (bind _returnvalue_11 (* _returnvalue_10 _pushdirection))
  (bind _returnvalue_12 (+ _returnvalue_11 _returnvalue))
  (bind _returnvalue_13 (+ _returnvalue_12 _returnvalue_4))
  (bind (_x _y) (Math|Vector|BreakVector _returnvalue_13))
  ;[1 1 1] Event Tick
  (if (not (Variables|Default|GetisPhysics))
    (Networking|SwitchHasAuthority
      (:Authority
        _)
      (:Remote
        _))
    (CallFunction|CheckFalling)
    (Utilities|IsValid (Variables|Default|GetPantin)
      (:Is%20Valid
        (if (Variables|Default|GetisPantinInterracting)
          (if (or (Variables|Default|GetcanPull) _returnvalue_8)
            (if (> (Math|Float|Absolute(Float) _returnvalue_7) 0.2)
              (Networking|SwitchHasAuthority
                (:Authority
                  (bind _output_get (Variables|/Game/AssetsMyrmidon/Blueprints/Character/BP_Pantin.BP_Pantin_C|SetisPushing _pantin_2 _returnvalue_8))
                  (Variables|/Game/AssetsMyrmidon/Blueprints/Character/BP_Pantin.BP_Pantin_C|SetisPulling _pantin_2 (not _output_get)))
                (:Remote
                  _))
              (bind _sweephitresult (Transformation|SetActorLocation _returnvalue_12 true false))
              (if (and (.bBlockingHit (Collision|BreakHitResult _sweephitresult)) (== (.HitActor (Collision|BreakHitResult _sweephitresult)) (Variables|Default|GetPantin)))
                (Transformation|SetActorLocation _returnvalue_12 false false))
              (Utilities|IsValid _pantin_3
                (:Is%20Valid
                  (bind _sweephitresult_2 (Transformation|SetActorLocation _pantin_3 (Math|Vector|MakeVector _x _y (.Z (Math|Vector|BreakVector (Transformation|GetActorLocation (Variables|Default|GetPantin))))) true false))
                  (Variables|Default|SetcanPull (not (.bBlockingHit (Collision|BreakHitResult _sweephitresult_2))))
                  (if (Variables|/Game/AssetsMyrmidon/Blueprints/Character/BP_Pantin.BP_Pantin_C|GetIsFalling (Variables|Default|GetPantin))
                    (CallFunction|FinishInteracting))))
              (else
                (Networking|SwitchHasAuthority
                  (:Authority
                    (Variables|/Game/AssetsMyrmidon/Blueprints/Character/BP_Pantin.BP_Pantin_C|SetisPushing _pantin false)
                    (Variables|/Game/AssetsMyrmidon/Blueprints/Character/BP_Pantin.BP_Pantin_C|SetisPulling _pantin false)))))))))))

(event EventBeginPlay
  ;[1 1 1] BeginPlay
  (Networking|SwitchHasAuthority
    (:Authority
      (if (Variables|Default|GetIsSecret)
        (Default|ReportNewSecret (.GameMode (CallFunction|GetBPGameMode)))))))

(fn ConstructionScript)