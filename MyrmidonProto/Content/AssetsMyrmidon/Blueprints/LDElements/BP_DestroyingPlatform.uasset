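; Pickable platform that crumbles after the Pantin steps on it, then becomes solid again after a delay.
; Tick runs disappear and respawn timers, paused while picked, that toggle Pawn collision and the trigger box.
; The Pantin view drives ABP_FallingPlatform and spawns debris on collapse, while the other view rotates AnimFalling by timeline.
; The construction script sizes meshes, trigger and god-ray occluder, which drops away on collapse.
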(event OnComponentBeginOverlap(Box)
  (params (OverlappedComponent :type Primitive%20Component%20Object%20Reference) (OtherActor :type Actor%20Object%20Reference) (OtherComp :type Primitive%20Component%20Object%20Reference) (OtherBodyIndex :type Integer) (bFromSweep :type Boolean) (SweepResult :type Hit%20Result%20Structure%20%28by%20ref%29))
  ;[1 1 1] Overlap
  (bind _asbp_pantin (Utilities|Casting|CastToBP_Pantin OtherActor))
  (if (Math|Boolean|NORBoolean (Variables|Default|GetShouldDisapear) (Variables|Default|GetShouldRespawn))
    (Variables|Default|SetTimer (Variables|Default|GetDisapearDelay))
    (Variables|Default|SetShouldDisapear true)))

(event Custom|Spawned
  (params (UsePantinMesh :type Boolean))
  ;[1 1 1] Spawned
  (if (Variables|/Game/AssetsMyrmidon/Blueprints/GameMode/BP_PlayerController.BP_PlayerController_C|GetCurrentViewIsPantin (.PlayerController (CallFunction|GetBPLocalPlayerController)))
    (Rendering|SetVisibility (Variables|Default|GetScene) false true))
  (CallFunction|ShouldLerpMulticast))

(event Custom|Collisions
  (params (Active :type Boolean))
  (bind _returnvalue (select Active "ECR_Block" "ECR_Ignore"))
  (bind _pantin_fallingplatform (Variables|Default|GetPantin_FallingPlatform))
  ;[1 1 1] PickUp and Drop
  (Collision|SetCollisionResponsetoChannel (Variables|Default|GetAnimSphere) "ECC_Pawn" _returnvalue)
  (Collision|SetCollisionResponsetoChannel (Variables|Default|GetPantinCube) "ECC_Pawn" _returnvalue)
  (if (Variables|/Game/AssetsMyrmidon/Blueprints/GameMode/BP_PlayerController.BP_PlayerController_C|GetCurrentViewIsPantin (Variables|Default|GetPlayer%20Controller))
    (Rendering|SetVisibility _pantin_fallingplatform Active true)
    (Variables|Default|SetPlatformAnimBPREF (Components|SkeletalMesh|GetAnimInstance _pantin_fallingplatform))
    (else
      (Rendering|SetVisibility (Variables|Default|GetAnim_Falling) true true))))

(event Custom|UpdateGodRays
  ;[1 1 1] UpdateGodRays
  (for _array_element (Variables|Default|GetGodRaysToUpdate)
    (Default|UpdateOccluders _array_element)))

(event Custom|ShouldLerpMulticast
  ;[1 1 1] Spawned
  (Variables|Default|SetShouldLerp true))

(event Custom|PlaceGodRay
  (params (Active :type Boolean))
  (bind _childactor (Variables|Default|GetChildActor))
  ;[1 1 1] PlaceGodRay
  (Development|PrintString (Utilities|String|ToString(Boolean) Active) false false "(R=0.000000,G=0.660000,B=1.000000,A=1.000000)" 15.0)
  (Utilities|IsValid _childactor
    (:Is%20Valid
      (Transformation|SetRelativeLocation _childactor (Math|Vector|SelectVector (Math|Vector|MakeVector 0.0 0.0 (- (* (.Z (Math|Vector|BreakVector (Variables|Default|GetPlatformScale))) 5e+01) (* (Variables|Default|GetZScaleOccluder) 5e+01))) (Math|Vector|MakeVector 0.0 0.0 -5e+03) Active) false false)
      (CallFunction|UpdateGodRays))))

(event Custom|DisablePlatform
  ;[1 1 1] Overlap
  (if (Math|Boolean|NORBoolean (Variables|Default|GetShouldDisapear) (Variables|Default|GetShouldRespawn))
    (Variables|Default|SetTimer (Variables|Default|GetDisapearDelay))
    (Variables|Default|SetShouldDisapear true)))

(event Custom|RotatePlatformAnim
  (params (shouldFall :type Boolean))
  (bind _anim_falling (Variables|Default|GetAnim_Falling))
  ;[1 1 1] Animation AnimView
  (if shouldFall
    (if (not (Variables|Default|GetisAnimPlaying))
      (Variables|Default|SetisAnimPlaying true)
      (bind _newtrack_0 (Timeline|Timeline PlayFromStart)
        (:Update
          (Transformation|SetRelativeRotation _anim_falling (Math|Rotator|Lerp(Rotator) "0.000000,90.000000,0.000000" "-90.000000,90.000000,0.000000" _newtrack_0) false false))
        (:Finished
          (Variables|Default|SetisAnimPlaying false :!label _label))))
    (elif (not (Variables|Default|GetisAnimPlaying))
      (Variables|Default|SetisAnimPlaying true)
      (bind _newtrack_0_2 (Timeline|Timeline_0 PlayFromStart)
        (:Update
          (Transformation|SetRelativeRotation _anim_falling (Math|Rotator|Lerp(Rotator) "0.000000,90.000000,0.000000" "-90.000000,90.000000,0.000000" _newtrack_0_2) false false))
        (:Finished
          (goto _label))))))

(event Custom|ChangeCorkIndex
  (params (id :type Integer))
  ;[1 1 1] ChangeCorkIndex
  (Variables|Default|SetBoardIndex id))

(event Custom|CustomEvent
  ;[1 1 1] Aim
  (if (not (Variables|/Game/AssetsMyrmidon/Blueprints/GameMode/BP_PlayerController.BP_PlayerController_C|GetisPantin (.PlayerController (CallFunction|GetBPLocalPlayerController))))
    (Rendering|SetCustomDepthStencilValue (Variables|Default|GetAnim_Falling) 1)))

(event Custom|CustomEvent_1
  ;[1 1 1] Aim
  (if (not (Variables|/Game/AssetsMyrmidon/Blueprints/GameMode/BP_PlayerController.BP_PlayerController_C|GetisPantin (.PlayerController (CallFunction|GetBPLocalPlayerController))))
    (Rendering|SetCustomDepthStencilValue (Variables|Default|GetAnim_Falling) 0)))

(event EventShowAim
  ;[1 1 1] Hovers
  (if (not (Variables|/Game/AssetsMyrmidon/Blueprints/GameMode/BP_PlayerController.BP_PlayerController_C|GetisPantin (.PlayerController (CallFunction|GetBPLocalPlayerController))))
    (Rendering|SetCustomDepthStencilValue (Variables|Default|GetAnim_Falling) 1)))

(event EventHideAim
  ;[1 1 1] Hovers
  (if (not (Variables|/Game/AssetsMyrmidon/Blueprints/GameMode/BP_PlayerController.BP_PlayerController_C|GetisPantin (.PlayerController (CallFunction|GetBPLocalPlayerController))))
    (Rendering|SetCustomDepthStencilValue (Variables|Default|GetAnim_Falling) 0)))

(event EventDrop
  ;[1 1 1] PickUp and Drop
  (CallFunction|Collisions true)
  (Variables|Default|SetPicked false))

(event EventEndHover
  ;[1 1 1] Hovers
)

(event EventSetPickableShouldLerp
  (params (bShouldLerp :type Boolean))
  ;[1 1 1] PlaceGodRay
  (Variables|Default|SetShouldLerp bShouldLerp))

(event EventBeginPlay
  (bind _pantin_fallingplatform (Variables|Default|GetPantin_FallingPlatform))
  (bind _anim_falling (Variables|Default|GetAnim_Falling))
  ;[1 1 1] BeginPlay
  (bind _output_get (Variables|Default|SetPlayer%20Controller (.PlayerController (CallFunction|GetBPLocalPlayerController))))
  (if (Rendering|IsVisible (Variables|Default|GetScene))
    (Rendering|SetVisibility _pantin_fallingplatform (Variables|/Game/AssetsMyrmidon/Blueprints/GameMode/BP_PlayerController.BP_PlayerController_C|GetCurrentViewIsPantin _output_get) true)
    (Rendering|SetVisibility _anim_falling (not (Variables|/Game/AssetsMyrmidon/Blueprints/GameMode/BP_PlayerController.BP_PlayerController_C|GetCurrentViewIsPantin _output_get)) true)
    (else
      (Rendering|SetVisibility _pantin_fallingplatform (not (Variables|/Game/AssetsMyrmidon/Blueprints/GameMode/BP_PlayerController.BP_PlayerController_C|GetCurrentViewIsPantin _output_get)) true)
      (Rendering|SetVisibility _anim_falling (not (not (Variables|/Game/AssetsMyrmidon/Blueprints/GameMode/BP_PlayerController.BP_PlayerController_C|GetCurrentViewIsPantin _output_get))) true))))

(event EventTick
  (params (DeltaSeconds :type Float%20%28single-precision%29))
  (bind _pantincube (Variables|Default|GetPantinCube))
  (bind _returnvalue (Transformation|GetWorldTransform _pantincube))
  (bind (_location _rotation) (Math|Transform|BreakTransform _returnvalue))
  ;[1 1 1] EventTick
  (if (not (Variables|Default|GetPicked))
    (if (or (Variables|Default|GetShouldRespawn) (Variables|Default|GetShouldDisapear))
      (Variables|Default|SetTimer (- (Variables|Default|GetTimer) DeltaSeconds))
      (if (Variables|Default|GetShouldDisapear)
        (if (<= (Variables|Default|GetTimer) 0.0)
          (if (Variables|/Game/AssetsMyrmidon/Blueprints/GameMode/BP_PlayerController.BP_PlayerController_C|GetCurrentViewIsPantin (Variables|Default|GetPlayer%20Controller))
            (bind _asabp_falling_platform (Utilities|Casting|CastToABP_FallingPlatform (Variables|Default|GetPlatformAnimBPREF)))
            (Variables|/Game/AssetsMyrmidon/Art/Meshs/GameDesignAsset/FallingPlatform/ABP_FallingPlatform.ABP_FallingPlatform_C|SetisFalling _asabp_falling_platform true)
            (else
              (CallFunction|RotatePlatformAnim true)))
          (Variables|Default|SetShouldRespawn true)
          (Variables|Default|SetShouldDisapear false)
          (Variables|Default|SetTimer (Variables|Default|GetRespawnDelay))
          (Collision|SetCollisionResponsetoChannel (Variables|Default|GetPantinCube) "ECC_Pawn" "ECR_Ignore")
          (Collision|SetCollisionResponsetoChannel (Variables|Default|GetAnimSphere) "ECC_Pawn" "ECR_Ignore")
          (Collision|SetCollisionEnabled (Variables|Default|GetBox) "NoCollision")
          (if (Variables|/Game/AssetsMyrmidon/Blueprints/GameMode/BP_PlayerController.BP_PlayerController_C|GetCurrentViewIsPantin (Variables|Default|GetPlayer%20Controller))
            (Game|SpawnActorfromClass "/Game/AssetsMyrmidon/Blueprints/VFX/BP_DestroyedPlatform.BP_DestroyedPlatform_C" (Math|Transform|MakeTransform _location _rotation "0.500000,0.500000,0.500000") "Undefined" "MultiplyWithRoot" 0 0))
          (CallFunction|PlaceGodRay false)
          (elif (Variables|/Game/AssetsMyrmidon/Blueprints/GameMode/BP_PlayerController.BP_PlayerController_C|GetCurrentViewIsPantin (Variables|Default|GetPlayer%20Controller))
            (bind _asabp_falling_platform_2 (Utilities|Casting|CastToABP_FallingPlatform (Variables|Default|GetPlatformAnimBPREF)))
            (Variables|/Game/AssetsMyrmidon/Art/Meshs/GameDesignAsset/FallingPlatform/ABP_FallingPlatform.ABP_FallingPlatform_C|SetisStepped _asabp_falling_platform_2 true)))
        (elif (<= (Variables|Default|GetTimer) 0.0)
          (if (Variables|/Game/AssetsMyrmidon/Blueprints/GameMode/BP_PlayerController.BP_PlayerController_C|GetCurrentViewIsPantin (Variables|Default|GetPlayer%20Controller))
            (bind _asabp_falling_platform_3 (Utilities|Casting|CastToABP_FallingPlatform (Variables|Default|GetPlatformAnimBPREF)))
            (Variables|/Game/AssetsMyrmidon/Art/Meshs/GameDesignAsset/FallingPlatform/ABP_FallingPlatform.ABP_FallingPlatform_C|SetisFalling _asabp_falling_platform_3 false)
            (Variables|/Game/AssetsMyrmidon/Art/Meshs/GameDesignAsset/FallingPlatform/ABP_FallingPlatform.ABP_FallingPlatform_C|SetisStepped _asabp_falling_platform_3 false)
            (else
              (CallFunction|RotatePlatformAnim false)))
          (Variables|Default|SetShouldRespawn false)
          (Collision|SetCollisionResponsetoChannel (Variables|Default|GetPantinCube) "ECC_Pawn" "ECR_Block")
          (Collision|SetCollisionResponsetoChannel (Variables|Default|GetAnimSphere) "ECC_Pawn" "ECR_Block")
          (Collision|SetCollisionEnabled (Variables|Default|GetBox) "QueryOnly"))))))

(event EventStartHover
  ;[1 1 1] Hovers
)

(event EventSwitchtoAnimator
  (Rendering|SetVisibility (Variables|Default|GetAnim_Falling) true false)
  (Rendering|SetVisibility (Variables|Default|GetPantin_FallingPlatform) false false))

(event EventSwitchtoPantin
  (Rendering|SetVisibility (Variables|Default|GetAnim_Falling) false false)
  (Rendering|SetVisibility (Variables|Default|GetPantin_FallingPlatform) true false))

(event EventPickUp
  ;[1 1 1] PickUp and Drop
  (CallFunction|Collisions false)
  (Variables|Default|SetPicked true))

(fn ConstructionScript
  (bind _childactor (Variables|Default|GetChildActor))
  (bind _platformscale (Variables|Default|GetPlatformScale))
  (bind (_x _y) (Math|Vector|BreakVector _platformscale))
  (bind _returnvalue (* _platformscale 5e+01))
  (bind (_x_2 _y_2) (Math|Vector|BreakVector _returnvalue))
  (|CallParentFunction)
  (Transformation|SetWorldScale3D (Variables|Default|GetAnimSphere) _platformscale)
  (Transformation|SetWorldScale3D (Variables|Default|GetPantinCube) _platformscale)
  (Utilities|IsValid _childactor
    (:Is%20Valid
      (Transformation|SetWorldScale3D _childactor (Math|Vector|MakeVector _x _y (Variables|Default|GetZScaleOccluder)))
      (Components|Box|SetBoxExtent (Variables|Default|GetBox) (Math|Vector|MakeVector _x_2 _y_2 3e+01) true)
      (Transformation|SetRelativeLocation (Variables|Default|GetBox) (+ (+ (Variables|/Script/Engine.SceneComponent|GetRelativeLocation (Variables|Default|GetPantinCube)) (* (Math|Vector|MakeVector 0.0 0.0 (.Z (Math|Vector|BreakVector (Variables|Default|GetPlatformScale)))) 5e+01)) "0.000000,0.000000,5.000000") false false)
      (CallFunction|PlaceGodRay true))))

(fn GetInterractPoint
  (return (Transformation|GetActorLocation)))

(fn IsPickable
  (return (Variables|Default|GetIsPickupable)))

(fn GetCorkBoardIndex
  (return (Variables|Default|GetBoardIndex)))

(fn GetInputInfos
  (bind _gameinstance (CallFunction|GetBPGameInstance))
  (bind _languages (Variables|/Script/MyrmidonProto.RecordingGameInstance|GetLanguages _gameinstance))
  (return true (Utilities|Struct|MakeSTRUC_InputInfos true (Utilities|Select :Index _languages :French "Maintenir +" :English "Hold +") (Utilities|Select :Index _languages :French "Déplacer" :English "Move") "/Game/AssetsMyrmidon/Art/UI/Tex/CONTROLS/NEW_SPRITES/CONTROLS_GachetteRT_NoBackground.CONTROLS_GachetteRT_NoBackground" "/Game/AssetsMyrmidon/Art/UI/Tex/CONTROLS/NEW_SPRITES/CONTROLS_R_NoBackground.CONTROLS_R_NoBackground" "/Game/AssetsMyrmidon/Art/UI/Tex/CONTROLS/NEW_SPRITES/souris_gauche_NoBackground.souris_gauche_NoBackground" "/Game/AssetsMyrmidon/Art/UI/Tex/CONTROLS/NEW_SPRITES/souris_tourne_NoBackground.souris_tourne_NoBackground")))

(fn GetCorkOffset
  (return 1.5e+02))

(fn GetRectMargins
  (return "250.000000,250.000000,150.000000"))

(fn IsPicked
  (return (Variables|Default|GetPicked)))

(fn PickableShouldLerp
  (return (Variables|Default|GetShouldLerp)))