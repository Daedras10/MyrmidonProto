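; Level-design ventilator that, while activated, spins its rotor and blows wind on Windable actors inside its box volume.
; The construction script stacks the base, scalable pillar and head by height multiplier, sizes the wind box and aims the arrow along WindDirection.
; Overlap events and a delayed BeginPlay scan track Windables.
; Active-state toggles and overlap changes switch their wind, with force from normalized WindDirection times WindPower.
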(event OnComponentBeginOverlap(Box)
  (params (OverlappedComponent :type Primitive%20Component%20Object%20Reference) (OtherActor :type Actor%20Object%20Reference) (OtherComp :type Primitive%20Component%20Object%20Reference) (OtherBodyIndex :type Integer) (bFromSweep :type Boolean) (SweepResult :type Hit%20Result%20Structure%20%28by%20ref%29))
  (bind (_aswindable _bsuccess) (Utilities|Casting|CastToWindable OtherActor))
  (if _bsuccess
    (Utilities|Array|AddUnique (Variables|Default|GetWindables) _aswindable)
    (if (Variables|Default|GetActivated)
      (Class|Windable|SetActiveWind _aswindable true)
      (Class|Windable|SetWindDirection _aswindable (* (Math|Vector|Normalize (Variables|Default|GetWindDirection)) (Variables|Default|GetWindPower))))))

(event OnComponentEndOverlap(Box)
  (params (OverlappedComponent :type Primitive%20Component%20Object%20Reference) (OtherActor :type Actor%20Object%20Reference) (OtherComp :type Primitive%20Component%20Object%20Reference) (OtherBodyIndex :type Integer))
  (bind (_aswindable _bsuccess) (Utilities|Casting|CastToWindable OtherActor))
  (if _bsuccess
    (Utilities|Array|RemoveItem (Variables|Default|GetWindables) _aswindable)
    (if (Variables|Default|GetActivated)
      (Class|Windable|SetActiveWind _aswindable false))))

(event Custom|FixPlacement
  (bind _returnvalue (Transformation|GetActorLocation))
  (bind _link (Variables|Default|GetLink))
  (bind _sphere (Variables|Default|GetSphere))
  (bind _box (Variables|Default|GetBox))
  (bind _ventilatorheightmult (Variables|Default|GetVentilatorHeightMult))
  (bind _cubebase (Variables|Default|GetCubeBase))
  (bind _head (Variables|Default|GetHead))
  (bind _returnvalue_2 (Transformation|GetWorldLocation _sphere))
  (bind _returnvalue_3 (Transformation|GetWorldLocation _link))
  (bind _returnvalue_4 (Transformation|GetWorldScale _head))
  (bind _returnvalue_5 (Transformation|GetWorldScale _cubebase))
  (bind _returnvalue_6 (* _ventilatorheightmult 5e+01))
  (bind (_x _y) (Math|Vector|BreakVector _returnvalue_2))
  (bind (_x_2 _y_2) (Math|Vector|BreakVector _returnvalue_3))
  (bind _returnvalue_7 (Math|Vector|MakeVector 0.0 0.0 _returnvalue_6))
  (bind _returnvalue_8 (* _returnvalue_4 "0.000000,0.000000,50.000000"))
  (bind _returnvalue_9 (* _returnvalue_5 "0.000000,0.000000,50.000000"))
  (bind _returnvalue_10 (+ _returnvalue _returnvalue_9))
  (bind _returnvalue_11 (+ _returnvalue_10 _returnvalue_7))
  (bind _returnvalue_12 (+ _returnvalue_11 _returnvalue_7))
  (bind _returnvalue_13 (+ _returnvalue_12 _returnvalue_8))
  (bind _z (Math|Vector|BreakVector _returnvalue_13))
  (bind _returnvalue_14 (Math|Vector|MakeVector _x _y _z))
  ;[1 1 1] FixPlacement
  (Transformation|SetWorldLocation (Variables|Default|GetCubeBase) _returnvalue false false)
  (Transformation|SetWorldLocation (Variables|Default|GetCylinder) _returnvalue_11 false false)
  (Transformation|SetWorldScale3D (Variables|Default|GetCylinder) (Math|Vector|MakeVector 1.0 1.0 (Variables|Default|GetVentilatorHeightMult)))
  (Transformation|SetWorldLocation (Variables|Default|GetHead) _returnvalue_13 false false)
  (Transformation|SetWorldLocation (Variables|Default|GetLink) (Math|Vector|MakeVector _x_2 _y_2 _z) false false)
  (Transformation|SetWorldLocation (Variables|Default|GetSphere) _returnvalue_14 false false)
  (Transformation|SetWorldLocation _box (+ _returnvalue_14 "75.000000,0.000000,0.000000" (Math|Vector|MakeVector (.X (Math|Vector|BreakVector (* (Variables|Default|GetWindBoxScale) 5e+01))) 0.0 0.0)) false false)
  (Components|Box|SetBoxExtent _box (* (Variables|Default|GetWindBoxScale) 5e+01) true))

(event Custom|FixRotation
  ;[1 1 1] FixRotation
  (Transformation|SetWorldRotation (Variables|Default|GetArrow) (Math|Rotator|FindLookatRotation (Math|Vector|MakeVector 0.0 0.0 0.0) (Variables|Default|GetWindDirection)) false false))

(event Custom|SetActive
  (Variables|Default|SetActivated true)
  (for _array_element (Variables|Default|GetWindables)
    (Class|Windable|SetActiveWind _array_element true)
    (Class|Windable|SetWindDirection _array_element (* (Math|Vector|Normalize (Variables|Default|GetWindDirection)) (Variables|Default|GetWindPower)))))

(event Custom|SetInactive
  (Variables|Default|SetActivated false)
  (for _array_element (Variables|Default|GetWindables)
    (Class|Windable|SetActiveWind _array_element false)))

(event Custom|ChangeActiveState
  (if (Variables|Default|GetActivated)
    (CallFunction|SetInactive)
    (else
      (CallFunction|SetActive))))

(event EventBeginPlay
  (Utilities|FlowControl|Delay 0.1)
  (for _array_element (Collision|GetOverlappingActors (Variables|Default|GetBox) 0 :!class /Script/Engine.PrimitiveComponent)
    (bind _aswindable (Utilities|Casting|CastToWindable _array_element))
    (Utilities|Array|AddUnique (Variables|Default|GetWindables) _aswindable)))

(event EventTick
  (params (DeltaSeconds :type Float%20%28single-precision%29))
  ;[1 1 1] EventTick
  (if (Variables|Default|GetActivated)
    (Transformation|AddRelativeRotation (Variables|Default|GetSphere) (Math|Rotator|MakeRotator (* DeltaSeconds (Variables|Default|GetRotationSpeed)) 0.0 0.0) false false)))

(fn ConstructionScript
  (CallFunction|FixPlacement)
  (CallFunction|FixRotation))