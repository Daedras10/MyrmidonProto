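; BP_CorkCage is a resizable level-design cage that opens any BP_ItemBox overlapping its trigger volume.
; The construction script uses Size to position and scale four wall cubes, then scales a base cube and the Box trigger to match the footprint.
; On overlap, the cage passes its CorkID to the item box's OpenBox and prints its own name for debugging.
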(event OnComponentBeginOverlap(Box)
  (params (OverlappedComponent :type Primitive%20Component%20Object%20Reference) (OtherActor :type Actor%20Object%20Reference) (OtherComp :type Primitive%20Component%20Object%20Reference) (OtherBodyIndex :type Integer) (bFromSweep :type Boolean) (SweepResult :type Hit%20Result%20Structure%20%28by%20ref%29))
  (bind _asbp_item_box (Utilities|Casting|CastToBP_ItemBox OtherActor))
  (Default|OpenBox _asbp_item_box (Variables|Default|GetCorkID))
  (Development|PrintString (Utilities|GetDisplayName self)))

(fn ConstructionScript
  (bind _cube1 (Variables|Default|GetCube1))
  (bind _cube3 (Variables|Default|GetCube3))
  (bind _cube4 (Variables|Default|GetCube4))
  (bind _size (Variables|Default|GetSize))
  (bind _size_2 (Variables|Default|GetSize))
  (bind _cube2 (Variables|Default|GetCube2))
  (bind _size_3 (Variables|Default|GetSize))
  (bind _size_4 (Variables|Default|GetSize))
  (bind _size_5 (Variables|Default|GetSize))
  (bind (_x _y) (Math|Vector|BreakVector _size_3))
  (bind (_x_2 _y_2) (Math|Vector|BreakVector _size_4))
  (bind (_x_3 _y_3) (Math|Vector|BreakVector _size_5))
  (bind (_x_4 _y_4) (Math|Vector|BreakVector _size))
  (bind (_x_5 _y_5) (Math|Vector|BreakVector _size_2))
  (bind _returnvalue (* _y_2 0.01))
  (bind _returnvalue_2 (* _x_2 0.01))
  (bind _returnvalue_3 (+ _returnvalue 0.2))
  (bind _returnvalue_4 (+ _returnvalue_2 0.2))
  (Utilities|FlowControl|Sequence
    (:then_0
      (Transformation|SetRelativeLocation _cube1 (Math|Vector|MakeVector (* _x_5 0.5) 0.0 5e+01) false false)
      (Transformation|SetRelativeScale3D _cube1 (Math|Vector|MakeVector 0.2 (* _y_5 0.01) 1.0)))
    (:then_1
      (Transformation|SetRelativeLocation _cube2 (Math|Vector|MakeVector (* _x -0.5) 0.0 5e+01) false false)
      (Transformation|SetRelativeScale3D _cube2 (Math|Vector|MakeVector 0.2 (* _y 0.01) 1.0)))
    (:then_2
      (Transformation|SetRelativeLocation _cube3 (Math|Vector|MakeVector 0.0 (* _y_3 0.5) 5e+01) false false)
      (Transformation|SetRelativeScale3D _cube3 (Math|Vector|MakeVector (+ (* _x_3 0.01) 0.2) 0.2 1.0)))
    (:then_3
      (Transformation|SetRelativeLocation _cube4 (Math|Vector|MakeVector 0.0 (* _y_4 -0.5) 5e+01) false false)
      (Transformation|SetRelativeScale3D _cube4 (Math|Vector|MakeVector (+ (* _x_4 0.01) 0.2) 0.2 1.0)))
    (:then_4
      (Transformation|SetRelativeScale3D (Variables|Default|GetCube) (Math|Vector|MakeVector _returnvalue_4 _returnvalue_3 0.2))
      (Transformation|SetRelativeScale3D (Variables|Default|GetBox) (Math|Vector|MakeVector _returnvalue_4 _returnvalue_3 1.0)))))