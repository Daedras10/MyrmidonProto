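; Base switch level-design element with two visual states, a Pantin view showing a cube and an Animator view showing a sphere.
; Switch events toggle which mesh is visible and record the current view.
; Pick up and drop toggle actor collision, while hover events enable custom depth outlines and turn the sphere red through multicast-named events.
; StartA and StartB are debug print stubs.
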(event Custom|EndHoverMulticasted
  ;[1 1 1] Start & End Hover
  (Rendering|SetRenderCustomDepth (Variables|Default|GetPantinCube) false)
  (Rendering|SetRenderCustomDepth (Variables|Default|GetAnimSphere) false)
  (Rendering|Material|SetMaterial (Variables|Default|GetAnimSphere) 0 "/Engine/BasicShapes/BasicShapeMaterial.BasicShapeMaterial"))

(event Custom|BeginHoverMulticasted
  ;[1 1 1] Start & End Hover
  (Rendering|SetRenderCustomDepth (Variables|Default|GetPantinCube) true)
  (Rendering|SetRenderCustomDepth (Variables|Default|GetAnimSphere) true)
  (Rendering|Material|SetMaterial (Variables|Default|GetAnimSphere) 0 "/Game/AssetsMyrmidon/Art/Materials/M_Red.M_Red"))

(event Custom|SetCollisions
  (params (Active :type Boolean))
  ;[1 1 1] PickUp and Drop
  (Collision|SetActorEnableCollision self Active))

(event EventPickUp
  ;[1 1 1] PickUp and Drop
  (CallFunction|SetCollisions false))

(event EventDrop
  ;[1 1 1] PickUp and Drop
  (CallFunction|SetCollisions true))

(event EventStartHover
  ;[1 1 1] Start & End Hover
  (CallFunction|BeginHoverMulticasted))

(event EventEndHover
  ;[1 1 1] Start & End Hover
  (CallFunction|EndHoverMulticasted))

(event EventStartA
  (Development|PrintString "StartA"))

(event EventStartB
  (Development|PrintString "StartB"))

(event EventSwitch
  (params (bToPantin :type Boolean))
  ;[1 1 1] Switch
  (if bToPantin
    (Class|VisualSwitcher|SwitchtoPantin)
    (else
      (Class|VisualSwitcher|SwitchtoAnimator))))

(event EventSwitchtoAnimator
  ;[1 1 1] SwitchTo
  (Rendering|SetVisibility (Variables|Default|GetAnimSphere) true false)
  (Rendering|SetVisibility (Variables|Default|GetPantinCube) false false)
  (Variables|Default|SetIsPantinView false))

(event EventSwitchtoPantin
  ;[1 1 1] SwitchTo
  (Rendering|SetVisibility (Variables|Default|GetAnimSphere) false false)
  (Rendering|SetVisibility (Variables|Default|GetPantinCube) true false)
  (Variables|Default|SetIsPantinView true))

(fn ConstructionScript)