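; Base button level-design element with hover, activate and deactivate states, providing empty hooks for specific button behavior.
; Hovering toggles custom depth rendering on AnimSphere.
; StartB turns the sphere red and sets IsActive; EndB restores the basic material, also through MulticastEndB, and clears the flag.
; Both fire OnButtonActivated or OnButtonDeactivated, and Tick calls ButtonActive while active.
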(event Custom|MulticastEndB
  (Rendering|Material|SetMaterial (Variables|Default|GetAnimSphere) 0 "/Engine/BasicShapes/BasicShapeMaterial.BasicShapeMaterial"))

(event Custom|ButtonActive
  (params (DeltaSeconds :type Float%20%28double-precision%29)))

(event Custom|OnButtonActivated)

(event Custom|OnButtonDeactivated)

(event EventTick
  (params (DeltaSeconds :type Float%20%28single-precision%29))
  (if (Variables|Default|GetIsActive)
    (CallFunction|ButtonActive DeltaSeconds)))

(event EventStartHover
  (Rendering|SetRenderCustomDepth (Variables|Default|GetAnimSphere) true))

(event EventEndHover
  (Rendering|SetRenderCustomDepth (Variables|Default|GetAnimSphere) false))

(event EventStartB
  (Rendering|Material|SetMaterial (Variables|Default|GetAnimSphere) 0 "/Game/AssetsMyrmidon/Art/Materials/M_Red.M_Red")
  (Variables|Default|SetIsActive true)
  (CallFunction|OnButtonActivated))

(event EventEndB
  (Rendering|Material|SetMaterial (Variables|Default|GetAnimSphere) 0 "/Engine/BasicShapes/BasicShapeMaterial.BasicShapeMaterial")
  (CallFunction|MulticastEndB)
  (Variables|Default|SetIsActive false)
  (CallFunction|OnButtonDeactivated))

(fn ConstructionScript
  (|CallParentFunction))