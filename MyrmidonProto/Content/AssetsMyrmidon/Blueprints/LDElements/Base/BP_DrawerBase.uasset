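; Base Blueprint for an interactive drawer that slides between a start and end position.
; Grabbing starts a server-side delay, then either flips direction or, in follow mode, matches stick or look input to the drawer axis by dot product.
; Tick lerps the drawer along that path and refreshes god ray occluders.
; Construction sizes handles and applies the initial open state; switch events swap Animator and Pantin meshes.
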(event Custom|Scale
  (bind _handlemain (Variables|Default|GetHandleMain))
  (bind _handle1 (Variables|Default|GetHandle1))
  (bind _returnvalue (Transformation|GetWorldScale _handle1))
  (bind _returnvalue_2 (Transformation|GetWorldScale _handlemain))
  (bind _z (Math|Vector|BreakVector _returnvalue))
  (bind _z_2 (Math|Vector|BreakVector _returnvalue_2))
  (bind _returnvalue_3 (* _z_2 -5e+01))
  (bind _returnvalue_4 (* _z 5e+01))
  (bind _returnvalue_5 (Math|Vector|MakeVector _returnvalue_4 _returnvalue_3 0.0))
  (bind _returnvalue_6 (* _returnvalue_5 "1.000000,-1.000000,0.000000"))
  (bind _returnvalue_7 (* _returnvalue_6 "2.000000,0.000000,0.000000"))
  (CallFunction|ScaleHandle)
  (CallFunction|ScaleContent)
  (Transformation|SetRelativeLocation _handle1 _returnvalue_5 false false)
  (Transformation|SetRelativeLocation (Variables|Default|GetHandle2) _returnvalue_6 false false)
  (Transformation|SetRelativeLocation (Variables|Default|GetHandleMain) _returnvalue_7 false false)
  (Transformation|SetRelativeLocation (Variables|Default|GetSphere) _returnvalue_7 false false)
  (Transformation|SetRelativeLocation (Variables|Default|GetBox) _returnvalue_7 false false)
  (CallFunction|PlaceHandle))

(event Custom|ScaleHandle
  (bind _handlescale (Variables|Default|GetHandleScale))
  (Transformation|SetRelativeScale3D (Variables|Default|GetHandleMain) _handlescale)
  (Transformation|SetRelativeScale3D (Variables|Default|GetHandle1) _handlescale)
  (Transformation|SetRelativeScale3D (Variables|Default|GetHandle2) _handlescale))

(event Custom|UpdateGodRays
  ;[1 1 1] UpdateGodRays
  (for _array_element (Variables|Settings|GetGodRaysToUpdate)
    (Default|UpdateOccluders _array_element)))

(event Custom|ToPantinDebug
  ;[1 1 1] Switchers
  (Class|VisualSwitcher|SwitchtoPantin))

(event Custom|ToAnimatorDebug
  ;[1 1 1] Switchers
  (Class|VisualSwitcher|SwitchtoAnimator))

(event Custom|FinishMovingAtAlpha
  (params (Alpha :type Float%20%28double-precision%29))
  ;[1 1 1] EventTick
  (Transformation|SetWorldLocation (Variables|Default|GetArrowParent) (Math|Vector|Lerp(Vector) (Variables|Default|GetInitialPosition) (Variables|Default|GetWorldEndPos) Alpha) false false)
  (CallFunction|UpdateGodRays))

(event Custom|SetInitialPos
  (bind _drawermeshanimator (Variables|Default|GetDrawerMeshAnimator))
  (bind _drawermeshpantin (Variables|Default|GetDrawerMeshPantin))
  ;[1 1 1] BeginPlay
  (Variables|Default|SetInitialPosition (Transformation|GetWorldLocation (Variables|Default|GetInitialPos)))
  (Variables|Default|SetWorldEndPos (+ (Math|Vector|RotateVector (Variables|Settings|GetEndPosition) (Transformation|GetActorRotation)) (Transformation|GetWorldLocation (Variables|Default|GetInitialPos))))
  (Transformation|SetRelativeLocation (Variables|Default|GetArrowMeshParent) (Math|Vector|MakeVector 0.0 0.0 (* (.Z (Math|Vector|BreakVector (Variables|Default|GetDrawerScale))) -5e+01)) false false)
  (Transformation|SetRelativeLocation _drawermeshanimator "0, 0, 0" false false)
  (Transformation|SetRelativeLocation _drawermeshpantin "0, 0, 0" false false)
  (Transformation|SetRelativeRotation _drawermeshanimator "0, 0, 0" false false)
  (Transformation|SetRelativeRotation _drawermeshpantin "0, 0, 0" false false))

(event Custom|InstantMoveToPos
  ;[1 1 1] InstantMoveToPos
  (Transformation|SetWorldLocation (Variables|Default|GetArrowParent) (Math|Vector|Lerp(Vector) (Variables|Default|GetInitialPosition) (Variables|Default|GetWorldEndPos) (Math|Float|SelectFloat 0.0 1.0 (Variables|Default|GetStartClosed))) false false)
  (Variables|Default|SetGoingBack (Variables|Default|GetStartClosed)))

(event Custom|Direction
  (bind _gamemode (CallFunction|GetBPGameMode))
  (bind _gamemode_2 (CallFunction|GetBPGameMode))
  (bind _returnvalue (Transformation|GetActorForwardVector))
  (bind _playercontroller (Default|GetBPPlayerController _gamemode false))
  (bind _playercontroller_2 (Default|GetBPPlayerController _gamemode_2 false))
  (bind _returnvalue_2 (* _returnvalue "1.000000,1.000000,0.000000"))
  (bind _returnvalue_3 (Pawn|GetControlledPawn _playercontroller_2))
  (bind _returnvalue_4 (Math|Vector|Normalize _returnvalue_2))
  (bind _playermoveinputs (Variables|/Game/AssetsMyrmidon/Blueprints/GameMode/BP_PlayerController.BP_PlayerController_C|GetPlayerMoveInputs _playercontroller))
  (bind _playerlookinputs (Variables|/Game/AssetsMyrmidon/Blueprints/GameMode/BP_PlayerController.BP_PlayerController_C|GetPlayerLookInputs _playercontroller))
  (bind _lastinputswasgamepad (Variables|/Game/AssetsMyrmidon/Blueprints/GameMode/BP_PlayerController.BP_PlayerController_C|GetLastInputsWasGamepad _playercontroller))
  (bind (_x _y) (Math|Vector2D|BreakVector2D _playerlookinputs))
  (bind _asbp_animateur (Utilities|Casting|CastToBP_Animateur _returnvalue_3))
  (bind _returnvalue_5 (Transformation|GetActorRotation _asbp_animateur))
  (bind _returnvalue_6 (* _y -1.0))
  (bind _returnvalue_7 (Math|Vector2D|MakeVector2D _returnvalue_6 _x))
  (bind _returnvalue_8 (select _lastinputswasgamepad _playermoveinputs _returnvalue_7))
  (bind _returnvalue_9 (Math|Conversions|ToVector(Vector2D) _returnvalue_8))
  (bind _returnvalue_10 (Math|Vector|RotateVector _returnvalue_9 _returnvalue_5))
  (bind _returnvalue_11 (Math|Vector|Normalize _returnvalue_10))
  (bind _returnvalue_12 (Math|Vector|DotProduct _returnvalue_11 _returnvalue_4))
  (bind _returnvalue_13 (Math|Float|NearlyEqual(Float) _returnvalue_12 -1.0 0.2))
  ;[1 1 1] Direction v2 (move inputs & look inputs)
  (Networking|SwitchHasAuthority
    (:Authority
      (if (and (Variables|Default|GetFollowMouse) (not (Variables|Default|GetIsMoving)))
        (if (and (>= (Math|Vector2D|Vector2DLength _returnvalue_8) 1.0) (or (Math|Float|NearlyEqual(Float) _returnvalue_12 1.0 0.2) _returnvalue_13))
          (Variables|Default|SetGoingBack _returnvalue_13)
          (if (> (Math|Vector|Distance(Vector) (Transformation|GetWorldLocation (Variables|Default|GetArrowParent)) (Math|Vector|SelectVector (Variables|Default|GetInitialPosition) (Variables|Default|GetWorldEndPos) (Variables|Default|GetGoingBack))) 1.0)
            (Variables|Default|SetTimer (Variables|Default|GetDelayBeforeMovement))
            (Variables|Default|SetCanMove false)
            (Utilities|FlowControl|Delay 0.01)
            (Variables|Default|SetIsMoving true)))))))

(event Custom|CheckTimerToStartMoving
  (params (DetaTime :type Float%20%28double-precision%29))
  ;[1 1 1] CheckTimerToStartMoving
  (if (and (not (Variables|Default|GetCanMove)) (>= (Variables|Default|GetTimer) 0.0))
    (Variables|Default|SetTimer (- (Variables|Default|GetTimer) DetaTime))
    (if (<= (Variables|Default|GetTimer) 0.0)
      (Variables|Default|SetTimer -1.0)
      (Variables|Default|SetCanMove true)
      (if (not (Variables|Default|GetModeFollowMouse))
        (Variables|Default|SetGoingBack (not (Variables|Default|GetGoingBack)))))))

(event Custom|ScaleContent)

(event Custom|PlaceHandle)

(event Custom|PlaceContent)

(event Custom|CustomEvent
  (params (DeltaSeconds :type Float%20%28single-precision%29))
  ;[1 1 1] EventTick
)

(event EventBeginPlay
  ;[1 1 1] BeginPlay
  (Networking|SwitchHasAuthority
    (:Authority
      (CallFunction|SetInitialPos))))

(event EventStartHover
  ;[1 1 1] Hover
)

(event EventSwitchtoAnimator
  ;[1 1 1] Switchers
  (Rendering|SetVisibility (Variables|Default|GetDrawerMeshAnimator) true false)
  (Rendering|SetVisibility (Variables|Default|GetDrawerMeshPantin) false false))

(event EventSwitch
  (params (bToPantin :type Boolean))
  ;[1 1 1] Switchers
  (if bToPantin
    (Class|VisualSwitcher|SwitchtoPantin)
    (else
      (Class|VisualSwitcher|SwitchtoAnimator))))

(event EventEndHover
  ;[1 1 1] Hover
)

(event EventTick
  (params (DeltaSeconds :type Float%20%28single-precision%29))
  (bind _returnvalue (* DeltaSeconds -1.0))
  (bind _goingback (Variables|Default|GetGoingBack))
  (bind _speed (Variables|Default|GetSpeed))
  (bind _goingback_2 (Variables|Default|GetGoingBack))
  (bind _initialposition (Variables|Default|GetInitialPosition))
  (bind _worldendpos (Variables|Default|GetWorldEndPos))
  (bind _worldendpos_2 (Variables|Default|GetWorldEndPos))
  (bind _arrowparent (Variables|Default|GetArrowParent))
  (bind _returnvalue_2 (Math|Float|SelectFloat 0.0 1.0 _goingback_2))
  (bind _returnvalue_3 (Math|Vector|Distance(Vector) _initialposition _worldendpos))
  (bind _returnvalue_4 (Transformation|GetWorldLocation _arrowparent))
  (bind _returnvalue_5 (select _goingback _returnvalue DeltaSeconds))
  (bind _returnvalue_6 (Math|Vector|Distance(Vector) _returnvalue_4 _worldendpos_2))
  (bind _returnvalue_7 (* _returnvalue_5 _speed))
  (bind _returnvalue_8 (/ _returnvalue_6 _returnvalue_3))
  (bind _returnvalue_9 (- 1.0 _returnvalue_8))
  (bind _returnvalue_10 (+ _returnvalue_7 _returnvalue_9))
  (bind _returnvalue_11 (Math|Float|Clamp(Float) _returnvalue_10))
  ;[1 1 1] EventTick
  (CallFunction|CheckTimertoStartMoving DeltaSeconds)
  (if (Variables|Default|GetCanMove)
    (if (Variables|Default|GetModeFollowMouse)
      (CallFunction|Direction))
    (if (Math|Boolean|ANDBoolean (Variables|Default|GetMoveAllowed) (Variables|Default|GetIsMoving) (Variables|Default|GetCanMove))
      (Transformation|SetWorldLocation (Variables|Default|GetArrowParent) (Math|Vector|Lerp(Vector) (Variables|Default|GetInitialPosition) (Variables|Default|GetWorldEndPos) _returnvalue_11) false false)
      (CallFunction|UpdateGodRays)
      (if (and (not (Variables|Default|GetModeFollowMouse)) (Math|Float|NearlyEqual(Float) _returnvalue_11 _returnvalue_2 (Variables|Default|GetMinimalPercentDistance)))
        (Networking|SwitchHasAuthority
          (:Authority
            (Variables|Default|SetCanMove false)
            (Variables|Default|SetIsMoving false)
            (CallFunction|FinishMovingatAlpha _returnvalue_2)))
        (elif (and (Math|Float|NearlyEqual(Float) _returnvalue_11 _returnvalue_2 1e-06) (Variables|Default|GetIsMoving))
          (Variables|Default|SetIsMoving false)
          (CallFunction|FinishMovingatAlpha _returnvalue_2))))))

(event EventShowAim
  ;[1 1 1] Hover
  (Rendering|SetVisibility (Variables|Default|GetSphere) true false))

(event EventStartB
  (bind _gamemode (CallFunction|GetBPGameMode))
  (bind _playercontroller (Default|GetBPPlayerController _gamemode false))
  ;[1 1 1] Interaction
  (Networking|SwitchHasAuthority
    (:Authority
      (Variables|Default|SetTimer (Variables|Default|GetDelayBeforeMovement))
      (Variables|Default|SetFollowMouse true)
      (if (Variables|/Game/AssetsMyrmidon/Blueprints/GameMode/BP_PlayerController.BP_PlayerController_C|GetLastInputsWasGamepad _playercontroller)
        (Default|DisableMvServer _playercontroller)
        (else
          (Default|DisableMvLookatServer _playercontroller))))))

(event EventHideAim
  ;[1 1 1] Hover
  (Rendering|SetVisibility (Variables|Default|GetSphere) false false))

(event EventEndB
  ;[1 1 1] Interaction
  (Networking|SwitchHasAuthority
    (:Authority
      (Variables|Default|SetTimer -1.0)
      (if (Variables|Default|GetModeFollowMouse)
        (Variables|Default|SetFollowMouse false)
        (Default|EnableMvLookatServer (Default|GetBPPlayerController (.GameMode (CallFunction|GetBPGameMode)) false))))))

(event EventSwitchtoPantin
  ;[1 1 1] Switchers
  (Rendering|SetVisibility (Variables|Default|GetDrawerMeshAnimator) false false)
  (Rendering|SetVisibility (Variables|Default|GetDrawerMeshPantin) true false))

(fn ConstructionScript
  (|CallParentFunction)
  (CallFunction|SetInitialPos)
  (CallFunction|Scale)
  (CallFunction|InstantMovetoPos))

(fn GetInterractPoint
  (return (Transformation|GetWorldLocation (Variables|Default|GetBox))))

(fn GetInputInfos
  (return true (Utilities|Struct|MakeSTRUC_InputInfos true "Grab +" "push / pull" "/Game/AssetsMyrmidon/Art/Textures/T_ButtonLT.T_ButtonLT" "/Game/AssetsMyrmidon/Art/Textures/T_StickL.T_StickL")))