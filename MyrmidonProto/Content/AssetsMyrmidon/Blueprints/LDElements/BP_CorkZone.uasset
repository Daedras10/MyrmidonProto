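; BP_CorkZone is a level-design element that defines a rectangular cork board area, identified by a CorkID.
; The construction script scales its Cube component to BoardSize.
; GetClosestPointOnBoard clamps a location in actor space to the board's XZ half extents, flattens Y to zero, and returns the world point with the actor's right vector as normal.
; GetCorkIndex exposes the CorkID.
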(fn ConstructionScript
  (Transformation|SetRelativeScale3D (Variables|Default|GetCube) (Variables|Default|GetBoardSize)))

(fn GetClosestPointonBoard
  (params (Location :type Vector :default "0, 0, 0"))
  (bind _returnvalue (Transformation|GetActorTransform))
  (bind _boardsize (Variables|Default|GetBoardSize))
  (bind _returnvalue_2 (Math|Transform|InverseTransformLocation _returnvalue Location))
  (bind _returnvalue_3 (* _boardsize 5e+01))
  (bind (_x _y _z) (Math|Vector|BreakVector _returnvalue_2))
  (bind (_x_2 _y_2 _z_2) (Math|Vector|BreakVector _returnvalue_3))
  (return (Math|Transform|TransformLocation (Transformation|GetActorTransform) (Math|Vector|MakeVector (Math|Float|Clamp(Float) _x (* _x_2 -1.0) _x_2) 0.0 (Math|Float|Clamp(Float) _z (* _z_2 -1.0) _z_2))) (Transformation|GetActorRightVector)))

(fn GetCorkIndex
  (return (Variables|Default|GetCorkID)))