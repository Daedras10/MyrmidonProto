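; Scalable drawer level-design element with a handle and an aim highlight.
; ScaleContent applies DrawerScale to the Cube, and PlaceHandle offsets the handle parent along X in proportion to the Cube's X scale.
; ShowAim and HideAim toggle the DrawerMeshAnimator's custom depth stencil value, only when the local player controller is not Pantin.
; The construction script only calls its parent, and no calls to the sizing events appear here.
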(event EventBeginPlay
  (|CallParentFunction) ; This node is disabled and will not be called.\nDrag off pins to build functionality.
)

(event Collision|EventActorBeginOverlap
  (params (OtherActor :type Actor%20Object%20Reference)))

(event EventTick
  (params (DeltaSeconds :type Float%20%28single-precision%29))
  (|CallParentFunction DeltaSeconds) ; This node is disabled and will not be called.\nDrag off pins to build functionality.
)

(event EventPlaceHandle
  (Transformation|SetRelativeLocation (Variables|Default|GetHandleParent) (Math|Vector|MakeVector (* (.X (Math|Vector|BreakVector (Variables|/Script/Engine.SceneComponent|GetRelativeScale3D (Variables|Default|GetCube)))) 5e+01) 0.0 0.0) false false))

(event EventScaleContent
  (Transformation|SetRelativeScale3D (Variables|Default|GetCube) (Variables|Default|GetDrawerScale)))

(event EventShowAim
  ;[1 1 1] Aim
  (if (not (Variables|/Game/AssetsMyrmidon/Blueprints/GameMode/BP_PlayerController.BP_PlayerController_C|GetisPantin (.PlayerController (CallFunction|GetBPLocalPlayerController))))
    (Rendering|SetCustomDepthStencilValue (Variables|Default|GetDrawerMeshAnimator) 1)))

(event EventHideAim
  ;[1 1 1] Aim
  (if (not (Variables|/Game/AssetsMyrmidon/Blueprints/GameMode/BP_PlayerController.BP_PlayerController_C|GetisPantin (.PlayerController (CallFunction|GetBPLocalPlayerController))))
    (Rendering|SetCustomDepthStencilValue (Variables|Default|GetDrawerMeshAnimator) 0)))

(fn ConstructionScript
  (|CallParentFunction))