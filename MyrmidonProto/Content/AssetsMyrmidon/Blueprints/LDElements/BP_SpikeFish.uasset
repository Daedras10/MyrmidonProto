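; BP_SpikeFish is a level hazard that moves a sphere up and down its local Z axis and kills BP_Pantin characters on overlap, on authority only.
; A timeline lerps the sphere between plus and minus MovementStrenght, with play rate from MovementTime and a StartTime offset.
; The construction script sizes the range arrows and sets the timeline's start time.
; BeginPlay is empty and the GameMode late-start binding is disconnected, so nothing here triggers the Start chain.
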(event OnComponentBeginOverlap(KillColision)
  (params (OverlappedComponent :type Primitive%20Component%20Object%20Reference) (OtherActor :type Actor%20Object%20Reference) (OtherComp :type Primitive%20Component%20Object%20Reference) (OtherBodyIndex :type Integer) (bFromSweep :type Boolean) (SweepResult :type Hit%20Result%20Structure%20%28by%20ref%29))
  (Networking|SwitchHasAuthority
    (:Authority
      (bind _asbp_pantin (Utilities|Casting|CastToBP_Pantin OtherActor))
      (Default|KillServer _asbp_pantin))))

(event Custom|StartMoving
  (bind _movementstrenght (Variables|Default|GetMovementStrenght))
  (Variables|Default|SetStarted true)
  (CallFunction|StartMoving2)
  (Development|PrintString (Utilities|GetDisplayName self))
  (Components|Timeline|SetPlayRate (Variables|Default|GetMovementCurve) (/ 1.0 (Variables|Default|GetMovementTime)))
  (bind _position (Timeline|MovementCurve Play)
    (:Update
      (Transformation|SetRelativeLocation (Variables|Default|GetSphere) (Math|Vector|MakeVector 0.0 0.0 (Math|Float|Lerp (* _movementstrenght -1.0) _movementstrenght _position)) false false))))

(event Custom|Start
  (EventDispatchers|UnbindEventfromGameLateStart (.GameMode (CallFunction|GetBPGameMode)) (delegate Custom|Start))
  (CallFunction|StartServer))

(event Custom|StartServer
  (CallFunction|StartMoving))

(event Custom|StartMoving2
  (bind _movementstrenght (Variables|Default|GetMovementStrenght))
  (if (not (Variables|Default|GetStarted))
    (Development|PrintString (Utilities|GetDisplayName self))
    (Components|Timeline|SetPlayRate (Variables|Default|GetMovementCurve) (/ 1.0 (Variables|Default|GetMovementTime)))
    (bind _position (Timeline|MovementCurve Play)
      (:Update
        (Transformation|SetRelativeLocation (Variables|Default|GetSphere) (Math|Vector|MakeVector 0.0 0.0 (Math|Float|Lerp (* _movementstrenght -1.0) _movementstrenght _position)) false false)))))

(event EventBeginPlay)

(fn ConstructionScript
  (bind _movementcurve (Variables|Default|GetMovementCurve))
  (Variables|/Script/Engine.ArrowComponent|SetArrowLength (Variables|Default|GetArrowUp) (Variables|Default|GetMovementStrenght))
  (Variables|/Script/Engine.ArrowComponent|SetArrowLength (Variables|Default|GetArrowDown) (Variables|Default|GetMovementStrenght))
  (Components|Timeline|SetNewTime _movementcurve (Variables|Default|GetStartTime))
  (Audio|Components|Audio|Play _movementcurve)
  (Audio|Components|Audio|Stop _movementcurve))