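; Base actor, by its name a parent class, for a pickable object that switches between a Pantin form (cube) and an Animateur form (sphere).
; Switch takes a boolean and shows one mesh while hiding the other.
; Pick disables actor collision and Dropped restores it.
; Hover events toggle custom depth on both meshes, swap the sphere's material to red and back, and print debug strings.
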(event Custom|SetCollisions
  (params (Active :type Boolean))
  (Collision|SetActorEnableCollision self Active))

(event Custom|BeginHover
  (params (TouchedActor :type Actor%20Object%20Reference))
  (Development|PrintString "BeginHover")
  (Rendering|SetRenderCustomDepth (Variables|Default|GetPantinCube) true)
  (Rendering|SetRenderCustomDepth (Variables|Default|GetAnimSphere) true)
  (Rendering|Material|SetMaterial (Variables|Default|GetAnimSphere) 0 "/Game/AssetsMyrmidon/Art/Materials/M_Red.M_Red"))

(event Custom|EndHover
  (params (TouchedActor :type Actor%20Object%20Reference))
  (Development|PrintString "EndHover")
  (Rendering|SetRenderCustomDepth (Variables|Default|GetPantinCube) false)
  (Rendering|SetRenderCustomDepth (Variables|Default|GetAnimSphere) false)
  (Rendering|Material|SetMaterial (Variables|Default|GetAnimSphere) 0 "/Engine/BasicShapes/BasicShapeMaterial.BasicShapeMaterial"))

(event EventSwitch
  (params (isPantin :type Boolean))
  (if isPantin
    (CallFunction|SwitchtoPantin)
    (else
      (CallFunction|SwitchtoAnimateur))))

(event EventSwitchtoAnimateur
  (Rendering|SetVisibility (Variables|Default|GetAnimSphere) true false)
  (Rendering|SetVisibility (Variables|Default|GetPantinCube) false false))

(event EventSwitchtoPantin
  (Rendering|SetVisibility (Variables|Default|GetAnimSphere) false false)
  (Rendering|SetVisibility (Variables|Default|GetPantinCube) true false))

(event EventPick
  (CallFunction|SetCollisions false))

(event EventDropped
  (CallFunction|SetCollisions true))

(fn ConstructionScript)