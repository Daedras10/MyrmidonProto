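; Static helper library that gives shared access to the game's core framework objects and spatial queries.
; Getters return player controller 0, the game mode and the game instance cast to project classes, with success flags.
; Cork board lookup finds the nearest point and normal among cork zones matching an index.
; Interactable lookup returns the interact point best aligned with a forward vector, using visibility traces that ignore interactables to reject blocked ones.
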(fn GetBPLocalPlayerController
  (bind ___worldcontext (LocalVariables|Get__WorldContext))
  (bind _returnvalue (Game|GetPlayerController ___worldcontext))
  (bind (_asbp_player_controller _bsuccess) (Utilities|Casting|CastToBP_PlayerController _returnvalue))
  (return _asbp_player_controller _bsuccess))

(fn GetBPGameMode
  (bind ___worldcontext (LocalVariables|Get__WorldContext))
  (bind _returnvalue (Game|GetGameMode ___worldcontext))
  (bind (_asbp_game_mode _bsuccess) (Utilities|Casting|CastToBP_GameMode _returnvalue))
  (return _asbp_game_mode _bsuccess))

(fn GetBPGameInstance
  (bind ___worldcontext (LocalVariables|Get__WorldContext))
  (bind _returnvalue (Game|GetGameInstance ___worldcontext))
  (bind (_asbp_game_instance _bsuccess) (Utilities|Casting|CastToBP_GameInstance _returnvalue))
  (return _asbp_game_instance _bsuccess))

(fn GetClosestPointonCorkBoardswithIndex
  (params (Location :type Vector) (Index :type Integer))
  (bind _outactors (Actor|GetAllActorsOfClass (LocalVariables|Get__WorldContext) "/Game/AssetsMyrmidon/Blueprints/LDElements/BP_CorkZone.BP_CorkZone_C"))
  (for _array_element _outactors
    (bind _index (Class|BPICorkZone|GetCorkIndex(Message) _array_element))
    (if (== _index Index)
      (bind (_closestpoint _pointnormal) (Class|BPICorkZone|GetClosestPointonBoard(Message) _array_element Location))
      (if (< (Math|Vector|Distance(Vector) _closestpoint Location) (LocalVariables|Getdist))
        (LocalVariables|Setdist (Math|Vector|Distance(Vector) _closestpoint Location))
        (LocalVariables|SetClosestLoc _closestpoint)
        (LocalVariables|SetClosestNor _pointnormal))))
  (return (LocalVariables|GetClosestLoc) (LocalVariables|GetClosestNor)))

(fn GetClosestInterractable
  (params (Position :type Vector) (Forward :type Vector))
  (bind _outactors (Actor|GetAllActorswithInterface (LocalVariables|Get__WorldContext) "/Script/MyrmidonProto.Interactable"))
  (for _array_element _outactors
    (bind _returnvalue (Class|Interactable|GetInterractPoint(Message) _array_element))
    (if (> (Math|Vector|DotProduct (Math|Vector|Normalize Forward) (Math|Vector|Normalize (- _returnvalue Position))) (LocalVariables|GetClosestDot))
      (bind _returnvalue_2 (Collision|LineTraceByChannel 0 Position _returnvalue "TraceTypeQuery1" false _outactors "None"))
      (if (not _returnvalue_2)
        (LocalVariables|SetClosestDot (Math|Vector|DotProduct (Math|Vector|Normalize Forward) (Math|Vector|Normalize (- _returnvalue Position))))
        (LocalVariables|SetClosestPos _returnvalue))))
  (return (LocalVariables|GetClosestPos)))