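; BP_LobbyGameMode is the lobby game mode that syncs lobby state to players when one joins.
; Its PlayerJoined event loops over the player controllers and calls UpdateValuesOnJoinOwning on each BP_LobbyController.
; It passes the HUD index from player controller 0 and the IsPantin flag from BP_GameInstance, sent as player one's Pantin state.
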(event Custom|PlayerJoined
  ;[1 1 1] PlayerJoined
  (for _index (range 0 (Class|GameplayStatics|GetNumPlayerControllers))
    (bind _asbp_lobby_controller (Utilities|Casting|CastToBP_LobbyController (Game|GetPlayerController _index)))
    (Default|UpdateValuesonJoinOwning _asbp_lobby_controller (Variables|/Game/AssetsMyrmidon/Blueprints/UI/WBP_Lobby.WBP_Lobby_C|GetIndex (Variables|/Game/AssetsMyrmidon/Blueprints/GameMode/BP_LobbyController.BP_LobbyController_C|GetHud (.AsBP%20Lobby%20Controller (Utilities|Casting|CastToBP_LobbyController (Game|GetPlayerController 0))))) (Variables|/Script/MyrmidonProto.RecordingGameInstance|GetIsPantin (.AsBP%20Game%20Instance (Utilities|Casting|CastToBP_GameInstance (Game|GetGameInstance)))))))

(fn ConstructionScript)