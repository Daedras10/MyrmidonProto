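; Main menu game mode that arbitrates which of two players takes the Pantin and Animator roles and relays lobby state to their BP_MenuPlayerControllers.
; SelectionButton claims a free role or releases the player's own, freeing their other role on a claim, then pushes the selection to both controllers.
; Roles map to the host's local Steam ID or the client ID stored by PlayerJoined.
; Sychro sends both IDs, two-player status and player position to each controller.
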(event Custom|Sychro
  ;[1 1 1] SynchroHost
  (bind _returnvalue (Class|GameModeBase|GetNumPlayers))
  (for _index (range 0 _returnvalue)
    (bind _asbp_menu_player_controller (Utilities|Casting|CastToBP_MenuPlayerController (Game|GetPlayerController _index)))
    (Default|Synchro _asbp_menu_player_controller (Class|AdvancedSteamFriendsLibrary|GetLocalSteamIDfromSteam) (Variables|Default|GetClient%20UID) (not (== _returnvalue 1)) (!= _index 0))))

(event Custom|PlayerJoined
  (params (UniqueID :type BP%20Unique%20Net%20Id%20Structure))
  ;[1 1 1] Player Joined
  (Variables|Default|SetClient%20UID UniqueID))

(event Custom|SynchroCharacterSelection
  (bind _returnvalue (Class|AdvancedSteamFriendsLibrary|GetLocalSteamIDfromSteam))
  (bind _returnvalue_2 (Class|AdvancedSteamFriendsLibrary|GetLocalSteamIDfromSteam))
  (bind _pantinplayer (Variables|Default|GetPantinPlayer))
  (bind _animatorplayer (Variables|Default|GetAnimatorPlayer))
  (bind _client_uid (Variables|Default|GetClient%20UID))
  (bind _client_uid_2 (Variables|Default|GetClient%20UID))
  (bind _pantinplayer_2 (Variables|Default|GetPantinPlayer))
  (bind _animatorplayer_2 (Variables|Default|GetAnimatorPlayer))
  (bind _returnvalue_3 (== _animatorplayer_2 1))
  (bind _returnvalue_4 (!= _pantinplayer -1))
  (bind _returnvalue_5 (!= _animatorplayer -1))
  (bind _returnvalue_6 (== _pantinplayer_2 1))
  (bind _returnvalue_7 (select _returnvalue_3 _returnvalue_2 _client_uid))
  (bind _returnvalue_8 (select _returnvalue_6 _returnvalue _client_uid_2))
  ;[1 1 1] SynchroCharacterSelection
  (Default|SynchronizeCharacterSelection (.AsBP%20Menu%20Player%20Controller (Utilities|Casting|CastToBP_MenuPlayerController (Game|GetPlayerController 0))) _returnvalue_4 _returnvalue_5 _returnvalue_8 _returnvalue_7)
  (Default|SynchronizeCharacterSelection (.AsBP%20Menu%20Player%20Controller (Utilities|Casting|CastToBP_MenuPlayerController (Game|GetPlayerController 1))) _returnvalue_4 _returnvalue_5 _returnvalue_8 _returnvalue_7)
  (Development|PrintText (Utilities|Text|FormatText "Pantin {pantin} ; {pantinP} ; Animator {animator} ; {animatorP}" _returnvalue_4 (Variables|Default|GetPantinPlayer) _returnvalue_5 (Variables|Default|GetAnimatorPlayer)) false false))

(event Custom|SelectionButton
  (params (ClickPantin :type Boolean) (IsP1 :type Boolean))
  (bind _returnvalue (Math|Integer|SelectInt 1 2 IsP1))
  (bind _returnvalue_2 (Math|Integer|SelectInt 1 2 IsP1))
  ;[1 1 1] SelectionButton
  (if ClickPantin
    (if (== (Variables|Default|GetPantinPlayer) -1)
      (Variables|Default|SetPantinPlayer _returnvalue_2)
      (if (== _returnvalue_2 (Variables|Default|GetAnimatorPlayer))
        (Variables|Default|SetAnimatorPlayer -1))
      (elif (== _returnvalue_2 (Variables|Default|GetPantinPlayer))
        (Variables|Default|SetPantinPlayer -1)))
    (elif (== (Variables|Default|GetAnimatorPlayer) -1)
      (Variables|Default|SetAnimatorPlayer _returnvalue)
      (if (== _returnvalue (Variables|Default|GetPantinPlayer))
        (Variables|Default|SetPantinPlayer -1))
      (elif (== _returnvalue (Variables|Default|GetAnimatorPlayer))
        (Variables|Default|SetAnimatorPlayer -1))))
  (CallFunction|SynchroCharacterSelection))

(fn ConstructionScript)