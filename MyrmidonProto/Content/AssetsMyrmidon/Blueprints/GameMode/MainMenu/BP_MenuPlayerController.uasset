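; Player controller for the main menu and two-player online lobby, covering host/join, character selection and game launch.
; Creates and switches the menu widgets, propagates language changes, and manages session hosting and joining.
; Relays ready and selection choices to BP_MenuGameMode, receives lobby sync, and triggers both controllers on start and launch.
; Turns Enhanced Input and mouse movement into menu navigation calls, quantizing stick input into four throttled directions.
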(event Custom|OpenMainMenu
  ;[1 1 1] OpenMainMenu
  (Default|MainMenuOpen (Variables|Default|GetMainMenu))
  (Widget|SetVisibility (Variables|Default|GetSettings) "Hidden")
  (Widget|SetVisibility (Variables|Default|GetAlbum) "Hidden")
  (Widget|SetVisibility (Variables|Default|GetHost) "Hidden")
  (Widget|SetVisibility (Variables|Default|GetJoin) "Hidden")
  (Default|InitFocus (Variables|Default|GetMainMenu)))

(event Custom|SynchronizeCharacterSelection
  (params (P1Choice :type Integer) (P2Choice :type Integer) (ShowReady :type Boolean) (ShowLanchGame :type Boolean))
  ;[1 1 1] SynchronizeCharacterSelection
  (Default|Synchronize (Variables|Default|GetCharacterSelect) P1Choice P2Choice ShowReady ShowLanchGame))

(event Custom|JoinLobby
  (params (LobbyInfo :type Blueprint%20Session%20Result%20Structure))
  ;[1 1 1] JoinLobby
  (if (not (Variables|Default|GetIsJoining))
    (CallFunction|Joining true)
    (Development|PrintString "Truely joining")
    (|JoinSession self LobbyInfo
      (:OnFailure
        (CallFunction|Joining false)
        (Development|PrintString "Failled to join")))))

(event Custom|OpenCharacterSelection
  (bind _characterselect (Variables|Default|GetCharacterSelect))
  ;[1 1 1] OpenCharacterSelection
  (Widget|SetVisibility (Variables|Default|GetMainMenu) "Hidden")
  (Widget|SetVisibility _characterselect "Visible")
  (Default|CloseCharaSelect _characterselect)
  (Default|InitFocus _characterselect))

(event Custom|InputMapping
  ;[1 1 1] InputMapping
  (if (and (Pawn|IsLocalController) (Utilities|IsValid (PlayerController|LocalPlayerSubsystems|GetEnhancedInputLocalPlayerSubsystem)))
    (Input|AddMappingContext (PlayerController|LocalPlayerSubsystems|GetEnhancedInputLocalPlayerSubsystem) "/Game/AssetsMyrmidon/Inputs/IMC_MainMenu.IMC_MainMenu" 0 "(bIgnoreAllPressedKeysUntilRelease=True,bForceImmediately=False,bNotifyUserSettings=False)")))

(event Custom|SetupMainMenu
  (bind _mainmenu (Variables|Default|GetMainMenu))
  ;[1 1 1] SetupMainMenu
  (EventDispatchers|BindEventtoOnUpdateLanguage (.GameInstance (CallFunction|GetBPGameInstance)) (delegate Custom|OnLanguageUpdated))
  (CallFunction|Setup)
  (EventDispatchers|BindEventtoOnHost _mainmenu (delegate Custom|OpenHost))
  (EventDispatchers|BindEventtoOnJoin _mainmenu (delegate Custom|OpenJoin))
  (EventDispatchers|BindEventtoOnSettings _mainmenu (delegate Custom|OpenSettings))
  (EventDispatchers|BindEventtoOnAlbums _mainmenu (delegate Custom|OpenAlbum))
  (CallFunction|OpenMainMenu))

(event Custom|PlayerJoined
  (params (UniqueID :type String))
  (Default|PlayerJoined (.AsBP%20Menu%20Game%20Mode (Utilities|Casting|CastToBP_MenuGameMode (Game|GetGameMode))) UniqueID)
  (CallFunction|AskSychro))

(event Custom|AskSychro
  ;[1 1 1] Sychro
  (Default|Sychro (.AsBP%20Menu%20Game%20Mode (Utilities|Casting|CastToBP_MenuGameMode (Game|GetGameMode)))))

(event Custom|AskStartGame
  ;[1 1 1] AskStartGame
  (CallFunction|PreStartGameOwning (.AsBP%20Menu%20Player%20Controller (Utilities|Casting|CastToBP_MenuPlayerController (Game|GetPlayerController 0))))
  (CallFunction|PreStartGameOwning (.AsBP%20Menu%20Player%20Controller (Utilities|Casting|CastToBP_MenuPlayerController (Game|GetPlayerController 1))))
  (CallFunction|StartGame))

(event Custom|StartGame
  ;[1 1 1] AskStartGame
  (Variables|/Game/AssetsMyrmidon/Blueprints/GameMode/BP_GameInstance.BP_GameInstance_C|SetPlayerQuantity (.GameInstance (CallFunction|GetBPGameInstance)) (Class|GameplayStatics|GetNumPlayerControllers)))

(event Custom|PreStartGameOwning
  ;[1 1 1] AskStartGame
  (Default|PreStartGame (Variables|Default|GetHost))
  (CallFunction|OpenCharacterSelection))

(event Custom|OpenJoin
  (bind _self self)
  ;[1 1 1] OpenJoin
  (Default|MainMenuClosed (Variables|Default|GetMainMenu))
  (Widget|SetVisibility (Variables|Default|GetJoin) "Visible")
  (Default|SetTimer (Variables|/Game/AssetsMyrmidon/Blueprints/UI/MainMenu/WBP_Join.WBP_Join_C|GetWBP_LobbyList (Variables|Default|GetJoin)))
  (Default|InitFocus (Variables|Default|GetJoin))
  (|DestroySession _self
    (:then
      (|EndSession _self))))

(event Custom|CloseMainMenu
  (bind _mainmenu (Variables|Default|GetMainMenu))
  ;[1 1 1] CloseMainMenu
  (EventDispatchers|UnbindallEventsfromOnHost _mainmenu)
  (EventDispatchers|UnbindallEventsfromOnJoin _mainmenu)
  (EventDispatchers|UnbindallEventsfromOnSettings _mainmenu)
  (Widget|RemovefromParent _mainmenu))

(event Custom|CreateHost
  ;[1 1 1] CreateHost
  (bind _returnvalue (UserInterface|CreateWidget "/Game/AssetsMyrmidon/Blueprints/UI/MainMenu/WBP_Host.WBP_Host_C" self))
  (bind _output_get (Variables|Default|SetHost _returnvalue))
  (UserInterface|Viewport|AddtoViewport _output_get 0)
  (Widget|SetVisibility _output_get "Hidden"))

(event Custom|P2Multicast
  ;[1 1 1] Event BeginPlay
  (Variables|Default|SetIsP1 false))

(event Custom|OpenSettings
  (bind _settings (Variables|Default|GetSettings))
  ;[1 1 1] OpenSettings
  (Default|MainMenuClosed (Variables|Default|GetMainMenu))
  (Widget|SetVisibility _settings "Visible")
  (CallFunction|Focus _settings (Variables|/Game/AssetsMyrmidon/Blueprints/UI/MainMenu/WBP_Settings.WBP_Settings_C|GetCB_Language _settings)))

(event Custom|P2Server
  ;[1 1 1] Event BeginPlay
  (CallFunction|P2Multicast))

(event Custom|ClickedOnSelectionButtonServer
  (params (ClickPantin :type Boolean))
  ;[1 1 1] ClickedOnSelectionButtonServer
  (Default|SelectionButton (.AsBP%20Menu%20Game%20Mode (Utilities|Casting|CastToBP_MenuGameMode (Game|GetGameMode))) ClickPantin (Variables|Default|GetIsP1)))

(event Custom|Synchro
  (params (P1 :type String) (P2 :type String) (Is2P :type Boolean) (IsP2 :type Boolean))
  ;[1 1 1] Sychro
  (Default|Synchro (Variables|Default|GetHost) P1 P2 Is2P IsP2))

(event Custom|LaunchGameServer
  (bind _gameinstance (CallFunction|GetBPGameInstance))
  ;[1 1 1] LaunchGame
  (CallFunction|PreLaunchGameOwning (.AsBP%20Menu%20Player%20Controller (Utilities|Casting|CastToBP_MenuPlayerController (Game|GetPlayerController 0))))
  (CallFunction|PreLaunchGameOwning (.AsBP%20Menu%20Player%20Controller (Utilities|Casting|CastToBP_MenuPlayerController (Game|GetPlayerController 1))))
  (Variables|/Script/MyrmidonProto.RecordingGameInstance|SetIsPantin _gameinstance (Utilities|Enum|Equal(Enum) (Variables|/Script/MyrmidonProto.MenuGameModeBase|GetPlayer1Choice (.AsBP%20Menu%20Game%20Mode (Utilities|Casting|CastToBP_MenuGameMode (Game|GetGameMode)))) "Pantin"))
  (Default|TraveltoScene _gameinstance (Variables|Default|GetStartLevel)))

(event Custom|PreLaunchGameOwning
  (bind _characterselect (Variables|Default|GetCharacterSelect))
  ;[1 1 1] LaunchGame
  (Utilities|IsValid _characterselect
    (:Is%20Valid
      (Default|PreLaunchGame _characterselect))))

(event Custom|PlayerReady
  (params (PlayerReady :type Boolean))
  (Default|PlayerReady (.AsBP%20Menu%20Game%20Mode (Utilities|Casting|CastToBP_MenuGameMode (Game|GetGameMode))) PlayerReady (Variables|Default|GetIsP1)))

(event Custom|SyncReady
  (params (Ready :type Boolean) (LaunchGame :type Boolean))
  (Default|SetReady (Variables|Default|GetCharacterSelect) Ready)
  (Default|EnableLaunchGame (Variables|Default|GetCharacterSelect) LaunchGame))

(event Custom|OpenHost
  ;[1 1 1] OpenHost
  (Default|MainMenuClosed (Variables|Default|GetMainMenu))
  (Widget|SetVisibility (Variables|Default|GetHost) "Visible")
  (Default|ShowGameButtons (Variables|Default|GetHost) false)
  (Default|InitFocus (Variables|Default|GetHost))
  (Networking|SwitchHasAuthority
    (:Authority
      (Default|CreateMenuSession (.AsBP%20Game%20Instance (Utilities|Casting|CastToBP_GameInstance (Game|GetGameInstance))))
      (CallFunction|AskSychro))))

(event Custom|OnLanguageUpdated
  (params (NewLanguage :type ELanguages%20Enum :default "French"))
  ;[1 1 1] OnLanguageUpdated
  (Class|LanguageDependent|SetLanguage (Variables|Default|GetMainMenu) NewLanguage)
  (Class|LanguageDependent|SetLanguage (Variables|Default|GetSettings) NewLanguage)
  (Class|LanguageDependent|SetLanguage (Variables|Default|GetHost) NewLanguage)
  (Default|SetLanguage (Variables|Default|GetJoin) NewLanguage)
  (Default|SetLanguage (Variables|Default|GetAlbum) NewLanguage)
  (Class|LanguageDependent|SetLanguage (Variables|Default|GetCharacterSelect) NewLanguage))

(event Custom|Focus
  (params (WidgetToFocus :type Widget%20Object%20Reference) (Target :type Widget%20Object%20Reference))
  ;[1 1 1] Focus
  (Input|SetInputModeGameandUI self Target "DoNotLock" true false)
  (Utilities|FlowControl|Delay 0.2)
  (Widget|SetKeyboardFocus Target))

(event Custom|Joining
  (params (Value :type Boolean))
  ;[1 1 1] Joining
  (bind _output_get (Variables|Default|SetIsJoining Value))
  (Default|SetReturnEnable (Variables|Default|GetJoin) (not _output_get)))

(event Custom|CreateJoin
  ;[1 1 1] CreateJoin
  (bind _returnvalue (UserInterface|CreateWidget "/Game/AssetsMyrmidon/Blueprints/UI/MainMenu/WBP_Join.WBP_Join_C" self))
  (bind _output_get (Variables|Default|SetJoin _returnvalue))
  (UserInterface|Viewport|AddtoViewport _output_get 0)
  (Widget|SetVisibility _output_get "Hidden")
  (EventDispatchers|BindEventtoOnLobbyJoined (Variables|/Game/AssetsMyrmidon/Blueprints/UI/MainMenu/WBP_Join.WBP_Join_C|GetWBP_LobbyList _output_get) (delegate Custom|JoinLobby)))

(event Custom|OpenAlbum
  (bind _album (Variables|Default|GetAlbum))
  ;[1 1 1] OpenAlbum
  (Default|MainMenuClosed (Variables|Default|GetMainMenu))
  (Widget|SetVisibility _album "Visible")
  (Default|InitFocus _album))

(event Custom|Setup
  ;[1 1 1] Setup
  (CallFunction|CreateMainMenu)
  (CallFunction|CreateAlbum)
  (CallFunction|CreateSettings)
  (CallFunction|CreateHost)
  (CallFunction|CreateJoin)
  (CallFunction|CreateCharacterSelect)
  (Default|UpdateLanguage (.GameInstance (CallFunction|GetBPGameInstance))))

(event Custom|CreateMainMenu
  ;[1 1 1] CreateMainMenu
  (bind _returnvalue (UserInterface|CreateWidget "/Game/AssetsMyrmidon/Blueprints/UI/MainMenu/WBP_MainMenu.WBP_MainMenu_C" self))
  (bind _output_get (Variables|Default|SetMainMenu _returnvalue))
  (UserInterface|Viewport|AddtoViewport _output_get 0)
  (Input|SetInputModeUIOnly self (Variables|Default|GetMainMenu) "DoNotLock" false)
  (Variables|/Script/Engine.PlayerController|SetbShowMouseCursor self true))

(event Custom|CreateAlbum
  ;[1 1 1] CreateAlbum
  (bind _returnvalue (UserInterface|CreateWidget "/Game/AssetsMyrmidon/Blueprints/UI/MainMenu/WBP_Album.WBP_Album_C" self))
  (bind _output_get (Variables|Default|SetAlbum _returnvalue))
  (UserInterface|Viewport|AddtoViewport _output_get 0)
  (Widget|SetVisibility _output_get "Hidden"))

(event Custom|CreateSettings
  ;[1 1 1] CreateSettings
  (bind _returnvalue (UserInterface|CreateWidget "/Game/AssetsMyrmidon/Blueprints/UI/MainMenu/WBP_Settings.WBP_Settings_C" self))
  (bind _output_get (Variables|Default|SetSettings _returnvalue))
  (UserInterface|Viewport|AddtoViewport _output_get 0)
  (Widget|SetVisibility (Variables|Default|GetSettings) "Hidden"))

(event Custom|CreateCharacterSelect
  ;[1 1 1] CreateCharacterSelect
  (bind _returnvalue (UserInterface|CreateWidget "/Game/AssetsMyrmidon/Blueprints/UI/MainMenu/WBP_SelectCharacter.WBP_SelectCharacter_C" self))
  (bind _output_get (Variables|Default|SetCharacterSelect _returnvalue))
  (UserInterface|Viewport|AddtoViewport _output_get 0)
  (Widget|SetVisibility _output_get "Hidden"))

(event Custom|P2Owning
  ;[1 1 1] Event BeginPlay
  (CallFunction|P2Server))

(event Input|EnhancedActionEvents|EnhancedInputActionIA_Return
  (params (ActionValue :type Boolean) (ElapsedSeconds :type Float%20%28double-precision%29) (TriggeredSeconds :type Float%20%28double-precision%29) (InputAction :type Input%20Action%20Object%20Reference :default "/Game/AssetsMyrmidon/Inputs/IA_Return.IA_Return"))
  ;[1 1 1] IA_Return
  (:Completed
    (Default|CallReturnButton)))

(event Input|EnhancedActionEvents|EnhancedInputActionIA_Move
  (params (ActionValue :type Vector%202D%20Structure) (ElapsedSeconds :type Float%20%28double-precision%29) (TriggeredSeconds :type Float%20%28double-precision%29) (InputAction :type Input%20Action%20Object%20Reference :default "/Game/AssetsMyrmidon/Inputs/IA_Move.IA_Move"))
  ;[1 1 1] Move
  (if (Variables|Default|GetCanUseInputs)
    (bind _valid (CallFunction|Identify2DInputs ActionValue))
    (if _valid
      (Variables|Default|SetCanUseInputs false)
      (Utilities|FlowControl|Delay (Variables|Default|GetDelayBetweenInputs))
      (Variables|Default|SetCanUseInputs true))))

(event Input|EnhancedActionEvents|EnhancedInputActionIA_Action
  (params (ActionValue :type Boolean) (ElapsedSeconds :type Float%20%28double-precision%29) (TriggeredSeconds :type Float%20%28double-precision%29) (InputAction :type Input%20Action%20Object%20Reference :default "/Game/AssetsMyrmidon/Inputs/IA_Action.IA_Action"))
  ;[1 1 1] IA_Action
  (:Started
    (Default|CallValidate)))

(event Input|EnhancedActionEvents|EnhancedInputActionIA_LookAt
  (params (ActionValue :type Vector%202D%20Structure) (ElapsedSeconds :type Float%20%28double-precision%29) (TriggeredSeconds :type Float%20%28double-precision%29) (InputAction :type Input%20Action%20Object%20Reference :default "/Game/AssetsMyrmidon/Inputs/IA_LookAt.IA_LookAt"))
  ;[1 1 1] IA_LookAt
  (:Triggered
    (Default|CallLookat :!label _label))
  (:Started
    (goto _label))
  (:Ongoing
    (goto _label)))

(event EventBeginPlay
  ;[1 1 1] Event BeginPlay
  (CallFunction|InputMapping)
  (Variables|Default|SetIsP1 (Ability|HasAuthority))
  (Networking|SwitchHasAuthority
    (:Authority
      (CallFunction|AskSychro))
    (:Remote
      (Development|PrintString "PLAYER JOINED !" true true "(R=0.250000,G=0.022263,B=0.000000,A=1.000000)" 25.0)
      (CallFunction|SetupMainMenu)
      (CallFunction|OpenHost)
      (CallFunction|PlayerJoined (Class|AdvancedSessionsLibrary|UniqueNetIdtoString (Class|AdvancedSteamFriendsLibrary|GetLocalSteamIDfromSteam)))
      (CallFunction|P2Owning))))

(event EventTick
  (params (DeltaSeconds :type Float%20%28single-precision%29))
  (bind (_locationx _locationy) (Game|Player|GetMousePosition))
  (bind _returnvalue (Math|Vector2D|MakeVector2D _locationx _locationy))
  ;[1 1 1] Event Tick check mouse pos
  (if (Class|KismetMathLibrary|EqualExactlyVector2DVector2D _returnvalue (Variables|Default|GetLastPos))
    _
    (else
      (Default|CallLookat)))
  (Variables|Default|SetLastPos _returnvalue))

(fn ConstructionScript)

(fn Identify2DInputs
  (params (Inputs :type Vector%202D%20Structure))
  (bind _returnvalue (Math|Vector2D|Normalize2D Inputs))
  (if (> (Math|Vector2D|Vector2DLength Inputs) 0.6)
    (if (Math|Float|NearlyEqual(Float) (Math|Vector2D|DotProduct(2D) _returnvalue "(X=1.000000,Y=0.000000)") 1.0 (LocalVariables|GetErrorTolerance))
      (Default|CallAnyDirection "Up")
      (return true)
      (elif (Math|Float|NearlyEqual(Float) (Math|Vector2D|DotProduct(2D) _returnvalue "(X=1.000000,Y=0.000000)") -1.0 (LocalVariables|GetErrorTolerance))
        (Default|CallAnyDirection "Down")
        (return true)
        (elif (Math|Float|NearlyEqual(Float) (Math|Vector2D|DotProduct(2D) _returnvalue "(X=0.000000,Y=1.000000)") 1.0 (LocalVariables|GetErrorTolerance))
          (Default|CallAnyDirection "Right")
          (return true)
          (elif (Math|Float|NearlyEqual(Float) (Math|Vector2D|DotProduct(2D) _returnvalue "(X=0.000000,Y=1.000000)") -1.0 (LocalVariables|GetErrorTolerance))
            (Default|CallAnyDirection "Left")
            (return true)
            (else
              _))))))
  (return false))