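; BP_LobbyController is the lobby player controller for up to two players, handling Pantin role assignment, map selection and departure to the chosen scene.
; Server-named events relay changes to player controllers 0 and 1, which update their lobby HUD and the Game Instance's IsPantin flag.
; It notifies BP_LobbyGameMode on BeginPlay and re-applies map and role values on join.
; Departure events remove HUD buttons, fade to black, store player count and travel through the Game Instance.
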(event Custom|SetHUD
  (params (Hud :type WBP%20Lobby%20Object%20Reference))
  ;[1 1 1] Set HUD
  (Variables|Default|SetHud Hud))

(event Custom|SetMapIndexServer
  (params (index :type Integer))
  ;[1 1 1] SetMapIndex
  (CallFunction|SetMapIndexAll (.AsBP%20Lobby%20Controller (Utilities|Casting|CastToBP_LobbyController (Game|GetPlayerController 0))) index)
  (bind _asbp_lobby_controller (Utilities|Casting|CastToBP_LobbyController (Game|GetPlayerController 1)))
  (CallFunction|SetMapIndexAll _asbp_lobby_controller index))

(event Custom|UpdateValuesOnJoinOwning
  (params (Index :type Integer) (P1IsPantin :type Boolean))
  ;[1 1 1] UpdateValuesOnJoinOwning
  (CallFunction|SetMapIndexServer Index)
  (CallFunction|SetIsPantinServer P1IsPantin))

(event Custom|SetIsPantinServer
  (params (P1IsPantin :type Boolean))
  ;[1 1 1] SwitchPlayersServer
  (CallFunction|SetIsPantin (.AsBP%20Lobby%20Controller (Utilities|Casting|CastToBP_LobbyController (Game|GetPlayerController 0))) P1IsPantin)
  (bind _asbp_lobby_controller (Utilities|Casting|CastToBP_LobbyController (Game|GetPlayerController 1)))
  (CallFunction|SetIsPantin _asbp_lobby_controller P1IsPantin))

(event Custom|SetMapIndexLocal
  (params (Index :type Integer))
  ;[1 1 1] SetMapIndex
  (Default|SetMapIndex (Variables|Default|GetHud) Index))

(event Custom|set%20isPantin
  (params (isPantin :type Boolean))
  ;[1 1 1] set isPantin
  (bind _output_get (Variables|/Game/AssetsMyrmidon/Blueprints/GameMode/BP_GameInstance.BP_GameInstance_C|SetisPantin (.GameInstance (CallFunction|GetBPGameInstance)) isPantin))
  (Default|SetIsPantin (Variables|BP_LobbyController_C|GetHud (.AsBP%20Lobby%20Controller (Utilities|Casting|CastToBP_LobbyController (Game|GetPlayerController 0)))) _output_get))

(event Custom|SetMapIndexAll
  (params (Index :type Integer))
  ;[1 1 1] SetMapIndex
  (CallFunction|SetMapIndexLocal (.AsBP%20Lobby%20Controller (Utilities|Casting|CastToBP_LobbyController (Game|GetPlayerController 0))) Index))

(event Custom|RemoveButtonsServer
  ;[1 1 1] RemoveButtons
  (CallFunction|RemoveButtonsOwning (.AsBP%20Lobby%20Controller (Utilities|Casting|CastToBP_LobbyController (Game|GetPlayerController 0))))
  (bind _asbp_lobby_controller (Utilities|Casting|CastToBP_LobbyController (Game|GetPlayerController 1)))
  (CallFunction|RemoveButtonsOwning _asbp_lobby_controller))

(event Custom|RemoveButtonsOwning
  ;[1 1 1] RemoveButtons
  (Default|RemoveButton (Variables|Default|GetHud))
  (bind _returnvalue (UserInterface|CreateWidget "/Game/AssetsMyrmidon/Blueprints/UI/WBP_BlackScreen.WBP_BlackScreen_C" self))
  (UserInterface|Viewport|AddtoViewport _returnvalue 0)
  (Default|FadetoBlack _returnvalue))

(event Custom|SwitchPlayersServer
  (bind _gameinstance (CallFunction|GetBPGameInstance))
  (bind _ispantin (Variables|/Game/AssetsMyrmidon/Blueprints/GameMode/BP_GameInstance.BP_GameInstance_C|GetisPantin _gameinstance))
  (bind _returnvalue (not _ispantin))
  ;[1 1 1] SwitchPlayersServer
  (CallFunction|SetIsPantin (.AsBP%20Lobby%20Controller (Utilities|Casting|CastToBP_LobbyController (Game|GetPlayerController 0))) _returnvalue)
  (bind _asbp_lobby_controller (Utilities|Casting|CastToBP_LobbyController (Game|GetPlayerController 1)))
  (CallFunction|SetIsPantin _asbp_lobby_controller (not _returnvalue)))

(event Custom|PlayerJoinServer
  ;[1 1 1] BeginPlay
  (Default|PlayerJoined (.AsBP%20Lobby%20Game%20Mode (Utilities|Casting|CastToBP_LobbyGameMode (Game|GetGameMode)))))

(event Custom|TravelToSceneServer
  (params (SceneName :type String))
  (bind _gameinstance (CallFunction|GetBPGameInstance))
  ;[1 1 1] TravelToSceneServer
  (bind _output_get (Variables|/Game/AssetsMyrmidon/Blueprints/GameMode/BP_GameInstance.BP_GameInstance_C|SetPlayerQuantity _gameinstance (Class|GameplayStatics|GetNumPlayerControllers)))
  (Development|PrintString (Utilities|String|ToString(Integer) _output_get))
  (Default|TraveltoScene _gameinstance SceneName))

(event EventBeginPlay
  ;[1 1 1] BeginPlay
  (CallFunction|PlayerJoinServer))

(fn ConstructionScript)