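; Game mode for a two-role game that assigns a Pantin and an Animateur once all expected players have loaded.
; A Game Instance flag maps roles to player controllers, each initialized at a tagged PlayerStart.
; The Pantin spawns or respawns at its checkpoint index, falling back to checkpoint zero.
; It also relays animator moves, triggers controller recording and replay, and broadcasts wind state to Windable actors.
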(event Custom|OnPlayerJoin
  (bind _gameinstance (CallFunction|GetBPGameInstance))
  (bind _playersspawned (Variables|Default|GetPlayersSpawned))
  (bind _playerquantity (Variables|/Game/AssetsMyrmidon/Blueprints/GameMode/BP_GameInstance.BP_GameInstance_C|GetPlayerQuantity _gameinstance))
  ;[1 1 1] OnPlayerJoin
  (Math|Integer|IncrementInt (Variables|Default|GetPlayersSpawned)
    (:%20%20
      (bind _returnvalue (Class|GameModeBase|GetNumPlayers))
      (Development|PrintString (Utilities|String|ToString(Text) (Utilities|Text|FormatText "{v1} / {v2} players have loaded" _playersspawned _playerquantity)) true true "(R=0.000000,G=0.660000,B=1.000000,A=1.000000)" 1e+01)
      (if (== _playerquantity _playersspawned)
        (bind _output_get (Variables|Default|SetPlayers _returnvalue))
        (Development|PrintString (Utilities|String|ToString(Integer) _output_get) true true "(R=1.000000,G=0.360171,B=0.000000,A=1.000000)" 2e+01)
        (Utilities|FlowControl|Sequence
          (:then_0
            (Variables|Default|SetP0IsPantin (Variables|/Game/AssetsMyrmidon/Blueprints/GameMode/BP_GameInstance.BP_GameInstance_C|GetisPantin (.GameInstance (CallFunction|GetBPGameInstance))))
            (CallFunction|SetPantinPlayer))
          (:then_1
            (CallFunction|SetAnimateurPlayer)))))))

(event Custom|SetPantinPlayer
  (bind _playercontroller (CallFunction|GetBPPlayerController true))
  ;[1 1 1] SetPantinPlayer
  (Utilities|FlowControl|DoOnce false
    (:Completed
      (if (CallFunction|IsPlayerPresent true)
        (Variables|/Script/MyrmidonProto.PantinAnimatorPlayerState|SetIsPantin (.PlayerState (Default|GetPlayerState _playercontroller)) true)
        (bind _playerstarttransform (CallFunction|GetPlayerStartInfo true))
        (Default|InitPantin _playercontroller _playerstarttransform)
        (else
          (Development|PrintString "Pantin MISSING" true true "(R=1.000000,G=0.029373,B=0.000000,A=1.000000)" 1e+01))))))

(event Custom|SetAnimateurPlayer
  ;[1 1 1] SetAnimateurPlayer
  (Utilities|FlowControl|DoOnce false
    (:Completed
      (if (CallFunction|IsPlayerPresent false)
        (bind _playerstarttransform (CallFunction|GetPlayerStartInfo false))
        (Default|InitAnimateur (CallFunction|GetBPPlayerController false) _playerstarttransform)
        (CallFunction|StartTestRecord)
        (else
          (Development|PrintString "Animator MISSING" true true "(R=1.000000,G=0.088168,B=0.000000,A=1.000000)" 1e+01))))))

(event Custom|StartTestRecord
  (bind _playercontroller (CallFunction|GetBPPlayerController true))
  (bind _playercontroller_2 (CallFunction|GetBPPlayerController false))
  ;[1 1 1] StartTestRecord
  (Utilities|FlowControl|Sequence
    (:then_0
      (Utilities|IsValid _playercontroller
        (:Is%20Valid
          (Default|StartTestRecord _playercontroller))))
    (:then_1
      (Utilities|IsValid _playercontroller_2
        (:Is%20Valid
          (Default|StartTestRecord _playercontroller_2))))))

(event Custom|AnimatorShouldMoveTo
  (params (Rotation :type Rotator) (Position :type Vector))
  ;[1 1 1] AnimatorShouldMoveTo
  (Default|AnimatorMoveto (CallFunction|GetBPPlayerController false) Rotation Position))

(event Custom|StartReplay
  (bind _playercontroller (CallFunction|GetBPPlayerController true))
  (bind _playercontroller_2 (CallFunction|GetBPPlayerController false))
  ;[1 1 1] StartReplay
  (if (CallFunction|IsPlayerPresent true)
    (Default|StopRecording _playercontroller))
  (if (CallFunction|IsPlayerPresent false)
    (Default|StopRecording _playercontroller_2))
  (Utilities|FlowControl|Sequence
    (:then_0
      (if (CallFunction|IsPlayerPresent true)
        (Default|StartReplaying _playercontroller 0.0)))
    (:then_1
      (if (CallFunction|IsPlayerPresent false)
        (Default|StartReplaying _playercontroller_2 0.0)))))

(event Custom|SetWindActive
  (params (Active :type Boolean) (Direction :type Vector))
  ;[1 1 1] SetWindActive
  (Variables|Default|SetWindDirection Direction)
  (Variables|Default|SetWindIsActive Active)
  (bind _outactors (Actor|GetAllActorswithInterface "/Script/MyrmidonProto.Windable"))
  (for _array_element _outactors
    (Class|Windable|SetActiveWind(Message) _array_element (Variables|Default|GetWindIsActive))
    (Class|Windable|SetWindDirection(Message) _array_element (Variables|Default|GetWindDirection))))

(fn ConstructionScript)

(fn GetBPPlayerController
  (params (GetPantin :type Boolean))
  (return (.AsBP%20Player%20Controller (Utilities|Casting|CastToBP_PlayerController (Game|GetPlayerController (Math|Integer|SelectInt 0 1 (not (Class|KismetMathLibrary|XORBoolean GetPantin (Variables|Default|GetP0IsPantin)))))))))

(fn GetPlayerStartInfo
  (params (Pantin :type Boolean))
  (bind _playercontroller (CallFunction|GetBPPlayerController true))
  (bind _pantintag (Variables|Default|GetPantinTag))
  (bind _playerstate (Default|GetPlayerState _playercontroller))
  (bind _returnvalue (Utilities|String|ToString(Name) _pantintag))
  (bind _pantincheckpointindex (Variables|/Script/MyrmidonProto.PantinAnimatorPlayerState|GetPantinCheckPointIndex _playerstate))
  (bind _returnvalue_2 (Utilities|String|ToString(Integer) _pantincheckpointindex))
  (bind _returnvalue_3 (Utilities|String|Append _returnvalue _returnvalue_2))
  (LocalVariables|SetSpawnFound false)
  (bind _outactors (Actor|GetAllActorsOfClass "/Script/Engine.PlayerStart"))
  (for _array_element _outactors
    (if (CallFunction|IsPlayerPresent true)
      (if (== (Variables|/Script/Engine.PlayerStart|GetPlayerStartTag _array_element) (select Pantin (Utilities|String|StringToName _returnvalue_3) (Variables|Default|GetAnimatorTag)))
        (LocalVariables|SetLocalTransform (Math|Transform|MakeTransform (.Location (Math|Transform|BreakTransform (Transformation|GetActorTransform _array_element))) (.Rotation (Math|Transform|BreakTransform (Transformation|GetActorTransform _array_element)))) :!label _label)
        (LocalVariables|SetSpawnFound true))
      (elif (== (Variables|/Script/Engine.PlayerStart|GetPlayerStartTag _array_element) (Variables|Default|GetAnimatorTag))
        (goto _label))))
  (if (and (not (LocalVariables|GetSpawnFound)) Pantin)
    (Development|PrintString (Utilities|String|ToString(Text) (Utilities|Text|FormatText "CheckPoint : {Name} NOT FOUND" _returnvalue_3)) true true "(R=0.437500,G=0.063242,B=0.000000,A=1.000000)" 1e+01)
    (for _array_element_2 _outactors
      (if (== (Variables|/Script/Engine.PlayerStart|GetPlayerStartTag _array_element_2) (Utilities|String|StringToName (Utilities|String|Append (Utilities|String|ToString(Name) (Variables|Default|GetPantinTag)) (Utilities|String|ToString(Integer) 0))))
        (LocalVariables|SetLocalTransform (Math|Transform|MakeTransform (.Location (Math|Transform|BreakTransform (Transformation|GetActorTransform _array_element_2))) (.Rotation (Math|Transform|BreakTransform (Transformation|GetActorTransform _array_element_2)))))))
    (return (LocalVariables|GetLocalTransform))
    (else
      (return (LocalVariables|GetLocalTransform)))))

(fn IsPlayerPresent
  (params (Pantin :type Boolean))
  (return (or (== (Variables|Default|GetPlayers) 2) (== Pantin (Variables|Default|GetP0IsPantin)))))

(fn GetRespawnPos
  (bind _playerstarttransform (CallFunction|GetPlayerStartInfo true))
  (return _playerstarttransform))