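; BP_Pantin is the player character, with camera-relative movement, 2D and vertical-only modes, jumping, ledge climbing and action-object interaction.
; Tick extends the spring arm with speed, using traces to avoid obstructions, and updates any 2D-zone camera.
; Traces find ledge space during falls, then a timeline climbs in two passes, up then across.
; Jumps vary gravity scale, and debug-toggled wind applies force weakened by upwind trace hits.
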(event Custom|SetCameraAngleOffset
  (params (angle :type Float%20%28double-precision%29))
  ;[1 1 1] SetCameraAngleOffset
  (Pawn|Input|AddControllerYawInput (/ (+ (* (.Yaw (Math|Rotator|BreakRotator (Pawn|GetControlRotation :!class /Script/Engine.Pawn))) -1.0) angle) (Class|PlayerController|GetDeprecatedInputYawScale (Game|GetPlayerController 0)))))

(event Custom|UpdateSpeedPercent
  ;[1 1 1] UpdateSpeedPercent
  (Variables|SpringArmLength|SetSpeedPercent (/ (Math|Vector|VectorLength (Transformation|GetVelocity)) (Class|MovementComponent|GetMaxSpeed (Variables|Character|GetCharacterMovement)))))

(event Custom|WindDebug
  ;[1 1 1] Wind
  (Variables|Wind|SetWindHitPoints 0.0)
  (CallFunction|LineTraceforWindDebug 0.0 2e+02 true)
  (CallFunction|LineTraceforWindDebug 5e+01 2e+02 true)
  (CallFunction|LineTraceforWindDebug -5e+01 2e+02 true))

(event Custom|WindEffect
  (params (DeltaTime :type Float%20%28double-precision%29))
  ;[1 1 1] Wind
  (Pawn|Components|CharacterMovement|ClearAccumulatedForces (Variables|Character|GetCharacterMovement))
  (Physics|AddForce (Variables|Character|GetCharacterMovement) (* (Variables|Default|GetWindDirection) (* DeltaTime (Variables|Default|GetWindPower) (/ (- (Variables|Default|GetWindMaxHit) (Variables|Wind|GetWindHitPoints)) (Variables|Default|GetWindMaxHit)) 1e+05))))

(event Custom|DisableActionInput
  ;[1 1 1] DisableActionInput
  (Variables|ActionInternal|SetActionIsPressed false)
  (if (Variables|ActionInternal|GetActionIsActive)
    (CallFunction|EndAction)))

(event Custom|EndAction
  ;[1 1 1] Action
  (Variables|ActionInternal|SetActionIsActive false)
  (bind _asbpi_action_object (Utilities|Casting|CastToBPI_ActionObject (Variables|Default|GetActionObject)))
  (Default|Deactivate _asbpi_action_object))

(event Custom|Wind
  (params (DeltaTime :type Float%20%28double-precision%29))
  ;[1 1 1] Wind
  (if (Variables|Wind|GetWindIsActive)
    (CallFunction|WindDebug)
    (CallFunction|WindEffect DeltaTime)))

(event Custom|Move
  (params (Direction :type Vector) (Cam :type BP%20Camera%20Object%20Reference))
  (bind _returnvalue (Math|Vector|VectorClampSizeMax Direction 1.0))
  (bind (_x _y _z) (Math|Vector|BreakVector _returnvalue))
  ;[1 1 1] MovePantinWithInputs
  (CallFunction|MovePantinwithInputs (Math|Vector|RotateVector (Math|Vector|SelectVector (Math|Vector|MakeVector 0.0 _y _z) _returnvalue (Variables|Default|Getin2D)) (Math|Rotator|MakeRotator 0.0 0.0 (.Yaw (Math|Rotator|BreakRotator (Transformation|GetActorRotation Cam))))) (Variables|Default|GetSpeed) false))

(event Custom|UpdateVelocity
  ;[1 1 1] Update Velocity (Not used for now)
)

(event Custom|AskEndAction
  ;[1 1 1] Action
  (CallFunction|EndAction)
  (Variables|Default|SetActionObject 0))

(event Custom|AskJump
  ;[1 1 1] AskJump
  (Utilities|IsValid (Variables|Default|GetLateralBar)
    (:Is%20Valid
      (Default|DetachPlayer (Variables|Default|GetLateralBar))
      (CallFunction|StartFunkyGravity :!label _label))
    (:Is%20Not%20Valid
      (if (Variables|ClimbInternal|GetJumpAllowed)
        (Character|Jump)
        (goto _label)))))

(event Custom|FunkyGravityTick
  (bind _charactermovement (Variables|Character|GetCharacterMovement))
  (if (Variables|Default|GetinFunkyGravity)
    (if (AI|Components|NavMovement|IsFalling (Variables|Character|GetCharacterMovement))
      (Variables|/Script/Engine.CharacterMovementComponent|SetGravityScale (Variables|Character|GetCharacterMovement) (Math|Float|Clamp(Float) (* (/ (Math|Float|Absolute(Float) (.Z (Math|Vector|BreakVector (Variables|/Script/Engine.MovementComponent|GetVelocity _charactermovement)))) (Variables|Default|GetMaxVelocity)) (Variables|Default|GetMaxGravity)) (Variables|Default|GetMinGravity) (Variables|Default|GetMaxGravity)))
      (else
        (Variables|Default|SetinFunkyGravity false)
        (Variables|/Script/Engine.CharacterMovementComponent|SetGravityScale _charactermovement (Variables|Default|GetMaxGravity))))))

(event Custom|UpdateTargetLength
  ;[1 1 1] UpdateTargetLength
  (Variables|SpringArmLength|SetTargetLength (+ (Variables|SpringArmLength|GetBaseTargetLength) (Math|Float|Lerp 0.0 (Variables|SpringArmLength|GetMaxLengthGained) (Variables|SpringArmLength|GetSpeedPercent)))))

(event Custom|StartFunkyGravity
  (Components|Timeline|SetPlayRate (Variables|Default|GetFunkyGravity) (/ 1.0 (Variables|Default|GetFunkyGravityDuration)))
  (bind _value (Timeline|FunkyGravity PlayFromStart)
    (:Update
      (Variables|/Script/Engine.CharacterMovementComponent|SetGravityScale (Variables|Character|GetCharacterMovement) (Math|Float|Lerp (Variables|Default|GetMinGravity) (Variables|Default|GetMaxGravity) _value)))))

(event Custom|ArmLengthTowardTarget
  (params (DeltaTime :type Float%20%28double-precision%29))
  (bind _returnvalue (Transformation|GetActorLocation))
  (bind _springarm (Variables|Default|GetSpringArm))
  (bind _relativelocation (Variables|/Script/Engine.SceneComponent|GetRelativeLocation _springarm))
  (bind _returnvalue_2 (+ _returnvalue _relativelocation))
  ;[1 1 1] ArmLengthTowardTarget
  (if (> (Variables|/Script/Engine.SpringArmComponent|GetTargetArmLength (Variables|Default|GetSpringArm)) (Variables|SpringArmLength|GetTargetLength))
    (Variables|SpringArmLength|SetTmpLength (Math|Float|Clamp(Float) (+ (* (Variables|SpringArmLength|GetDecelerationRate) (Variables|SpringArmLength|GetSpeedGain) -1.0 DeltaTime) (Variables|/Script/Engine.SpringArmComponent|GetTargetArmLength (Variables|Default|GetSpringArm))) (Variables|SpringArmLength|GetTargetLength) (+ (Variables|SpringArmLength|GetBaseTargetLength) (Variables|SpringArmLength|GetMaxLengthGained))))
    (else
      (Variables|SpringArmLength|SetTmpLength (Math|Float|Clamp(Float) (+ (* (Variables|SpringArmLength|GetSpeedPercent) (Variables|SpringArmLength|GetSpeedGain) DeltaTime) (Variables|/Script/Engine.SpringArmComponent|GetTargetArmLength (Variables|Default|GetSpringArm))) (Variables|SpringArmLength|GetBaseTargetLength) (Variables|SpringArmLength|GetTargetLength)))))
  (bind (_outhit _returnvalue_3) (Collision|LineTraceByChannel _returnvalue_2 (+ _returnvalue_2 (* (Math|Vector|GetForwardVector (Variables|Default|GetCameraPos)) -1.0 (Variables|SpringArmLength|GetTmpLength))) "TraceTypeQuery1" false 0 "None" :!label _label))
  (if (not _returnvalue_3)
    _
    (else
      (Variables|SpringArmLength|SetTmpLength (- (.Distance (Collision|BreakHitResult _outhit)) 2e+01))
      (bind _returnvalue_4 (Collision|MultiSphereTraceByChannel (+ (Transformation|GetActorLocation) (Variables|/Script/Engine.SceneComponent|GetRelativeLocation (Variables|Default|GetSpringArm)) (* (Math|Vector|GetForwardVector (Variables|Default|GetCameraPos)) -1.0 (Variables|SpringArmLength|GetTmpLength))) (+ (Transformation|GetActorLocation) (Variables|/Script/Engine.SceneComponent|GetRelativeLocation (Variables|Default|GetSpringArm)) (* (Math|Vector|GetForwardVector (Variables|Default|GetCameraPos)) -1.0 (Variables|SpringArmLength|GetTmpLength))) 65.0 "TraceTypeQuery1" false 0 "None" true "(R=1.000000,G=0.000000,B=0.000000,A=1.000000)" "(R=0.000000,G=1.000000,B=0.000000,A=1.000000)" 0.5 :!label _label_2))
      (if _returnvalue_4
        (Variables|SpringArmLength|SetTmpLength (- (Variables|SpringArmLength|GetTmpLength) 65.0))
        (if (> (Variables|SpringArmLength|GetTmpLength) 65.0)
          (goto _label_2)
          (else
            _))
        (else
          (goto _label)))))
  (Variables|/Script/Engine.SpringArmComponent|SetTargetArmLength (Variables|Default|GetSpringArm) (Variables|SpringArmLength|GetTmpLength)))

(event Custom|RotateTowardPantin
  (params (DeltaTime :type Float%20%28double-precision%29))
  ;[1 1 1] RotateTowardPantin
  (Variables|Default|SetTargetRotation (Math|Rotator|Lerp(Rotator) (Variables|Default|GetTargetRotation) (Transformation|GetWorldRotation (Variables|Default|GetCameraPos)) (* DeltaTime 3.0) true)))

(event Custom|UpdateSpaceToClimb
  (bind _returnvalue (Transformation|GetActorLocation))
  (bind _returnvalue_2 (Transformation|GetActorLocation))
  (bind _returnvalue_3 (Transformation|GetActorForwardVector))
  (bind _climbpantinheight (Variables|Default|GetClimbPantinHeight))
  (bind _climbpantinheight_2 (Variables|Default|GetClimbPantinHeight))
  (bind _returnvalue_4 (Math|Vector|MakeVector 0.0 0.0 _climbpantinheight_2))
  (bind _returnvalue_5 (Math|Vector|MakeVector 0.0 0.0 _climbpantinheight))
  (bind _returnvalue_6 (* _returnvalue_3 5e+01))
  (bind _returnvalue_7 (+ _returnvalue _returnvalue_4))
  (bind _returnvalue_8 (+ _returnvalue_2 _returnvalue_5))
  (bind _returnvalue_9 (+ _returnvalue_7 _returnvalue_6))
  ;[1 1 1] SpaceToClimb
  (Variables|ClimbInternal|SetSpaceToClimb false)
  (bind _returnvalue_10 (Collision|LineTraceByChannel _returnvalue_8 (+ _returnvalue_8 (* (Transformation|GetActorForwardVector) (Variables|Default|GetClimbMinArea))) "TraceTypeQuery1" false 0 (Variables|DEBUG|GetDebugClimb)))
  (if (not _returnvalue_10)
    (bind (_outhit _returnvalue_11) (Collision|LineTraceByChannel _returnvalue_9 (- _returnvalue_9 "0.000000,0.000000,60.000000") "TraceTypeQuery1" false 0 (Variables|DEBUG|GetDebugClimb) true "(R=1.000000,G=0.000000,B=0.000000,A=1.000000)" "(R=0.000000,G=1.000000,B=0.000000,A=1.000000)" 0.1))
    (if _returnvalue_11
      (Variables|ClimbInternal|SetClimbCenter (+ (.ImpactPoint (Collision|BreakHitResult _outhit)) "0.000000,0.000000,101.000000" (* (Transformation|GetActorForwardVector) 5e+01)))
      (bind _returnvalue_12 (Collision|BoxTraceByChannel (+ (.ImpactPoint (Collision|BreakHitResult _outhit)) "0.000000,0.000000,101.000000" (* (Transformation|GetActorForwardVector) 5e+01)) (+ (.ImpactPoint (Collision|BreakHitResult _outhit)) "0.000000,0.000000,101.000000" (* (Transformation|GetActorForwardVector) 5e+01)) (Math|Vector|MakeVector 5e+01 5e+01 1e+02) (Transformation|GetActorRotation) "TraceTypeQuery1" false 0 (Variables|DEBUG|GetDebugClimb)))
      (Variables|ClimbInternal|SetSpaceToClimb (not _returnvalue_12)))))

(event Custom|Climb
  ;[1 1 1] Climb
  (if (Math|Boolean|ANDBoolean (Variables|ClimbInternal|GetSpaceToClimb) (Variables|ActionInternal|GetCanMoveWithInputs) (AI|Components|NavMovement|IsFalling (Variables|Character|GetCharacterMovement)) (< (.Z (Math|Vector|BreakVector (Transformation|GetVelocity))) 0.0))
    (Variables|Wind|SetWindWasActive (Variables|Wind|GetWindIsActive))
    (Variables|Wind|SetWindIsActive false)
    (Pawn|Components|CharacterMovement|ClearAccumulatedForces (Variables|Character|GetCharacterMovement))
    (Variables|ActionInternal|SetCanMoveWithInputs false)
    (CallFunction|FreezeinAir)
    (Variables|ClimbInternal|SetClimbUp true)
    (Variables|ClimbInternal|SetClimbFirstPos (Transformation|GetActorLocation) :!label _label)
    (bind _climb (Timeline|Climbing PlayFromStart)
      (:Update
        (if (Variables|ClimbInternal|GetClimbUp)
          (Transformation|SetActorLocation (Math|Vector|Lerp(Vector) (Variables|ClimbInternal|GetClimbFirstPos) (Math|Vector|MakeVector (.X (Math|Vector|BreakVector (Variables|ClimbInternal|GetClimbFirstPos))) (.Y (Math|Vector|BreakVector (Variables|ClimbInternal|GetClimbFirstPos))) (.Z (Math|Vector|BreakVector (Variables|ClimbInternal|GetClimbCenter)))) _climb) false false)
          (else
            (Transformation|SetActorLocation (Math|Vector|Lerp(Vector) (Variables|ClimbInternal|GetClimbFirstPos) (Variables|ClimbInternal|GetClimbCenter) _climb) false false))))
      (:Finished
        (if (Variables|ClimbInternal|GetClimbUp)
          (Variables|ClimbInternal|SetClimbUp false)
          (goto _label)
          (else
            (Pawn|Components|CharacterMovement|ClearAccumulatedForces (Variables|Character|GetCharacterMovement))
            (Variables|/Script/Engine.CharacterMovementComponent|SetGravityScale (Variables|Character|GetCharacterMovement) 1.0)
            (Variables|ActionInternal|SetCanMoveWithInputs true)
            (if (Variables|Wind|GetWindWasActive)
              (Utilities|FlowControl|Delay 0.2)
              (Variables|Wind|SetWindIsActive true))))))))

(event Custom|MovePantinWithInputs
  (params (WorldDirection :type Vector) (ScaleValue :type Float%20%28double-precision%29) (IsForce :type Boolean))
  ;[1 1 1] MovePantinWithInputs
  (if (Variables|ActionInternal|GetCanMoveWithInputs)
    (if (not (Variables|Default|GetMoveOnlyUpDown))
      (Pawn|Input|AddMovementInput WorldDirection ScaleValue IsForce)
      (else
        (Variables|/Script/Engine.MovementComponent|SetVelocity (Variables|Character|GetCharacterMovement) (Math|Vector|MakeVector (.X (Math|Vector|BreakVector (Variables|/Script/Engine.MovementComponent|GetVelocity (Variables|Character|GetCharacterMovement)))) (.Y (Math|Vector|BreakVector (Variables|/Script/Engine.MovementComponent|GetVelocity (Variables|Character|GetCharacterMovement)))) (.Z (Math|Vector|BreakVector (* (Math|Vector|MakeVector 0.0 0.0 (.Y (Math|Vector|BreakVector WorldDirection))) ScaleValue (Variables|Default|GetFlightSpeed))))))))))

(event Custom|FreezeInAir
  ;[1 1 1] FreezeInAir
  (Variables|/Script/Engine.CharacterMovementComponent|SetGravityScale (Variables|Character|GetCharacterMovement) 0.0)
  (Variables|/Script/Engine.MovementComponent|SetVelocity (Variables|Character|GetCharacterMovement) "0, 0, 0"))

(event Custom|TryActivateEvent
  (bind _actionobject (Variables|Default|GetActionObject))
  (bind _asbpi_action_object (Utilities|Casting|CastToBPI_ActionObject _actionobject))
  ;[1 1 1] Action
  (if (Math|Boolean|ANDBoolean true (not (Variables|ActionInternal|GetActionIsActive)) (Utilities|IsValid (Variables|Default|GetActionObject)))
    (Default|TryActivate _asbpi_action_object)
    (bind _isactive (Default|GetIsActive _asbpi_action_object))
    (Variables|ActionInternal|SetActionIsActive _isactive)))

(event EventTick
  (params (DeltaSeconds :type Float%20%28single-precision%29))
  (bind _returnvalue (* DeltaSeconds 5.0))
  (bind _2dzone (Variables|Default|Get2dZone))
  ;[1 1 1] EventTick
  (CallFunction|RotateTowardPantin DeltaSeconds)
  (CallFunction|UpdateSpeedPercent)
  (CallFunction|UpdateTargetLength)
  (CallFunction|ArmLengthTowardTarget DeltaSeconds)
  (Variables|Default|SetTargetRotation (Math|Rotator|Lerp(Rotator) (Variables|Default|GetTargetRotation) (Pawn|GetControlRotation :!class /Script/Engine.Pawn) _returnvalue true))
  (CallFunction|UpdateSpacetoClimb)
  (CallFunction|Climb)
  (CallFunction|TryActivateEvent)
  (bind _asbpi_action_object (Utilities|Casting|CastToBPI_ActionObject (Variables|Default|GetActionObject))
    (:then
      (Default|Active _asbpi_action_object _returnvalue))
    (:CastFailed
      _))
  (CallFunction|Wind _returnvalue)
  (CallFunction|UpdateVelocity)
  (Utilities|IsValid _2dzone
    (:Is%20Valid
      (Default|TickCam _2dzone _returnvalue))
    (:Is%20Not%20Valid
      _))
  (CallFunction|FunkyGravityTick))

(event Input|KeyboardEvents|W
  (params (Key :type Key%20Structure :default "None"))
  ;[1 1 1] DEBUG : Activate Wind
  (:Pressed
    (Variables|Wind|SetWindIsActive (not (Variables|Wind|GetWindIsActive)))
    (Variables|Default|SetWindDirection (Transformation|GetActorForwardVector (Variables|/Game/AssetsMyrmidon/Blueprints/BP_PlayerController.BP_PlayerController_C|GetCam (.AsBP%20Player%20Controller (Utilities|Casting|CastToBP_PlayerController (Game|GetPlayerController 0))))))
    (Development|PrintString (Utilities|String|SelectString "Wind activated" "Wind deactivated" (Variables|Wind|GetWindIsActive)))))

(fn ConstructionScript)

(fn LineTraceforWindDebug
  (params (MultDistanceFromCenter :type Float%20%28double-precision%29) (Length :type Float%20%28double-precision%29) (TakeIntoAccount :type Boolean))
  (bind _returnvalue (Transformation|GetActorLocation))
  (bind _returnvalue_2 (Transformation|GetActorLocation))
  (bind _winddirection (Variables|Default|GetWindDirection))
  (bind _returnvalue_3 (Math|Vector|RotateVector _winddirection "0.000000,90.000000,0.000000"))
  (bind _returnvalue_4 (* _returnvalue_3 MultDistanceFromCenter))
  (bind _returnvalue_5 (+ _returnvalue_2 _returnvalue_4))
  (if (== MultDistanceFromCenter 0.0)
    (bind _returnvalue_6 (Collision|LineTraceByChannel (- _returnvalue (* (Variables|Default|GetWindDirection) Length)) _returnvalue "TraceTypeQuery1" false 0 (Variables|DEBUG|GetDebugWind) true "(R=0.000000,G=0.166656,B=1.000000,A=1.000000)" "(R=0.462745,G=0.000000,B=0.003922,A=1.000000)"))
    (if (and _returnvalue_6 TakeIntoAccount)
      (Variables|Wind|SetWindHitPoints (+ (Variables|Wind|GetWindHitPoints) 1.0) :!label _label))
    (else
      (bind _returnvalue_7 (Collision|LineTraceByChannel (- _returnvalue_5 (* (Variables|Default|GetWindDirection) Length)) _returnvalue_5 "TraceTypeQuery1" false 0 (Variables|DEBUG|GetDebugWind) true "(R=0.000000,G=0.166656,B=1.000000,A=1.000000)" "(R=0.462745,G=0.000000,B=0.003922,A=1.000000)"))
      (if (and TakeIntoAccount _returnvalue_7)
        (goto _label)))))