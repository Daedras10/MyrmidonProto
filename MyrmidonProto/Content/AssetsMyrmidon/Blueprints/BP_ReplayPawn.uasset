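; BP_ReplayPawn is the replay viewer pawn that follows BP_Pantin through the camera currently selected by the game instance's CamIndex.
; On BeginPlay it registers with the game instance, creates the replay UI and snaps to the camera.
; Each tick it eases toward the position and rotation that camera from BP_CameraManager computes.
; SnapCamera teleports there instead, just after a brief black screen.
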(event Custom|SnapCamera
  (bind _uiwidget (Variables|Default|GetUIWidget))
  ;[1 1 1] SnapCamera
  (Default|SetBlackScreen _uiwidget true)
  (Utilities|FlowControl|Delay 0.4)
  (Default|SetBlackScreen _uiwidget false)
  (bind _returnvalue (Actor|GetActorOfClass "/Game/AssetsMyrmidon/Blueprints/BP_CameraManager.BP_CameraManager_C"))
  (Utilities|IsValid (Utilities|Array|Get(acopy) (Variables|/Game/AssetsMyrmidon/Blueprints/BP_CameraManager.BP_CameraManager_C|GetAllCameras _returnvalue) (Variables|/Game/AssetsMyrmidon/Blueprints/GameMode/BP_GameInstance.BP_GameInstance_C|GetcamIndex (.AsBP%20Game%20Instance (Utilities|Casting|CastToBP_GameInstance (Game|GetGameInstance)))))
    (:Is%20Valid
      (bind _returnvalue_2 (Actor|GetActorOfClass "/Game/AssetsMyrmidon/Blueprints/BP_Pantin.BP_Pantin_C"))
      (bind (_pos _rot) (Default|GetCameraPosandRot (Utilities|Array|Get(acopy) (Variables|/Game/AssetsMyrmidon/Blueprints/BP_CameraManager.BP_CameraManager_C|GetAllCameras _returnvalue) (Variables|/Game/AssetsMyrmidon/Blueprints/GameMode/BP_GameInstance.BP_GameInstance_C|GetcamIndex (.AsBP%20Game%20Instance (Utilities|Casting|CastToBP_GameInstance (Game|GetGameInstance))))) (Transformation|GetActorTransform) (Transformation|GetActorTransform _returnvalue_2)))
      (Transformation|SetActorLocationAndRotation _pos _rot false true))))

(event EventBeginPlay
  ;[1 1 1] BeginPlay
  (Variables|/Game/AssetsMyrmidon/Blueprints/GameMode/BP_GameInstance.BP_GameInstance_C|SetReplayPawn (.AsBP%20Game%20Instance (Utilities|Casting|CastToBP_GameInstance (Game|GetGameInstance))) self)
  (bind _returnvalue (UserInterface|CreateWidget "/Game/AssetsMyrmidon/Blueprints/WBP_ReplayUI.WBP_ReplayUI_C" (Game|GetPlayerController 0)))
  (bind _output_get (Variables|Default|SetUIWidget _returnvalue))
  (UserInterface|Viewport|AddtoViewport _output_get 0)
  (CallFunction|SnapCamera))

(event EventTick
  (params (DeltaSeconds :type Float%20%28single-precision%29))
  (bind _returnvalue (* DeltaSeconds 3.0))
  ;[1 1 1] EventTick
  (bind _returnvalue_2 (Actor|GetActorOfClass "/Game/AssetsMyrmidon/Blueprints/BP_Pantin.BP_Pantin_C"))
  (Utilities|IsValid _returnvalue_2
    (:Is%20Valid
      (bind _returnvalue_3 (Actor|GetActorOfClass "/Game/AssetsMyrmidon/Blueprints/BP_CameraManager.BP_CameraManager_C"))
      (bind (_pos _rot) (Default|GetCameraPosandRot (Utilities|Array|Get(acopy) (Variables|/Game/AssetsMyrmidon/Blueprints/BP_CameraManager.BP_CameraManager_C|GetAllCameras _returnvalue_3) (Variables|/Game/AssetsMyrmidon/Blueprints/GameMode/BP_GameInstance.BP_GameInstance_C|GetcamIndex (.AsBP%20Game%20Instance (Utilities|Casting|CastToBP_GameInstance (Game|GetGameInstance))))) (Transformation|GetActorTransform) (Transformation|GetActorTransform _returnvalue_2)))
      (Transformation|SetActorLocationAndRotation (Math|Vector|Lerp(Vector) (Transformation|GetActorLocation) _pos _returnvalue) (Math|Rotator|Lerp(Rotator) (Transformation|GetActorRotation) _rot _returnvalue true)))))

(fn ConstructionScript)