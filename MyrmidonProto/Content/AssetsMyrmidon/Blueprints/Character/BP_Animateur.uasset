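; First-person networked character (Animateur) that hovers, uses and carries Interactable objects.
; Tick-driven camera traces update hover hints, send interactions to the server and slide held objects along indexed cork boards, dropping them at free spots via recursive random retries.
; The camera bobs with speed, zooms and turns toward interactables when focused.
; Movement is client-authoritative, and MoveTo multicasts a timeline lerp while toggling movement replication.
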(event Custom|TryInteract
  (params (Start :type Vector) (End :type Vector) (IsA :type Boolean))
  (bind _debug (Variables|Default|GetDEBUG))
  ;[1 1 1] TryInteract
  (Development|PrintText (Utilities|Text|FormatText "TryInteract[{A?}]" (Utilities|String|SelectString "A" "B" IsA)) _debug _debug "(R=0.000000,G=0.660000,B=1.000000,A=1.000000)" 1e+01)
  (bind _outhit (Collision|LineTraceByChannel Start End "TraceTypeQuery2" false 0 "None"))
  (if (Utilities|DoesObjectImplementInterface (.HitActor (Collision|BreakHitResult _outhit)) "/Script/MyrmidonProto.Interactable")
    (bind _returnvalue (Class|Interactable|IsInteractable (.AsInteractable (Utilities|Casting|CastToInteractable (.HitActor (Collision|BreakHitResult _outhit))))))
    (if _returnvalue
      (Class|Interactable|StartB (.AsInteractable (Utilities|Casting|CastToInteractable (.HitActor (Collision|BreakHitResult _outhit)))))
      (Variables|Default|SetInteractorB (.HitActor (Collision|BreakHitResult _outhit)))
      (Class|Interactable|StartA (.AsInteractable (Utilities|Casting|CastToInteractable (.HitActor (Collision|BreakHitResult _outhit)))))
      (Variables|Default|SetInteractorA (.HitActor (Collision|BreakHitResult _outhit))))
    (bind _returnvalue_2 (Class|Interactable|IsPickable (.AsInteractable (Utilities|Casting|CastToInteractable (.HitActor (Collision|BreakHitResult _outhit))))))
    (if _returnvalue_2
      (Class|Interactable|PickUp(Message) (.HitActor (Collision|BreakHitResult _outhit)))
      (Variables|Default|SetObjectInHand (.HitActor (Collision|BreakHitResult _outhit)))
      (else
        (Development|PrintString "NotPickable" false false)))))

(event Custom|PutDownObject
  (bind (_start _end) (CallFunction|GetInteractionLocations))
  (bind _debug (Variables|Default|GetDEBUG))
  ;[1 1 1] PutDownObject
  (Development|PrintText "PutDownObject" _debug _debug "(R=0.000000,G=0.660000,B=1.000000,A=1.000000)" 1e+01)
  (Utilities|IsValid (Variables|Default|GetObjectInHand)
    (:Is%20Valid
      (bind _outhit (Collision|LineTraceByChannel _start _end "TraceTypeQuery2" false 0 "None"))
      (bind _returnvalue (Class|Interactable|GetCorkBoardIndex(Message) (Variables|Default|GetObjectInHand)))
      (CallFunction|PutItemDownCloseto (.Location (Collision|BreakHitResult _outhit)) _returnvalue 50))))

(event Custom|InteractAndDrop
  (bind (_start _end) (CallFunction|GetInteractionLocations))
  (bind (_start_2 _end_2) (CallFunction|GetInteractionLocations))
  (bind _uiwidget (Variables|Default|GetUIWidget))
  (bind _uiwidget_2 (Variables|Default|GetUIWidget))
  (bind _objectinhand (Variables|Default|GetObjectInHand))
  ;[1 1 1] EventTick
  (Utilities|IsValid (Variables|Default|GetObjectInHand)
    (:Is%20Valid
      (bind (_outhit _returnvalue) (Collision|LineTraceByChannel _start_2 _end_2 "TraceTypeQuery2" false 0 "None" true "(R=1.000000,G=0.000000,B=0.000000,A=1.000000)" "(R=0.000000,G=1.000000,B=0.000000,A=1.000000)" 0.1))
      (if _returnvalue
        (bind _returnvalue_2 (Class|Interactable|GetCorkBoardIndex(Message) (Variables|Default|GetObjectInHand)))
        (bind (_closestpoint _closestnormal) (CallFunction|GetClosestPointonCorkBoardswithIndex (.Location (Collision|BreakHitResult _outhit)) _returnvalue_2))
        (Transformation|SetActorLocationAndRotation _objectinhand (+ _closestpoint (* _closestnormal 3e+02)) (Math|Rotator|MakeRotator (.Roll (Math|Rotator|BreakRotator (Math|Rotator|FindLookatRotation _closestpoint (+ _closestpoint (* _closestnormal 3e+02))))) (.Pitch (Math|Rotator|BreakRotator (Math|Rotator|FindLookatRotation _closestpoint (+ _closestpoint (* _closestnormal 3e+02))))) (+ (.Yaw (Math|Rotator|BreakRotator (Math|Rotator|FindLookatRotation _closestpoint (+ _closestpoint (* _closestnormal 3e+02))))) 9e+01)))
        (Class|Interactable|Moved(Message) _objectinhand (+ _closestpoint (* _closestnormal 1e+01)))))
    (:Is%20Not%20Valid
      (bind (_outhit_2 _returnvalue_3) (Collision|LineTraceByChannel _start _end "TraceTypeQuery2" false 0 "None" true "(R=1.000000,G=0.000000,B=0.000000,A=1.000000)" "(R=0.000000,G=1.000000,B=0.000000,A=1.000000)" 0.1))
      (if (Utilities|DoesObjectImplementInterface (.HitActor (Collision|BreakHitResult _outhit_2)) "/Script/MyrmidonProto.Interactable")
        (if _returnvalue_3
          (if (not (== (.HitActor (Collision|BreakHitResult _outhit_2)) (Variables|Default|GetHoveredObject)))
            (Utilities|IsValid (Variables|Default|GetHoveredObject)
              (:Is%20Valid
                (Class|Interactable|EndHover(Message) (Variables|Default|GetHoveredObject))
                (Variables|Default|SetHoveredObject 0))
              (:Is%20Not%20Valid
                _))
            (bind _output_get (Variables|Default|SetHoveredObject (.HitActor (Collision|BreakHitResult _outhit_2))))
            (Class|Interactable|StartHover(Message) _output_get)
            (bind (_bdisplay _returnvalue_4) (Class|Interactable|GetInputInfos(Message) _output_get))
            (if _bdisplay
              (Utilities|IsValid _uiwidget_2
                (:Is%20Valid
                  (Default|SetControlIndics _uiwidget_2 _returnvalue_4)))
              (else
                (Utilities|IsValid _uiwidget_2
                  (:Is%20Valid
                    (Default|DisableControlIndics _uiwidget_2))))))
          (else
            (Utilities|IsValid (Variables|Default|GetHoveredObject)
              (:Is%20Valid
                (Class|Interactable|EndHover(Message) (Variables|Default|GetHoveredObject) :!label _label)
                (Variables|Default|SetHoveredObject 0)
                (Utilities|IsValid _uiwidget
                  (:Is%20Valid
                    (Default|DisableControlIndics _uiwidget)))))))
        (else
          (goto _label))))))

(event Custom|SetZoom
  (params (zoom :type Boolean))
  ;[1 1 1] CameraZoom
  (Variables|Default|SetinZoom zoom))

(event Custom|CameraZoom
  (params (DeltaTime :type Float%20%28double-precision%29))
  (bind _firstpersoncamera (Variables|Default|GetFirstPersonCamera))
  ;[1 1 1] CameraZoom
  (Camera|SetFieldOfView _firstpersoncamera (Math|Float|Lerp (Variables|/Script/Engine.CameraComponent|GetFieldOfView _firstpersoncamera) (Math|Float|SelectFloat 45.0 9e+01 (Variables|Default|GetinZoom)) (* DeltaTime 5.0))))

(event Custom|FocusToClosest
  (params (DeltaTime :type Float%20%28double-precision%29))
  (bind _location (CallFunction|GetInteractableLocation))
  (bind _self self)
  (bind _returnvalue (Pawn|GetController _self))
  ;[1 1 1] FocusClosest
  (if (and (or (Variables|Default|GetinFocus) (Variables|Default|GetGrabFocus)) (not (Utilities|Operators|EqualEqual :B _location :ErrorTolerance 0.01)))
    (Utilities|IsValid _returnvalue
      (:Is%20Valid
        (Pawn|SetControlRotation _returnvalue (Math|Rotator|Lerp(Rotator) (Pawn|GetControlRotation _returnvalue :!class /Script/Engine.Controller) (Math|Rotator|FindLookatRotation (Transformation|GetWorldLocation (Variables|Default|GetFirstPersonCamera)) _location) (* DeltaTime 1e+01) true))))))

(event Custom|SetFocus
  (params (Focus :type Boolean))
  ;[1 1 1] FocusClosest
  (Variables|Default|SetinFocus Focus))

(event Custom|Truc
  (params (Value :type Boolean))
  ;[1 1 1] BeginPlay
  (CallFunction|Truc2 Value))

(event Custom|truc2
  (params (Value :type Boolean))
  (bind _charactermovement (Variables|Character|GetCharacterMovement))
  ;[1 1 1] BeginPlay
  (bind _output_get (Variables|/Script/Engine.CharacterMovementComponent|SetbServerAcceptClientAuthoritativePosition _charactermovement true))
  (bind _output_get_2 (Variables|/Script/Engine.CharacterMovementComponent|SetbIgnoreClientMovementErrorChecksAndCorrection _charactermovement _output_get))
  (Variables|Default|SetbNetUseOwnerRelevancy _output_get_2))

(event Custom|Tst
  ;[1 1 1] BeginPlay
  (CallFunction|TstMulticast))

(event Custom|TstMulticast
  ;[1 1 1] BeginPlay
  (Class|Actor|SetReplicateMovement false))

(event Custom|FocusAndInteract
  (params (Value :type Boolean) (InteractAsA? :type Boolean))
  (bind _debug (Variables|Default|GetDEBUG))
  ;[1 1 1] FocusAndInteract
  (Development|PrintText (Utilities|Text|FormatText "Value {val} ; A? {A?}" Value InteractAsA?) _debug _debug "(R=1.000000,G=0.042986,B=0.000000,A=1.000000)" 2e+01)
  (bind _output_get (Variables|Default|SetTryInteractEachFrame Value))
  (bind _output_get_2 (Variables|Default|SetGrabFocus _output_get))
  (Variables|Default|SetInteractAsA InteractAsA?)
  (Variables|Default|SetinFocus _output_get_2)
  (CallFunction|EndInteractionsMulticast)
  (CallFunction|PutDownObject))

(event Custom|AddPitchInputValue
  (params (rot :type Rotator))
  ;[1 1 1] PitchInput
  (CallFunction|AddEventInputMulticast rot))

(event Custom|TryInteractTick
  (bind (_start _end) (CallFunction|GetInteractionLocations))
  ;[1 1 1] TryInteractTick
  (if (and (Variables|Default|GetTryInteractEachFrame) (Pawn|IsLocallyControlled))
    (CallFunction|TryInteractServer _start _end (and (Variables|Default|GetInteractAsA) (Variables|/Game/AssetsMyrmidon/Blueprints/GameMode/BP_PlayerController.BP_PlayerController_C|GetLastInputsWasGamepad (.AsBP%20Player%20Controller (Utilities|Casting|CastToBP_PlayerController (Pawn|GetController))))))))

(event Custom|PutItemDownCloseTo
  (params (Location :type Vector) (Index :type Integer) (MaxIteration :type Integer))
  (bind _debug (Variables|Default|GetDEBUG))
  ;[1 1 1] PutDownObject
  (if (> MaxIteration 0)
    (bind (_closestpoint _closestnormal) (CallFunction|GetClosestPointonCorkBoardswithIndex Location Index))
    (if (CallFunction|PointIsTooClosetoObject _closestpoint Index)
      (CallFunction|PutItemDownCloseto (CallFunction|GetRandomPointAroundVector Location _closestnormal) Index (- MaxIteration 1))
      (else
        (bind _returnvalue (Class|Interactable|GetCorkOffset(Message) (Variables|Default|GetObjectInHand)))
        (Transformation|SetActorLocation (Variables|Default|GetObjectInHand) (+ _closestpoint (* _closestnormal _returnvalue)) false false)
        (Class|Interactable|Drop(Message) (Variables|Default|GetObjectInHand))
        (Variables|Default|SetObjectInHand 0)
        (Development|PrintString "DROPPED" _debug _debug)))
    (else
      (Development|PrintString "CAN'T DROP ITEM" true true "(R=0.466667,G=0.000000,B=0.027342,A=1.000000)" 2e+01))))

(event Custom|CheckInteract
  ;[1 1 1] TryInteractTick
  (Networking|SwitchHasAuthority
    (:Authority
      (if (Variables|Default|GetTryInteractEachFrame)
        (Utilities|IsValid (Variables|Default|GetInteractorB)
          (:Is%20Valid
            _)
          (:Is%20Not%20Valid
            (Utilities|IsValid (Variables|Default|GetInteractorA)
              (:Is%20Valid
                _)
              (:Is%20Not%20Valid
                (Utilities|IsValid (Variables|Default|GetObjectInHand)
                  (:Is%20Valid
                    _))))))
        (Variables|Default|SetTryInteractEachFrame false)
        (Variables|Default|SetinFocus false)
        (Utilities|IsValid (Variables|Default|GetObjectInHand)
          (:Is%20Valid
            (Variables|Default|SetTryInteractEachFrame false)
            (Variables|Default|SetGrabFocus false)
            (Variables|Default|SetinFocus false)))))))

(event Custom|TryInteractServer
  (params (Start :type Vector) (End :type Vector) (IsA? :type Boolean))
  ;[1 1 1] TryInteractTick
  (CallFunction|TryInteract Start End IsA?))

(event Custom|EndInteractionsMulticast
  ;[1 1 1] FocusAndInteract
  (Utilities|IsValid (Variables|Default|GetInteractorA)
    (:Is%20Valid
      (Class|Interactable|EndA(Message) (Variables|Default|GetInteractorA))
      (Variables|Default|SetInteractorA 0))
    (:Is%20Not%20Valid
      _))
  (Utilities|IsValid (Variables|Default|GetInteractorB)
    (:Is%20Valid
      (Class|Interactable|EndB(Message) (Variables|Default|GetInteractorB))
      (Variables|Default|SetInteractorB 0))))

(event Custom|DropIfTooFar
  (bind _objectinhand (Variables|Default|GetObjectInHand))
  (Networking|SwitchHasAuthority
    (:Authority
      (if (Utilities|IsValid _objectinhand)
        (if (>= (Math|Vector|VectorLength (- (Transformation|GetActorLocation _objectinhand) (Transformation|GetActorLocation))) (Variables|Default|GetMaxGrabbedRange))
          (CallFunction|PutDownObject))))))

(event Custom|AddEventInputMulticast
  (params (Rot :type Rotator))
  ;[1 1 1] PitchInput
  (if (not (Pawn|IsLocallyControlled))
    (if (not (Variables|Default|GetinFocus))
      (Transformation|SetRelativeRotation (Variables|Default|GetFirstPersonCamera) Rot false false))))

(event Custom|CameraNod
  (bind _charactermovement (Variables|Character|GetCharacterMovement))
  ;[1 1 1] CameraNod
  (Transformation|SetRelativeLocation (Variables|Default|GetFirstPersonCamera) (+ (Math|Vector|MakeVector 0.0 0.0 (* (* (Math|Trig|Sin(Radians) (* (Utilities|Time|GetTimeSeconds) 1e+01)) 1e+01) (Math|Float|Clamp(Float) (/ (Math|Vector|VectorLengthXY (Variables|/Script/Engine.MovementComponent|GetVelocity _charactermovement)) (Class|MovementComponent|GetMaxSpeed _charactermovement))))) (* (Variables|Default|GetBaseEyeHeight) "0.000000,0.000000,1.000000")) false false))

(event Custom|MoveTo
  (params (Rotation :type Rotator) (Position :type Vector))
  ;[1 1 1] MoveTo (Server)
  (if (Variables|Default|GetCanBeMovedByOthers)
    (Class|Actor|SetReplicateMovement false)
    (CallFunction|MovetoMulticasted Rotation Position)))

(event Custom|MoveAnimateurWithInputs
  (params (WorldDircection :type Vector) (Scale :type Float%20%28double-precision%29) (IsForce :type Boolean))
  ;[1 1 1] MoveAnimateurWithInputs
  (Pawn|Input|AddMovementInput (Math|Vector|SelectVector WorldDircection (Math|Vector|Normalize WorldDircection) (<= (Math|Vector|VectorLength WorldDircection) 1.0)) Scale IsForce))

(event Custom|MoveToMulticasted
  (params (NewParam :type Rotator) (Position :type Vector))
  (bind _returnvalue (Transformation|GetActorLocation))
  (bind (_x _y) (Math|Vector|BreakVector Position))
  ;[1 1 1] MoveTo (Multicast)
  (bind _alpha (Timeline|LerpTowardTarget PlayFromStart)
    (:Update
      (Transformation|SetActorLocation (Math|Vector|Lerp(Vector) _returnvalue (Math|Vector|MakeVector _x _y (.Z (Math|Vector|BreakVector _returnvalue))) _alpha) false false)
      (Networking|SwitchHasAuthority
        (:Authority
          (CallFunction|RevertReplication))))))

(event Custom|TryEndInteract
  (params (IsA :type Boolean))
  (bind _debug (Variables|Default|GetDEBUG))
  ;[1 1 1] TryEndInteract
  (Development|PrintText (Utilities|Text|FormatText "TryInteract[{A?}]" (Utilities|String|SelectString "A" "B" IsA)) _debug _debug "(R=0.000000,G=0.660000,B=1.000000,A=1.000000)" 1e+01)
  (if IsA
    (Utilities|IsValid (Variables|Default|GetInteractorA)
      (:Is%20Valid
        (Class|Interactable|EndA(Message) (Variables|Default|GetInteractorA))
        (Variables|Default|SetInteractorA 0))
      (:Is%20Not%20Valid
        _))
    (else
      (Utilities|IsValid (Variables|Default|GetInteractorB)
        (:Is%20Valid
          (Class|Interactable|EndB(Message) (Variables|Default|GetInteractorB))
          (Variables|Default|SetInteractorB 0))
        (:Is%20Not%20Valid
          _))))
  (CallFunction|PutDownObject))

(event Custom|RevertReplication
  ;[1 1 1] RevertMvtReplication
  (Class|Actor|SetReplicateMovement true))

(event EventTick
  (params (DeltaSeconds :type Float%20%28single-precision%29))
  ;[1 1 1] EventTick
  (CallFunction|CameraNod)
  (CallFunction|InteractandDrop)
  (CallFunction|CameraZoom DeltaSeconds)
  (CallFunction|TryInteractTick)
  (CallFunction|CheckInteract)
  (CallFunction|DropifTooFar)
  (CallFunction|FocustoClosest DeltaSeconds))

(event EventBeginPlay
  ;[1 1 1] BeginPlay
  (Utilities|FlowControl|Delay 1.0)
  (if (Pawn|IsLocallyControlled)
    (CallFunction|Truc true)))

(event Input|KeyboardEvents|NumPadTwo
  (params (Key :type Key%20Structure :default "None"))
  ;[1 1 1] BeginPlay
  (:Pressed
    (CallFunction|Tst)))

(fn ConstructionScript)

(fn GetInteractionLocations
  (bind _firstpersoncamera (Variables|Default|GetFirstPersonCamera))
  (bind _returnvalue (Transformation|GetWorldLocation _firstpersoncamera))
  (return _returnvalue (+ _returnvalue (* (Math|Vector|GetForwardVector _firstpersoncamera) (Variables|Default|GetArmReach)))))

(fn GetInteractableLocation
  (bind _firstpersoncamera (Variables|Default|GetFirstPersonCamera))
  (if (Variables|Default|GetinFocus)
    (return (CallFunction|GetClosestInterractable (Transformation|GetWorldLocation _firstpersoncamera) (Math|Vector|GetForwardVector _firstpersoncamera) (Variables|Default|GetMaxFocusRange)))
    (else
      (if (Variables|Default|GetGrabFocus)
        (bind _asinteractable (Utilities|Casting|CastToInteractable (Variables|Default|GetInteractorB))
          (:then
            (bind _returnvalue (Class|Interactable|GetInterractPoint _asinteractable))
            (return _returnvalue))
          (:CastFailed
            _)))
      (return "0, 0, 0"))))

(fn GetRandomPointAroundVector
  (params (Point :type Vector) (PlanNormal :type Vector))
  (return (+ Point (* (Math|Vector|ProjectVectorontoPlane (Math|Vector|MakeVector (- (Math|Random|RandomFloat) 0.5) (- (Math|Random|RandomFloat) 0.5) (- (Math|Random|RandomFloat) 0.5)) PlanNormal) (* (Math|Random|RandomFloat) 1.5e+02)))))

(fn OnRepTryInteractEachFrame)

(fn OnRepGrabFocus)

(fn OnRepinFocus)