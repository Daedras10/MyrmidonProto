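; BP_ReplayPawn is the replay viewer pawn, which smoothly follows the BP_Camera actor each tick through delta-time-scaled location and rotation lerps.
; On BeginPlay it registers with BP_GameInstance, creates WBP_ReplayUI and passes it the current scene name.
; SnapCamera only flashes a brief black screen on that UI.
; Disconnected graphs hold unused BP_CameraManager logic for placing the view relative to BP_Pantin.
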(event Custom|SnapCamera
  (bind _uiwidget (Variables|Default|GetUIWidget))
  ;[1 1 1] SnapCamera
  (Default|SetBlackScreen _uiwidget true)
  (Utilities|FlowControl|Delay 0.4)
  (Default|SetBlackScreen _uiwidget false))

(event EventBeginPlay
  (bind _returnvalue (Game|GetGameInstance))
  (bind _asbp_game_instance (Utilities|Casting|CastToBP_GameInstance _returnvalue))
  ;[1 1 1] BeginPlay
  (Variables|/Game/AssetsMyrmidon/Blueprints/GameMode/BP_GameInstance.BP_GameInstance_C|SetReplayPawn _asbp_game_instance self)
  (bind _returnvalue_2 (UserInterface|CreateWidget "/Game/AssetsMyrmidon/Blueprints/UI/WBP_ReplayUI.WBP_ReplayUI_C" (Game|GetPlayerController 0)))
  (bind _output_get (Variables|Default|SetUIWidget _returnvalue_2))
  (UserInterface|Viewport|AddtoViewport _output_get 0)
  (CallFunction|SnapCamera)
  (Default|SetScene _output_get (Variables|/Game/AssetsMyrmidon/Blueprints/GameMode/BP_GameInstance.BP_GameInstance_C|GetSceneName _asbp_game_instance)))

(event EventTick
  (params (DeltaSeconds :type Float%20%28single-precision%29))
  (bind _returnvalue (* DeltaSeconds 8.0))
  ;[1 1 1] EventTick
  (bind _returnvalue_2 (Actor|GetActorOfClass "/Game/AssetsMyrmidon/Blueprints/Camera/BP_Camera.BP_Camera_C"))
  (Utilities|IsValid _returnvalue_2
    (:Is%20Valid
      (Transformation|SetActorLocationAndRotation (Math|Vector|Lerp(Vector) (Transformation|GetActorLocation) (Transformation|GetActorLocation _returnvalue_2) _returnvalue) (Math|Rotator|Lerp(Rotator) (Transformation|GetActorRotation) (Transformation|GetActorRotation _returnvalue_2) _returnvalue true)))))

(fn ConstructionScript)