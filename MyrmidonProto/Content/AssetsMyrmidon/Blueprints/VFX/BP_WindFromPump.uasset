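; BP_WindFromPump is a VFX Blueprint that wraps a Niagara component to show wind from a pump.
; Its events feed size, multiplied by 100, and direction into the Niagara BoxSize and WindDirection vector variables.
; Activate and Deactivate start (with reset) and stop the effect while updating an IsActive flag.
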(event Custom|Activate
  (Components|Activation|Activate (Variables|NiagaraActor|GetNiagaraComponent) true)
  (Variables|Default|SetIsActive true))

(event Custom|Deactivate
  (Components|Activation|Deactivate (Variables|NiagaraActor|GetNiagaraComponent))
  (Variables|Default|SetIsActive false))

(event Custom|SetSize
  (params (Scale :type Vector))
  (Niagara|SetNiagaraVariable(Vector3) (Variables|NiagaraActor|GetNiagaraComponent) "BoxSize" (* Scale 1e+02)))

(event Custom|SetDirection
  (params (Direction :type Vector))
  (Niagara|SetNiagaraVariable(Vector3) (Variables|NiagaraActor|GetNiagaraComponent) "WindDirection" Direction))

(fn ConstructionScript)