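; BP_WindEffect is a VFX actor that shows a Niagara wind effect around the BP_Pantin actor while its wind is active.
; On Tick it polls for BP_Pantin until found, then binds to its wind-state change event to activate or deactivate the Niagara component.
; While wind is active, it places itself upwind of Pantin with a slight height offset and feeds the wind direction to Niagara each frame.
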(event Custom|Activate
  (Components|Activation|Activate (Variables|NiagaraActor|GetNiagaraComponent) true))

(event Custom|Deactivate
  (Components|Activation|Deactivate (Variables|NiagaraActor|GetNiagaraComponent)))

(event Custom|OnWindActifChanged
  (params (NewState :type Boolean))
  (if NewState
    (CallFunction|Activate)
    (else
      (CallFunction|Deactivate))))

(event EventTick
  (params (DeltaSeconds :type Float%20%28single-precision%29))
  (if (Variables|Default|GetStarted)
    (if (Variables|/Script/MyrmidonProto.PantinCharacter|GetWindIsActive (Variables|Default|GetPantin))
      (Transformation|SetActorLocation (+ (- (Transformation|GetActorLocation (Variables|Default|GetPantin)) (* (Math|Vector|Normalize (Variables|/Script/MyrmidonProto.PantinCharacter|GetWindDirection (Variables|Default|GetPantin))) (Variables|Default|GetDistanceFromPantin))) "0.000000,0.000000,50.000000") false false)
      (Niagara|SetNiagaraVariable(Vector3) (Variables|NiagaraActor|GetNiagaraComponent) "WindDirection" (Variables|/Script/MyrmidonProto.PantinCharacter|GetWindDirection (Variables|Default|GetPantin))))
    (else
      (bind _returnvalue (Actor|GetActorOfClass "/Game/AssetsMyrmidon/Blueprints/Character/BP_Pantin.BP_Pantin_C"))
      (Utilities|IsValid _returnvalue
        (:Is%20Valid
          (bind _output_get (Variables|Default|SetPantin _returnvalue))
          (EventDispatchers|BindEventtoWindActifStateChanged _output_get (delegate Custom|OnWindActifChanged))
          (CallFunction|OnWindActifChanged (Variables|/Script/MyrmidonProto.PantinCharacter|GetWindIsActive _output_get))
          (Variables|Default|SetStarted true))))))

(fn ConstructionScript)