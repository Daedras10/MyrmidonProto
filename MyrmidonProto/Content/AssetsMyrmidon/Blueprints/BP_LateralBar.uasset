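; Horizontal swing bar that a BP_Pantin grabs on overlap and swings around; it can also be picked up, dropped and highlighted on hover.
; A hand-rolled pendulum on Tick updates angle and velocity with drag, blending the character's location and mesh roll onto the bar.
; On the Pantin player's side, movement input feeds the swing.
; Detaching restores gravity and launches the character along the swing velocity; pickup forces detach and disables collision.
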(event OnComponentBeginOverlap(Capsule)
  (params (OverlappedComponent :type Primitive%20Component%20Object%20Reference) (OtherActor :type Actor%20Object%20Reference) (OtherComp :type Primitive%20Component%20Object%20Reference) (OtherBodyIndex :type Integer) (bFromSweep :type Boolean) (SweepResult :type Hit%20Result%20Structure%20%28by%20ref%29))
  ;[1 1 1] Overlap
  (Utilities|IsValid (Variables|Default|GetPantinAttached)
    (:Is%20Not%20Valid
      (if (Variables|/Script/MyrmidonProto.RecordingGameInstance|GetinReplay (.AsBP%20Game%20Instance (Utilities|Casting|CastToBP_GameInstance (Game|GetGameInstance))))
        _
        (else
          (Variables|Default|SetPantinSide (Variables|/Game/AssetsMyrmidon/Blueprints/BP_PlayerController.BP_PlayerController_C|GetisPantin (.AsBP%20Player%20Controller (Utilities|Casting|CastToBP_PlayerController (Game|GetPlayerController 0)))))))
      (bind _asbp_pantin (Utilities|Casting|CastToBP_Pantin OtherActor))
      (if (not (Utilities|IsValid (Variables|/Game/AssetsMyrmidon/Blueprints/BP_Pantin.BP_Pantin_C|GetLateralBar _asbp_pantin)))
        (bind _output_get (Variables|Default|SetPantinAttached _asbp_pantin))
        (Variables|Default|SetMemPos (Transformation|GetActorLocation _output_get))
        (CallFunction|SetAnglefromPosition (Transformation|GetActorLocation _output_get))
        (Variables|/Game/AssetsMyrmidon/Blueprints/BP_Pantin.BP_Pantin_C|SetLateralBar _output_get self)
        (Variables|Default|SetTransitionTime 0.0)
        (Variables|/Script/Engine.CharacterMovementComponent|SetGravityScale (Variables|/Script/Engine.Character|GetCharacterMovement _output_get) 0.0)
        (Variables|/Script/Engine.CharacterMovementComponent|SetbOrientRotationToMovement (Variables|/Script/Engine.Character|GetCharacterMovement _output_get) false)))))

(event Custom|EndHoverMulticasted
  (bind _cylinder (Variables|Default|GetCylinder))
  ;[1 1 1] Start & End Hover
  (Rendering|SetRenderCustomDepth _cylinder false)
  (Rendering|Material|SetMaterial _cylinder 0 "/Engine/BasicShapes/BasicShapeMaterial.BasicShapeMaterial"))

(event Custom|BeginHoverMulticasted
  (bind _cylinder (Variables|Default|GetCylinder))
  ;[1 1 1] Start & End Hover
  (Rendering|SetRenderCustomDepth _cylinder true)
  (Rendering|Material|SetMaterial _cylinder 0 "/Game/AssetsMyrmidon/Art/Materials/M_Red.M_Red"))

(event Custom|SetCollisions
  (params (Active :type Boolean))
  ;[1 1 1] PickUp and Drop
  (Collision|SetActorEnableCollision self Active))

(event Custom|PhysicTick
  (params (DeltaSeconds :type Float%20%28double-precision%29) (TransitionTime :type Float%20%28double-precision%29))
  (bind _maxvelocity (Variables|Default|GetMaxVelocity))
  (bind _pantinattached (Variables|Default|GetPantinAttached))
  ;[1 1 1] PhysicsTick
  (bind _output_get (Variables|Default|SetAngle (+ (Variables|Default|GetAngle) (* (* DeltaSeconds (Variables|Default|GetVelocity)) 3.0))))
  (if (> _output_get 1.8e+02)
    (Variables|Default|SetAngle (+ (Variables|Default|GetAngle) -3.6e+02))
    (elif (< _output_get -1.8e+02)
      (Variables|Default|SetAngle (+ (Variables|Default|GetAngle) 3.6e+02))))
  (Transformation|SetRelativeRotation (Variables|Default|GetArrow) (Math|Rotator|MakeRotator 0.0 (+ (Variables|Default|GetAngle) 2.7e+02) 0.0) false false)
  (bind _output_get_2 (Variables|Default|SetVelocity (Math|Float|Clamp(Float) (+ (* (Variables|Default|GetVelocity) (Variables|Default|GetDrag)) (* (* DeltaSeconds -3e+02) (/ (Variables|Default|GetAngle) 1.8e+02))) (* _maxvelocity -1.0) _maxvelocity)))
  (Variables|/Script/Engine.ArrowComponent|SetArrowLength (Variables|Default|GetVelocityArrow) _output_get_2)
  (bind _position (CallFunction|GetPositiononBar 1.5e+02))
  (CallFunction|RotateCharacterModel TransitionTime)
  (Transformation|SetActorLocation _pantinattached (Math|Vector|Lerp(Vector) (Variables|Default|GetMemPos) _position TransitionTime) false false)
  (if (Variables|Default|GetPantinSide)
    (Variables|/Script/Engine.MovementComponent|SetVelocity (Variables|/Script/Engine.Character|GetCharacterMovement _pantinattached) (* (Math|Vector|GetForwardVector (Variables|Default|GetVelocityArrow)) (* (Math|Trig|DegreesToRadians (Variables|Default|GetVelocity)) 1.5e+02)))
    (CallFunction|ConvertInputIntoVelocity DeltaSeconds)))

(event Custom|SetAngleFromPosition
  (params (Position :type Vector))
  (bind _returnvalue (Transformation|GetActorTransform))
  (bind _returnvalue_2 (Math|Transform|InverseTransformLocation _returnvalue Position))
  (bind (_x _y _z) (Math|Vector|BreakVector _returnvalue_2))
  ;[1 1 1] SetAngleFromPosition
  (Variables|Default|SetAngle (* (Math|Vector|DotProduct (Math|Vector|Normalize (Math|Vector|MakeVector _x _z 0.0)) "-1.000000,0.000000,0.000000") -9e+01))
  (CallFunction|PhysicTick 0.0 0.0))

(event Custom|RotateCharacterModel
  (params (Alpha :type Float%20%28double-precision%29))
  (bind _angle (Variables|Default|GetAngle))
  (bind _returnvalue (Math|Float|Lerp 0.0 _angle Alpha))
  (bind _returnvalue_2 (Math|Rotator|MakeRotator _returnvalue 0.0 -9e+01))
  (Transformation|SetRelativeLocationAndRotation (Variables|/Script/Engine.Character|GetMesh (Variables|Default|GetPantinAttached)) (Math|Vector|RotateVector "0.000000,0.000000,-90.000000" _returnvalue_2) _returnvalue_2 false false))

(event Custom|DetachPlayer
  ;[1 1 1] DetachPlayer
  (Utilities|IsValid (Variables|Default|GetPantinAttached)
    (:Is%20Valid
      (Variables|/Script/Engine.CharacterMovementComponent|SetGravityScale (Variables|/Script/Engine.Character|GetCharacterMovement (Variables|Default|GetPantinAttached)) 1.0))
    (:Is%20Not%20Valid
      _))
  (Variables|/Game/AssetsMyrmidon/Blueprints/BP_Pantin.BP_Pantin_C|SetLateralBar (Variables|Default|GetPantinAttached) 0)
  (Variables|/Script/Engine.MovementComponent|SetVelocity (Variables|/Script/Engine.Character|GetCharacterMovement (Variables|Default|GetPantinAttached)) (* (Math|Vector|GetForwardVector (Variables|Default|GetVelocityArrow)) (* (Variables|Default|GetVelocity) (Variables|Default|GetExitForce))))
  (Variables|/Script/Engine.CharacterMovementComponent|SetbOrientRotationToMovement (Variables|/Script/Engine.Character|GetCharacterMovement (Variables|Default|GetPantinAttached)) true)
  (Transformation|SetRelativeLocationAndRotation (Variables|/Script/Engine.Character|GetMesh (Variables|Default|GetPantinAttached)) "0.000000,0.000000,-90.000000" (Math|Rotator|MakeRotator 0.0 0.0 -9e+01) false false)
  (Variables|Default|SetPantinAttached 0)
  (Variables|Default|SetVelocity 0.0))

(event Custom|ConvertInputIntoVelocity
  (params (DeltaSeconds :type Float%20%28double-precision%29))
  ;[1 1 1] ConvertInputIntoVelocity
  (Variables|Default|SetVelocity (+ (* (* DeltaSeconds (.X (Math|Vector|BreakVector (Math|Transform|InverseTransformDirection (Transformation|GetActorTransform) (Pawn|Components|PawnMovement|GetLastInputVector (Variables|/Script/Engine.Character|GetCharacterMovement (Variables|Default|GetPantinAttached))))))) (Variables|Default|GetInputForce)) (Variables|Default|GetVelocity))))

(event EventPickUp
  ;[1 1 1] PickUp and Drop
  (CallFunction|SetCollisions false)
  (Utilities|IsValid (Variables|Default|GetPantinAttached)
    (:Is%20Valid
      (CallFunction|DetachPlayer))))

(event EventDrop
  ;[1 1 1] PickUp and Drop
  (CallFunction|SetCollisions true))

(event EventEndHover
  ;[1 1 1] Start & End Hover
  (CallFunction|EndHoverMulticasted))

(event EventTick
  (params (DeltaSeconds :type Float%20%28single-precision%29))
  (Utilities|IsValid (Variables|Default|GetPantinAttached)
    (:Is%20Valid
      (CallFunction|PhysicTick DeltaSeconds (Variables|Default|GetTransitionTime))
      (Variables|Default|SetTransitionTime (Math|Float|Clamp(Float) (+ (Variables|Default|GetTransitionTime) (* DeltaSeconds 2.0)))))))

(event EventStartHover
  ;[1 1 1] Start & End Hover
  (CallFunction|BeginHoverMulticasted))

(fn ConstructionScript)

(fn GetPositiononBar
  (params (Distance :type Float%20%28double-precision%29))
  (return (Math|Transform|TransformLocation (Transformation|GetActorTransform) (* (Math|Vector|RotateVectorAroundAxis "0.000000,0.000000,-1.000000" (* (Variables|Default|GetAngle) -1.0) "0.000000,1.000000,0.000000") Distance))))

(fn OnRepAngleReplicated
  (Development|PrintString (Utilities|String|Append "REPLICATED " (Utilities|String|ToString(Boolean) (Variables|Default|GetPantinSide))) true true "(R=1.000000,G=0.330191,B=0.000000,A=1.000000)" 5.0))

(fn GetCorkBoard
  (return (Variables|Default|GetCorkBoard)))

(fn IsPickable
  (return true))