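; BP_MovablePlatformButton is a button that drives a linked movable platform.
; On activation it copies its GoToA flag into the platform's TargetPosIsA to choose the destination, then sets IsMoving to start the platform.
; On deactivation it clears IsMoving, so the platform is only flagged as moving while the button is active.
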(event EventTick
  (params (DeltaSeconds :type Float%20%28single-precision%29))
  (|CallParentFunction DeltaSeconds) ; This node is disabled and will not be called.\nDrag off pins to build functionality.
)

(event EventButtonActive)

(event EventOnButtonActivated
  (Variables|/Game/AssetsMyrmidon/Blueprints/BP_MovablePlatform.BP_MovablePlatform_C|SetTargetPosIsA (Variables|Default|GetMovablePlatform) (Variables|Default|GetGoToA))
  (Variables|/Game/AssetsMyrmidon/Blueprints/BP_MovablePlatform.BP_MovablePlatform_C|SetIsMoving (Variables|Default|GetMovablePlatform) true))

(event EventOnButtonDeactivated
  (Variables|/Game/AssetsMyrmidon/Blueprints/BP_MovablePlatform.BP_MovablePlatform_C|SetIsMoving (Variables|Default|GetMovablePlatform) false))

(fn ConstructionScript
  (|CallParentFunction))