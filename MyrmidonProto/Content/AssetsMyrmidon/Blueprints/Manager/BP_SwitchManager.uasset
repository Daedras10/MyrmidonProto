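; BP_SwitchManager is a manager actor that toggles level visibility between a Pantin view and an Animator view.
; On BeginPlay it gathers actors tagged AddPantin and AddAnimator into two arrays.
; View events route through Visible, which shows one group and hides the other by setting root component visibility, propagated to children.
; ViewAll shows both groups at once.
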(event Custom|AnimatorView
  (Class|VisualSwitcher|Switch false))

(event Custom|PantinView
  (Class|VisualSwitcher|Switch true))

(event Custom|ViewAll
  (for _array_element (Variables|Default|GetActorsAnimator)
    (Rendering|SetVisibility (Variables|/Script/Engine.Actor|GetRootComponent _array_element) true true))
  (for _array_element_2 (Variables|Default|GetActorsPantin)
    (Rendering|SetVisibility (Variables|/Script/Engine.Actor|GetRootComponent _array_element_2) true true)))

(event Custom|PopulateArrays
  (CallFunction|ClearArrays)
  (bind _outactors (Actor|GetAllActorsOfClasswithTag "/Script/Engine.Actor" "AddPantin"))
  (for _array_element _outactors
    (Utilities|Array|AddUnique (Variables|Default|GetActorsPantin) _array_element))
  (bind _outactors_2 (Actor|GetAllActorsOfClasswithTag "/Script/Engine.Actor" "AddAnimator"))
  (for _array_element_2 _outactors_2
    (Utilities|Array|AddUnique (Variables|Default|GetActorsAnimator) _array_element_2)))

(event Custom|Visible
  (params (Pantin :type Boolean))
  (bind _output_get (Variables|Default|SetIsPantinView Pantin))
  (for _array_element (Variables|Default|GetActorsAnimator)
    (Rendering|SetVisibility (Variables|/Script/Engine.Actor|GetRootComponent _array_element) (not _output_get) true))
  (for _array_element_2 (Variables|Default|GetActorsPantin)
    (Rendering|SetVisibility (Variables|/Script/Engine.Actor|GetRootComponent _array_element_2) _output_get true)))

(event Custom|ClearArrays
  (Utilities|Array|Clear (Variables|Default|GetActorsPantin))
  (Utilities|Array|Clear (Variables|Default|GetActorsAnimator)))

(event EventBeginPlay
  (CallFunction|PopulateArrays))

(event EventSwitchtoAnimator
  (CallFunction|Visible false))

(event EventSwitchtoPantin
  (CallFunction|Visible true))

(event EventSwitch
  (params (bToPantin :type Boolean))
  (if bToPantin
    (Class|VisualSwitcher|SwitchtoPantin)
    (else
      (Class|VisualSwitcher|SwitchtoAnimator))))

(fn ConstructionScript)