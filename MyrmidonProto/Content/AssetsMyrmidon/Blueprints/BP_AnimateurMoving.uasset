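; BP_AnimateurMoving is a first-person character that can carry pickable objects and highlight switches it looks at.
; Pickup and put-down events use line traces, placing dropped objects offset along the surface normal.
; Tick adds speed-scaled sine camera bob, pins the held object to PickedObject, or otherwise traces within ArmReach to toggle hover on BP_SwitchParentClass actors.
; Camera rotation is relayed through a multicast-named event and applied only on non-locally-controlled instances.
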(event Custom|TryPickup
  (params (Start :type Vector) (End :type Vector))
  (Development|PrintString "Hello")
  (bind _outhit (Collision|LineTraceByChannel Start End "TraceTypeQuery1" false 0 "None"))
  (if (Utilities|DoesObjectImplementInterface (.HitActor (Collision|BreakHitResult _outhit)) "/Game/AssetsMyrmidon/Blueprints/Interfaces/BPI_Pickable.BPI_Pickable_C")
    (Default|Pick (.AsBPI%20Pickable (Utilities|Casting|CastToBPI_Pickable (.HitActor (Collision|BreakHitResult _outhit)))))
    (Variables|Default|SetObjectInHand (.HitActor (Collision|BreakHitResult _outhit)))))

(event Custom|PutDownObject
  (params (Start :type Vector) (End :type Vector))
  (Utilities|IsValid (Variables|Default|GetObjectInHand)
    (:Is%20Valid
      (bind (_outhit _returnvalue) (Collision|LineTraceByChannel Start End "TraceTypeQuery1" false 0 "None"))
      (if _returnvalue
        (Transformation|SetActorLocation (Variables|Default|GetObjectInHand) (+ (.Location (Collision|BreakHitResult _outhit)) (* (.ImpactNormal (Collision|BreakHitResult _outhit)) 5e+01)) false false)
        (Class|BPIPickable|Dropped(Message) (Variables|Default|GetObjectInHand))
        (Variables|Default|SetObjectInHand 0)))))

(event Custom|AddPitchInputValue
  (params (rot :type Rotator))
  ;[1 1 1] PitchInput
  (CallFunction|AddEventInputMulticast rot))

(event Custom|AddEventInputMulticast
  (params (Rot :type Rotator))
  ;[1 1 1] PitchInput
  (if (not (Pawn|IsLocallyControlled))
    (Transformation|SetRelativeRotation (Variables|Default|GetFirstPersonCamera) Rot false false)))

(event Custom|CameraNod
  (bind _charactermovement (Variables|Character|GetCharacterMovement))
  ;[1 1 1] CameraNod
  (Transformation|SetRelativeLocation (Variables|Default|GetFirstPersonCamera) (+ (Math|Vector|MakeVector 0.0 0.0 (* (* (Math|Trig|Sin(Radians) (* (Utilities|Time|GetTimeSeconds) 1e+01)) 3.0) (Math|Float|Clamp(Float) (/ (Math|Vector|VectorLengthXY (Variables|/Script/Engine.MovementComponent|GetVelocity _charactermovement)) (Class|MovementComponent|GetMaxSpeed _charactermovement))))) "0.000000,0.000000,60.000000") false false))

(event EventTick
  (params (DeltaSeconds :type Float%20%28single-precision%29))
  (bind _objectinhand (Variables|Default|GetObjectInHand))
  (bind _firstpersoncamera (Variables|Default|GetFirstPersonCamera))
  (bind _returnvalue (Transformation|GetWorldLocation _firstpersoncamera))
  (CallFunction|CameraNod)
  (Utilities|IsValid _objectinhand
    (:Is%20Valid
      (Transformation|SetActorLocation _objectinhand (Transformation|GetWorldLocation (Variables|Default|GetPickedObject)) false false))
    (:Is%20Not%20Valid
      (bind (_outhit _returnvalue_2) (Collision|LineTraceByChannel _returnvalue (+ (* (Math|Vector|GetForwardVector _firstpersoncamera) (Variables|Default|GetArmReach)) _returnvalue) "TraceTypeQuery1" false 0 "None" true "(R=1.000000,G=0.000000,B=0.000000,A=1.000000)" "(R=0.000000,G=1.000000,B=0.000000,A=1.000000)" 0.1))
      (if _returnvalue_2
        (if (not (== (.HitActor (Collision|BreakHitResult _outhit)) (Variables|Default|GetHoveredObject)))
          (Utilities|IsValid (Variables|Default|GetHoveredObject)
            (:Is%20Valid
              (Default|EndHover (.AsBP%20Switch%20Parent%20Class (Utilities|Casting|CastToBP_SwitchParentClass (Variables|Default|GetHoveredObject))))
              (Variables|Default|SetHoveredObject 0))
            (:Is%20Not%20Valid
              _))
          (bind _asbp_switch_parent_class (Utilities|Casting|CastToBP_SwitchParentClass (.HitActor (Collision|BreakHitResult _outhit))))
          (Variables|Default|SetHoveredObject _asbp_switch_parent_class)
          (Default|BeginHover _asbp_switch_parent_class))
        (else
          (Utilities|IsValid (Variables|Default|GetHoveredObject)
            (:Is%20Valid
              (Default|EndHover (.AsBP%20Switch%20Parent%20Class (Utilities|Casting|CastToBP_SwitchParentClass (Variables|Default|GetHoveredObject))))
              (Variables|Default|SetHoveredObject 0))))))))

(fn ConstructionScript)