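; BP_4thWallTrigger is a trigger volume that toggles a player controller's visual setup as BP_Pantin characters enter and leave it.
; On the server, a living Pantin beginning overlap calls SetUpVisuals(false) on the controller fetched from the game mode.
; Any Pantin ending overlap calls SetUpVisuals(true), with no alive check and no count of Pantins still inside.
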(event OnComponentBeginOverlap(Trigger)
  (params (OverlappedComponent :type Primitive%20Component%20Object%20Reference) (OtherActor :type Actor%20Object%20Reference) (OtherComp :type Primitive%20Component%20Object%20Reference) (OtherBodyIndex :type Integer) (bFromSweep :type Boolean) (SweepResult :type Hit%20Result%20Structure%20%28by%20ref%29))
  (Networking|SwitchHasAuthority
    (:Authority
      (bind _asbp_pantin (Utilities|Casting|CastToBP_Pantin OtherActor))
      (if (Variables|/Script/MyrmidonProto.PantinCharacter|GetIsAlive _asbp_pantin)
        (Default|SetUpVisuals (Default|GetBPPlayerController (.GameMode (CallFunction|GetBPGameMode)) true) false)))))

(event OnComponentEndOverlap(Trigger)
  (params (OverlappedComponent :type Primitive%20Component%20Object%20Reference) (OtherActor :type Actor%20Object%20Reference) (OtherComp :type Primitive%20Component%20Object%20Reference) (OtherBodyIndex :type Integer))
  (Networking|SwitchHasAuthority
    (:Authority
      (Utilities|Casting|CastToBP_Pantin OtherActor)
      (Default|SetUpVisuals (Default|GetBPPlayerController (.GameMode (CallFunction|GetBPGameMode)) true) true))))

(fn ConstructionScript)