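; Trigger zone that keeps its assigned lights off for non-Pantin players until a living Pantin enters its box.
; On game start, the server multicasts after a delay; each non-Pantin client caches intensities and materials, then darkens lights, props and heavy lights.
; The first living Pantin overlap, including an initial check, permanently restores materials and heavy lights, with a timeline fading intensities back in.
; Pantin players' lighting stays untouched.
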(event OnComponentBeginOverlap(Box)
  (params (OverlappedComponent :type Primitive%20Component%20Object%20Reference) (OtherActor :type Actor%20Object%20Reference) (OtherComp :type Primitive%20Component%20Object%20Reference) (OtherBodyIndex :type Integer) (bFromSweep :type Boolean) (SweepResult :type Hit%20Result%20Structure%20%28by%20ref%29))
  (bind _asbp_pantin (Utilities|Casting|CastToBP_Pantin OtherActor))
  (CallFunction|OverlapPantin _asbp_pantin))

(event Custom|ForceCheck
  (for _array_element (Collision|GetOverlappingActors (Variables|Default|GetBox) "/Game/AssetsMyrmidon/Blueprints/Character/BP_Pantin.BP_Pantin_C" :!class /Script/Engine.PrimitiveComponent)
    (CallFunction|OverlapPantin (.AsBP%20Pantin (Utilities|Casting|CastToBP_Pantin _array_element)))))

(event Custom|OverlapPantin
  (params (Pantin :type BP%20Pantin%20Object%20Reference))
  (bind _playercontroller (CallFunction|GetBPLocalPlayerController))
  (Utilities|IsValid _playercontroller
    (:Is%20Valid
      (if (Variables|/Script/MyrmidonProto.PantinCharacter|GetIsAlive Pantin)
        (if (not (Variables|Default|GetActivated))
          (Variables|Default|SetActivated true)
          (if (Variables|/Game/AssetsMyrmidon/Blueprints/GameMode/BP_PlayerController.BP_PlayerController_C|GetisPantin _playercontroller)
            (Development|PrintString "PANTIN LIGHT")
            (else
              (Utilities|FlowControl|Sequence
                (:then_0
                  (for (_array_element _array_index) (Variables|Default|GetObjects)
                    (Rendering|Material|SetMaterial (Variables|/Script/Engine.StaticMeshActor|GetStaticMeshComponent _array_element) 1 (Utilities|Array|Get(acopy) (Variables|Default|GetMaterials) _array_index)))
                  (for _array_element_2 (Variables|Default|GetHeavyLights)
                    (Default|Turnon _array_element_2)))
                (:then_1
                  (Development|PrintString "ANIM LIGHT")
                  (bind _intensity (Timeline|LightAnimation Play)
                    (:Update
                      (for (_array_element_3 _array_index_2) (Variables|Default|GetLights)
                        (Rendering|Components|Light|SetIntensity (Variables|/Script/Engine.Light|GetLightComponent _array_element_3) (Math|Float|Lerp 0.0 (Utilities|Array|Get(acopy) (Variables|Default|GetIntensities) _array_index_2) _intensity))))))))))))))

(event Custom|OnGameStartServer
  (EventDispatchers|UnbindEventfromGameStart (.GameMode (CallFunction|GetBPGameMode)) (delegate Custom|OnGameStartServer))
  (Utilities|FlowControl|Delay 2.0)
  (CallFunction|OnGameStartMulticast))

(event Custom|OnGameStartMulticast
  (CallFunction|SetupLights)
  (CallFunction|ForceCheck))

(event Custom|SetupLights
  (bind _playercontroller (CallFunction|GetBPLocalPlayerController))
  (bind _ispantin (Variables|/Game/AssetsMyrmidon/Blueprints/GameMode/BP_PlayerController.BP_PlayerController_C|GetisPantin _playercontroller))
  (if _ispantin
    (Development|PrintString "BAH ALORS?????????????? " true true "(R=0.000000,G=0.660000,B=1.000000,A=1.000000)" 5e+02)
    (else
      (Development|PrintString "LIGHTS OFFFFFFF " true true "(R=0.000000,G=0.660000,B=1.000000,A=1.000000)" 5e+02)))
  (Utilities|FlowControl|Delay 1.0)
  (if (not _ispantin)
    (for _array_element (Variables|Default|GetLights)
      (Utilities|Array|Add (Variables|Default|GetIntensities) (Variables|/Script/Engine.LightComponentBase|GetIntensity (Variables|/Script/Engine.Light|GetLightComponent _array_element)))
      (Rendering|Components|Light|SetIntensity (Variables|/Script/Engine.Light|GetLightComponent _array_element) 0.0))
    (for _array_element_2 (Variables|Default|GetObjects)
      (Utilities|Array|Add (Variables|Default|GetMaterials) (Rendering|Material|GetMaterial (Variables|/Script/Engine.StaticMeshActor|GetStaticMeshComponent _array_element_2) 1))
      (Rendering|Material|SetMaterial (Variables|/Script/Engine.StaticMeshActor|GetStaticMeshComponent _array_element_2) 1 (Variables|Default|GetOffMat)))
    (for _array_element_3 (Variables|Default|GetHeavyLights)
      (Default|TurnOff _array_element_3))))

(event EventBeginPlay
  (Networking|SwitchHasAuthority
    (:Authority
      (EventDispatchers|BindEventtoGameStart (.GameMode (CallFunction|GetBPGameMode)) (delegate Custom|OnGameStartServer)))))

(fn ConstructionScript)