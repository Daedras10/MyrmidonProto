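; Trigger zone that reconfigures the local player's camera when a living BP_Pantin overlaps its box.
; It applies distance, preview and angle settings and assigns a camera rail, optionally cutting to position when the rail changes.
; The camera change requires the local controller's IsPantin check, retried once after a short delay.
; At game start, the server multicasts a forced check of Pantins already inside.
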(event OnComponentBeginOverlap(Box)
  (params (OverlappedComponent :type Primitive%20Component%20Object%20Reference) (OtherActor :type Actor%20Object%20Reference) (OtherComp :type Primitive%20Component%20Object%20Reference) (OtherBodyIndex :type Integer) (bFromSweep :type Boolean) (SweepResult :type Hit%20Result%20Structure%20%28by%20ref%29))
  (bind _asbp_pantin (Utilities|Casting|CastToBP_Pantin OtherActor))
  (CallFunction|OverlapPantin _asbp_pantin))

(event Custom|ForceCheck
  (for _array_element (Collision|GetOverlappingActors (Variables|Default|GetBox) "/Game/AssetsMyrmidon/Blueprints/Character/BP_Pantin.BP_Pantin_C" :!class /Script/Engine.PrimitiveComponent)
    (CallFunction|OverlapPantin (.AsBP%20Pantin (Utilities|Casting|CastToBP_Pantin _array_element)))))

(event Custom|OverlapPantin
  (params (Pantin :type BP%20Pantin%20Object%20Reference))
  (bind _playercontroller (CallFunction|GetBPLocalPlayerController))
  (bind _cam (Variables|/Game/AssetsMyrmidon/Blueprints/GameMode/BP_PlayerController.BP_PlayerController_C|GetCam _playercontroller))
  (Utilities|IsValid _playercontroller
    (:Is%20Valid
      (if (Variables|/Script/MyrmidonProto.PantinCharacter|GetIsAlive Pantin)
        (if (Variables|/Game/AssetsMyrmidon/Blueprints/GameMode/BP_PlayerController.BP_PlayerController_C|GetisPantin _playercontroller)
          (Default|SetupParameters _cam (Variables|Default|GetCamDistance) (Variables|Default|GetPreviewDist) (Variables|Default|GetCamAngle) :!label _label)
          (if (and (Variables|Default|GetCutToPosition) (!= (Variables|Default|GetCameraRail) (Variables|/Game/AssetsMyrmidon/Blueprints/Camera/BP_Camera.BP_Camera_C|GetCurrentRail _cam)))
            (Variables|/Game/AssetsMyrmidon/Blueprints/Camera/BP_Camera.BP_Camera_C|SetCurrentRail _cam (Variables|Default|GetCameraRail))
            (Default|CuttoPosition _cam))
          (Variables|/Game/AssetsMyrmidon/Blueprints/Camera/BP_Camera.BP_Camera_C|SetCurrentRail _cam (Variables|Default|GetCameraRail))
          (if (Variables|/Game/AssetsMyrmidon/Blueprints/GameMode/BP_PlayerController.BP_PlayerController_C|GetisPantin (.PlayerController (CallFunction|GetBPLocalPlayerController)))
            _)
          (else
            (Utilities|FlowControl|Delay 0.2)
            (if (Variables|/Game/AssetsMyrmidon/Blueprints/GameMode/BP_PlayerController.BP_PlayerController_C|GetisPantin (.PlayerController (CallFunction|GetBPLocalPlayerController)))
              (goto _label))))))))

(event Custom|OnGameStartServer
  (EventDispatchers|UnbindEventfromGameStart (.GameMode (CallFunction|GetBPGameMode)) (delegate Custom|OnGameStartServer))
  (CallFunction|OnGameStartMulticast))

(event Custom|OnGameStartMulticast
  (CallFunction|ForceCheck))

(event EventBeginPlay
  (Networking|SwitchHasAuthority
    (:Authority
      (EventDispatchers|BindEventtoGameStart (.GameMode (CallFunction|GetBPGameMode)) (delegate Custom|OnGameStartServer)))))

(fn ConstructionScript)