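; Trigger volume that switches the Pantin character into 2D side-view mode and registers itself as the camera's current 2D zone.
; TickCam snaps the character's XY to an optional 2dRail, using its velocity to move along it.
; The camera function returns a zone-aligned view at CameraDist, with velocity look-ahead clamped to local bounds.
; When another zone owns an overlapping character, input toward local -X hands control back to this one.
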(event OnComponentBeginOverlap(Box)
  (params (OverlappedComponent :type Primitive%20Component%20Object%20Reference) (OtherActor :type Actor%20Object%20Reference) (OtherComp :type Primitive%20Component%20Object%20Reference) (OtherBodyIndex :type Integer) (bFromSweep :type Boolean) (SweepResult :type Hit%20Result%20Structure%20%28by%20ref%29))
  ;[1 1 1] Overlap ( Start / End )
  (bind _asbp_pantin (Utilities|Casting|CastToBP_Pantin OtherActor))
  (CallFunction|Setup2DZone _asbp_pantin))

(event OnComponentEndOverlap(Box)
  (params (OverlappedComponent :type Primitive%20Component%20Object%20Reference) (OtherActor :type Actor%20Object%20Reference) (OtherComp :type Primitive%20Component%20Object%20Reference) (OtherBodyIndex :type Integer))
  ;[1 1 1] Overlap ( Start / End )
  (bind _asbp_pantin (Utilities|Casting|CastToBP_Pantin OtherActor))
  (bind _asbp_player_controller (Utilities|Casting|CastToBP_PlayerController (Game|GetPlayerController 0)))
  (Variables|Default|SetPantin 0)
  (if (== (Variables|/Game/AssetsMyrmidon/Blueprints/Character/BP_Pantin.BP_Pantin_C|Get2dZone _asbp_pantin) self)
    (Variables|/Game/AssetsMyrmidon/Blueprints/Camera/BP_Camera.BP_Camera_C|SetCurrent2DZone (Variables|/Game/AssetsMyrmidon/Blueprints/GameMode/BP_PlayerController.BP_PlayerController_C|GetCam _asbp_player_controller) 0)
    (Variables|/Game/AssetsMyrmidon/Blueprints/Character/BP_Pantin.BP_Pantin_C|Setin2D _asbp_pantin false)
    (Variables|/Game/AssetsMyrmidon/Blueprints/Character/BP_Pantin.BP_Pantin_C|Set2dZone _asbp_pantin 0)))

(event Custom|TickCam
  (params (DeltaSeconds :type Float%20%28double-precision%29))
  (bind _pantin (Variables|Default|GetPantin))
  (bind _2drail (Variables|Default|Get2dRail))
  (bind _returnvalue (Transformation|GetActorLocation _pantin))
  (bind _charactermovement (Variables|/Script/Engine.Character|GetCharacterMovement _pantin))
  (bind _z (Math|Vector|BreakVector _returnvalue))
  (bind _returnvalue_2 (Class|CharacterMovementComponent|GetImpartedMovementBaseVelocity _charactermovement))
  (bind _velocity (Variables|/Script/Engine.MovementComponent|GetVelocity _charactermovement))
  (bind _returnvalue_3 (+ _velocity _returnvalue_2))
  (bind (_x _y) (Math|Vector|BreakVector _returnvalue_3))
  ;[1 1 1] TickCam
  (Utilities|IsValid _pantin
    (:Is%20Valid
      (Utilities|IsValid _2drail
        (:Is%20Valid
          (bind _pos (Default|GetPlayerMovement _2drail (Math|Vector|MakeVector _x _y 0.0) DeltaSeconds))
          (Transformation|SetActorLocation _pantin (Math|Vector|Lerp(Vector) _returnvalue (Math|Vector|MakeVector (.X (Math|Vector|BreakVector _pos)) (.Y (Math|Vector|BreakVector _pos)) _z) 1.0) true false)
          (bind _pos_2 (Default|GetPlayerPos _2drail _returnvalue))
          (Transformation|SetActorLocation _pantin (Math|Vector|MakeVector (.X (Math|Vector|BreakVector _pos_2)) (.Y (Math|Vector|BreakVector _pos_2)) _z) true false))))))

(event Custom|Setup2DZone
  (params (Pantin :type BP%20Pantin%20Object%20Reference))
  (bind _2drail (Variables|Default|Get2dRail))
  ;[1 1 1] SetupZone
  (bind _asbp_player_controller (Utilities|Casting|CastToBP_PlayerController (Game|GetPlayerController 0)))
  (Variables|/Game/AssetsMyrmidon/Blueprints/Camera/BP_Camera.BP_Camera_C|SetCurrent2DZone (Variables|/Game/AssetsMyrmidon/Blueprints/GameMode/BP_PlayerController.BP_PlayerController_C|GetCam _asbp_player_controller) self)
  (bind _output_get (Variables|Default|SetPantin Pantin))
  (Variables|/Game/AssetsMyrmidon/Blueprints/Character/BP_Pantin.BP_Pantin_C|Setin2D _output_get true)
  (Variables|/Game/AssetsMyrmidon/Blueprints/Character/BP_Pantin.BP_Pantin_C|Set2dZone _output_get self)
  (Utilities|IsValid _2drail
    (:Is%20Valid
      (Default|GetPlayerPos _2drail (Transformation|GetActorLocation _output_get)))))

(event EventTick
  (params (DeltaSeconds :type Float%20%28single-precision%29))
  (bind _pantin (Variables|Default|GetPantin))
  ;[1 1 1] Event Tick
  (Utilities|IsValid _pantin
    (:Is%20Valid
      (if (not (== (Variables|/Game/AssetsMyrmidon/Blueprints/Character/BP_Pantin.BP_Pantin_C|Get2dZone _pantin) self))
        (if (< (.X (Math|Vector|BreakVector (Math|Transform|InverseTransformDirection (Transformation|GetActorTransform) (Pawn|Components|PawnMovement|GetLastInputVector (Variables|/Script/Engine.Character|GetCharacterMovement _pantin))))) -0.1)
          (CallFunction|Setup2DZone _pantin))))))

(fn ConstructionScript
  (Components|Box|SetBoxExtent (Variables|Default|GetBox) (Variables|Default|GetBoxExtents) false)
  (Transformation|SetRelativeLocation (Variables|Default|GetArrow) (Math|Vector|MakeVector (* (Variables|Default|GetCameraDist) -1.0) 0.0 0.0) false false))

(fn GetCameraLocationandRotation
  (params (PantinTransform :type BP%20Pantin%20Object%20Reference) (DeltaSeconds :type Float%20%28double-precision%29))
  (bind _returnvalue (Transformation|GetActorTransform))
  (bind _charactermovement (Variables|/Script/Engine.Character|GetCharacterMovement PantinTransform))
  (bind _camminbounds (Variables|Default|GetCamMinBounds))
  (bind _cammaxbounds (Variables|Default|GetCamMaxBounds))
  (bind _returnvalue_2 (Class|MovementComponent|GetMaxSpeed _charactermovement))
  (bind (_x _y _z) (Math|Vector|BreakVector _camminbounds))
  (bind (_x_2 _y_2 _z_2) (Math|Vector|BreakVector _cammaxbounds))
  (bind _velocity (Variables|/Script/Engine.MovementComponent|GetVelocity _charactermovement))
  (bind _returnvalue_3 (/ _velocity _returnvalue_2))
  (bind (_x_3 _y_3) (Math|Vector|BreakVector _returnvalue_3))
  (Variables|Default|SetPreviewDist (Math|Float|Lerp (Variables|Default|GetPreviewDist) (Variables|Default|GetCameraPreviewDist) DeltaSeconds))
  (return (+ (Math|Transform|TransformLocation _returnvalue (Math|Vector|MakeVector (* (Variables|Default|GetCameraDist) -1.0) (Math|Float|Clamp(Float) (.Y (Math|Vector|BreakVector (Math|Transform|InverseTransformLocation _returnvalue (+ (.Location (Math|Transform|BreakTransform (Transformation|GetActorTransform PantinTransform))) (* (Math|Vector|MakeVector _x_3 _y_3 0.0) (Variables|Default|GetPreviewDist)))))) _y _y_2) (Math|Float|Clamp(Float) (.Z (Math|Vector|BreakVector (Math|Transform|InverseTransformLocation _returnvalue (+ (.Location (Math|Transform|BreakTransform (Transformation|GetActorTransform PantinTransform))) (* (Math|Vector|MakeVector _x_3 _y_3 0.0) (Variables|Default|GetPreviewDist)))))) _z _z_2))) (Variables|Default|GetCameraOffset)) (Math|Transform|TransformRotation _returnvalue "0, 0, 0")))