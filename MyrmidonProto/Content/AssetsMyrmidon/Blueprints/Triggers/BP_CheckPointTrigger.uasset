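; BP_CheckPointTrigger is a trigger volume that records checkpoint progress and sets the camera rail when a living BP_Pantin enters it.
; On authority only, it raises the Pantin player state's checkpoint index to this trigger's index, never lowering it.
; If the local controller is the Pantin, it assigns this trigger's camera rail, first cutting the camera to position when CutToPosition is set and the rail differs.
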(event OnComponentBeginOverlap(Trigger)
  (params (OverlappedComponent :type Primitive%20Component%20Object%20Reference) (OtherActor :type Actor%20Object%20Reference) (OtherComp :type Primitive%20Component%20Object%20Reference) (OtherBodyIndex :type Integer) (bFromSweep :type Boolean) (SweepResult :type Hit%20Result%20Structure%20%28by%20ref%29))
  (bind _gamemode (CallFunction|GetBPGameMode))
  (bind _playercontroller (CallFunction|GetBPLocalPlayerController))
  (bind _playercontroller_2 (Default|GetBPPlayerController _gamemode true))
  (bind _cam (Variables|/Game/AssetsMyrmidon/Blueprints/GameMode/BP_PlayerController.BP_PlayerController_C|GetCam _playercontroller))
  (bind _playerstate (Default|GetPlayerState _playercontroller_2))
  (Networking|SwitchHasAuthority
    (:Authority
      (bind _asbp_pantin (Utilities|Casting|CastToBP_Pantin OtherActor))
      (if (Variables|/Script/MyrmidonProto.PantinCharacter|GetIsAlive _asbp_pantin)
        (Variables|/Script/MyrmidonProto.PantinAnimatorPlayerState|SetPantinCheckPointIndex _playerstate (Math|Integer|Max(Integer) (Variables|/Script/MyrmidonProto.PantinAnimatorPlayerState|GetPantinCheckPointIndex _playerstate) (Variables|Default|GetCheckpointIndex)))
        (if (Variables|/Game/AssetsMyrmidon/Blueprints/GameMode/BP_PlayerController.BP_PlayerController_C|GetisPantin (.PlayerController (CallFunction|GetBPLocalPlayerController)))
          (if (and (Variables|Default|GetCutToPosition) (!= (Variables|Default|GetCameraRail) (Variables|/Game/AssetsMyrmidon/Blueprints/Camera/BP_Camera.BP_Camera_C|GetCurrentRail _cam)))
            (Variables|/Game/AssetsMyrmidon/Blueprints/Camera/BP_Camera.BP_Camera_C|SetCurrentRail _cam (Variables|Default|GetCameraRail))
            (Default|CuttoPosition _cam))
          (Variables|/Game/AssetsMyrmidon/Blueprints/Camera/BP_Camera.BP_Camera_C|SetCurrentRail _cam (Variables|Default|GetCameraRail)))))))

(fn ConstructionScript)