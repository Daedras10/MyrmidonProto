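; BP_SequenceTrigger is a one-shot box trigger that registers a recorded sequence when a BP_Pantin overlaps it.
; On authority, the first such overlap sets a Triggered flag and calls AddRecordedSequence on the local player controller with the configured start offset, duration and camera index.
; The construction script sizes the box from Size; its unconnected nodes for positioning thin boxes along the Y edges never run.
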(event OnComponentBeginOverlap(Trigger)
  (params (OverlappedComponent :type Primitive%20Component%20Object%20Reference) (OtherActor :type Actor%20Object%20Reference) (OtherComp :type Primitive%20Component%20Object%20Reference) (OtherBodyIndex :type Integer) (bFromSweep :type Boolean) (SweepResult :type Hit%20Result%20Structure%20%28by%20ref%29))
  (Utilities|Casting|CastToBP_Pantin OtherActor)
  (Networking|SwitchHasAuthority
    (:Authority
      (Development|PrintString "COLLIDDED")
      (if (not (Variables|Default|GetTriggered))
        (Variables|Default|SetTriggered true)
        (Default|AddRecordedSequence (.PlayerController (CallFunction|GetBPLocalPlayerController)) (Variables|Default|GetSequenceStart) (Variables|Default|GetSequenceDuration) (Variables|Default|GetCameraIndex))
        (Development|PrintString "AddedRecordedSequence")))))

(fn ConstructionScript
  (Components|Box|SetBoxExtent (Variables|Default|GetTrigger) (Variables|Default|GetSize) true))