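; BP_CinematicTrigger is a server-side trigger volume that starts a cinematic when a living Pantin enters it.
; On overlap, authority casts the actor to BP_Pantin, checks it is alive and passes through a DoOnce, so it fires a single time.
; It then unlocks the configured Steam achievement and asks the game mode to start the cinematic by ID, with end positions and optional teleports for Pantin and Animator.
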(event OnComponentBeginOverlap(Trigger)
  (params (OverlappedComponent :type Primitive%20Component%20Object%20Reference) (OtherActor :type Actor%20Object%20Reference) (OtherComp :type Primitive%20Component%20Object%20Reference) (OtherBodyIndex :type Integer) (bFromSweep :type Boolean) (SweepResult :type Hit%20Result%20Structure%20%28by%20ref%29))
  (bind _gamemode (CallFunction|GetBPGameMode))
  (Networking|SwitchHasAuthority
    (:Authority
      (bind _asbp_pantin (Utilities|Casting|CastToBP_Pantin OtherActor))
      (if (Variables|/Script/MyrmidonProto.PantinCharacter|GetIsAlive _asbp_pantin)
        (Utilities|FlowControl|DoOnce false
          (:Completed
            (Default|Achievement _gamemode (Variables|Default|GetSteamAchievement))
            (Default|StartCinematicID _gamemode (Variables|Default|GetCinematicId) (Variables|Default|GetEndPosPantin) (Variables|Default|GetEndPosAnimator) (Variables|Default|GetShouldTPPantin) (Variables|Default|GetShouldTPAnimator))))))))

(fn ConstructionScript)