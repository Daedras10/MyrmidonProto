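; Parametric table actor that rebuilds its shape in the construction script from Size and Height variables.
; Size scales the Cube component and places four feet at its corners with a fixed inset.
; Each foot reuses the same corner offset, mirrored on X and Y by sign vectors.
; Height stretches the feet vertically and shifts them down to compensate.
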(fn ConstructionScript
  (bind _size (Variables|Default|GetSize))
  (bind _foot1 (Variables|Default|GetFoot1))
  (bind _height (Variables|Default|Getheight))
  (bind _foot2 (Variables|Default|GetFoot2))
  (bind _foot3 (Variables|Default|GetFoot3))
  (bind _foot4 (Variables|Default|GetFoot4))
  (bind (_x _y) (Math|Vector|BreakVector _size))
  (bind _returnvalue (* _height 0.1))
  (bind _returnvalue_2 (* _height -5.0))
  (bind _returnvalue_3 (Math|Vector|MakeVector 1.0 1.0 _returnvalue))
  (bind _returnvalue_4 (* _y 5e+01))
  (bind _returnvalue_5 (* _x 5e+01))
  (bind _returnvalue_6 (+ _returnvalue_2 5e+01))
  (bind _returnvalue_7 (- _returnvalue_4 1e+01))
  (bind _returnvalue_8 (- _returnvalue_5 1e+01))
  (bind _returnvalue_9 (Math|Vector|MakeVector _returnvalue_8 _returnvalue_7 _returnvalue_6))
  (Transformation|SetRelativeScale3D (Variables|Default|GetCube) _size)
  (Utilities|FlowControl|Sequence
    (:then_0
      (Transformation|SetRelativeLocation _foot1 _returnvalue_9 false false)
      (Transformation|SetRelativeScale3D _foot1 _returnvalue_3))
    (:then_1
      (Transformation|SetRelativeLocation _foot2 (* _returnvalue_9 "-1.000000,1.000000,1.000000") false false)
      (Transformation|SetRelativeScale3D _foot2 _returnvalue_3))
    (:then_2
      (Transformation|SetRelativeLocation _foot3 (* _returnvalue_9 "-1.000000,-1.000000,1.000000") false false)
      (Transformation|SetRelativeScale3D _foot3 _returnvalue_3))
    (:then_3
      (Transformation|SetRelativeLocation _foot4 (* _returnvalue_9 "1.000000,-1.000000,1.000000") false false)
      (Transformation|SetRelativeScale3D _foot4 _returnvalue_3))))