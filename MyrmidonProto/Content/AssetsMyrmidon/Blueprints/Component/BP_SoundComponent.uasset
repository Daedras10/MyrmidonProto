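; Sound component that manages the game's music tracks: intro, tutorial, village, Act 1 transition and village cinematic.
; On BeginPlay it creates a 2D sound for each track, scaled by the GameInstance music volume, and binds to the GameInstance Saved event to reapply that volume.
; Start and Stop events fade each track in and out.
; StartVillage retries each tick until its sound is valid.
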(event Custom|StartTransitionAct1
  (Audio|Components|Audio|FadeIn (Variables|Default|GetTransitionSound) 1.0 (CallFunction|Mult) 0.0 "Linear" :!class /Script/Engine.AudioComponent)
  (Development|PrintString "Arh" true true "(R=0.000000,G=0.660000,B=1.000000,A=1.000000)" 2e+03))

(event Custom|StopIntro
  (Audio|Components|Audio|FadeOut (Variables|Default|GetIntroSound) 0.5 0.0 "Linear" :!class /Script/Engine.AudioComponent))

(event Custom|StartVillage
  (bind _villagebgsound (Variables|Default|GetVillageBGSound))
  (Utilities|IsValid _villagebgsound :!label _label
    (:Is%20Valid
      (Audio|Components|Audio|FadeIn _villagebgsound 1.0 (CallFunction|Mult) 0.0 "Linear" :!class /Script/Engine.AudioComponent))
    (:Is%20Not%20Valid
      (Utilities|FlowControl|DelayUntilNextTick)
      (goto _label))))

(event Custom|StopVillage
  (Audio|Components|Audio|FadeOut (Variables|Default|GetVillageBGSound) 0.5 0.0 "Linear" :!class /Script/Engine.AudioComponent))

(event Custom|StartVillageCine
  (Audio|Components|Audio|FadeIn (Variables|Default|GetVillageCineSound) 1.0 (CallFunction|Mult) 0.0 "Linear" :!class /Script/Engine.AudioComponent))

(event Custom|StopVillageCine
  (Audio|Components|Audio|FadeOut (Variables|Default|GetVillageCineSound) 0.5 0.0 "Linear" :!class /Script/Engine.AudioComponent))

(event Custom|OnSoundChanged
  (for _array_element (Utilities|Array|MakeArray (Variables|Default|GetTutorialBGSound) (Variables|Default|GetVillageBGSound) (Variables|Default|GetTransitionSound) (Variables|Default|GetVillageCineSound) (Variables|Default|GetIntroSound))
    (Audio|Components|Audio|SetVolumeMultiplier _array_element (CallFunction|Mult) :!class /Script/Engine.AudioComponent)))

(event Custom|Saved_Event
  (CallFunction|OnSoundChanged))

(event Custom|CreateSounds
  (bind _val (CallFunction|Mult))
  (bind _returnvalue (Audio|CreateSound2D "/Game/AssetsMyrmidon/Sons/Musiques/MyrmidonTutoBGSound.MyrmidonTutoBGSound" _val 1.0 0.0 0))
  (Variables|Default|SetTutorialBGSound _returnvalue)
  (bind _returnvalue_2 (Audio|CreateSound2D "/Game/AssetsMyrmidon/Sons/Musiques/VillageBGSound.VillageBGSound" _val 1.0 0.0 0))
  (Variables|Default|SetVillageBGSound _returnvalue_2)
  (bind _returnvalue_3 (Audio|CreateSound2D "/Game/AssetsMyrmidon/Sons/Musiques/TransitionCineSound.TransitionCineSound" _val 1.0 0.0 0))
  (Variables|Default|SetTransitionSound _returnvalue_3)
  (bind _returnvalue_4 (Audio|CreateSound2D "/Game/AssetsMyrmidon/Sons/Musiques/VillageCineSound.VillageCineSound" _val 1.0 0.0 0))
  (Variables|Default|SetVillageCineSound _returnvalue_4)
  (bind _returnvalue_5 (Audio|CreateSound2D "/Game/AssetsMyrmidon/Sons/Musiques/IntroSound.IntroSound" _val 1.0 0.0 0))
  (Variables|Default|SetIntroSound _returnvalue_5))

(event Custom|StartIntro
  (Audio|Components|Audio|FadeIn (Variables|Default|GetIntroSound) 1.0 (CallFunction|Mult) 0.0 "Linear" :!class /Script/Engine.AudioComponent))

(event Custom|StopTransitionAct1
  (Audio|Components|Audio|FadeOut (Variables|Default|GetTransitionSound) 0.5 0.0 "Linear" :!class /Script/Engine.AudioComponent))

(event Custom|StartTutorial
  (Audio|Components|Audio|FadeIn (Variables|Default|GetTutorialBGSound) 1.0 (CallFunction|Mult) 0.0 "Linear" :!class /Script/Engine.AudioComponent))

(event Custom|StopTutorial
  (Audio|Components|Audio|FadeOut (Variables|Default|GetTutorialBGSound) 0.5 0.0 "Linear" :!class /Script/Engine.AudioComponent))

(event EventBeginPlay
  (bind _output_get (Variables|Default|SetGame%20Instance (.GameInstance (CallFunction|GetBPGameInstance))))
  (EventDispatchers|AssignSaved _output_get (delegate Custom|Saved_Event))
  (CallFunction|CreateSounds))

(fn Mult
  (return (Default|GetMusicVolume (Variables|Default|GetGame%20Instance))))