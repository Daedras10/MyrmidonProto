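; BP_SteamAchievementComponent is a player controller component that unlocks Steam achievements.
; AddSteamAchievement converts an achievement enum to its string name and prints a warning when that resolves to "None".
; Otherwise it prints the name, caches achievements for the owning BP_PlayerController, and on success writes that achievement's progress as complete.
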(event EventAddSteamAchievement
  (params (Achievement :type ESteamAchievement%20Enum :default "ACHIEVEMENT_ACTION"))
  (bind _returnvalue (Class|SteamAchievementComponent|EnumtoStringAchievement Achievement))
  (bind _returnvalue_2 (Components|GetOwner))
  (bind _asbp_player_controller (Utilities|Casting|CastToBP_PlayerController _returnvalue_2))
  (if (Utilities|Enum|Equal(Enum) _returnvalue "None")
    (Development|PrintText (Utilities|Text|FormatText "Achievement not implemented: {ach}" (Utilities|String|EnumtoString Achievement)) true true "(R=1.000000,G=0.000000,B=0.024040,A=1.000000)" 4e+01)
    (else
      (Development|PrintString _returnvalue true true "(R=0.000000,G=1.000000,B=0.155676,A=1.000000)" 1e+01)
      (|CacheAchievements _asbp_player_controller
        (:OnSuccess
          (|WriteAchievementProgress _asbp_player_controller (Utilities|String|StringToName _returnvalue) 1.0))))))