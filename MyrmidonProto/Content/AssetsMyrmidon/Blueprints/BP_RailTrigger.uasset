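; Trigger volume that switches the player camera's rail as BP_Pantin passes through it.
; Thin boxes at both Y ends, laid out from Size in the construction script, record which side the Pantin last touched.
; Leaving the main box applies that side's rail and camera angle offset, starts a camera transition and shows cinematic borders if the rail is valid.
; The switch is skipped during replays or when the player controller is not Pantin.
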(event OnComponentEndOverlap(Trigger)
  (params (OverlappedComponent :type Primitive%20Component%20Object%20Reference) (OtherActor :type Actor%20Object%20Reference) (OtherComp :type Primitive%20Component%20Object%20Reference) (OtherBodyIndex :type Integer))
  (bind _returnvalue (Game|GetPlayerController 0))
  (bind _entrystate (Variables|Default|GetentryState))
  (bind _asbp_player_controller (Utilities|Casting|CastToBP_PlayerController _returnvalue))
  (bind _asbp_pantin (Utilities|Casting|CastToBP_Pantin OtherActor))
  (if (not (Variables|/Game/AssetsMyrmidon/Blueprints/GameMode/BP_GameInstance.BP_GameInstance_C|GetinReplay (.AsBP%20Game%20Instance (Utilities|Casting|CastToBP_GameInstance (Game|GetGameInstance)))))
    (if (Variables|/Game/AssetsMyrmidon/Blueprints/BP_PlayerController.BP_PlayerController_C|GetisPantin _asbp_player_controller)
      (bind _output_get (Variables|/Game/AssetsMyrmidon/Blueprints/BP_Camera.BP_Camera_C|SetCurrentRail (Variables|/Game/AssetsMyrmidon/Blueprints/BP_PlayerController.BP_PlayerController_C|GetCam _asbp_player_controller) (select _entrystate (Variables|Default|GetRailEntry) (Variables|Default|GetRailExit))))
      (Default|SetCinematicBorders _asbp_player_controller (Utilities|IsValid _output_get))
      (Default|SetCameraAngleOffset _asbp_pantin (Math|Float|SelectFloat (Variables|Default|GetCamAngleEntry) (Variables|Default|GetCamAngleExit) _entrystate))
      (Variables|/Game/AssetsMyrmidon/Blueprints/BP_Camera.BP_Camera_C|SetinTransition (Variables|/Game/AssetsMyrmidon/Blueprints/BP_PlayerController.BP_PlayerController_C|GetCam _asbp_player_controller) true))))

(event OnComponentBeginOverlap(EntryTrigger)
  (params (OverlappedComponent :type Primitive%20Component%20Object%20Reference) (OtherActor :type Actor%20Object%20Reference) (OtherComp :type Primitive%20Component%20Object%20Reference) (OtherBodyIndex :type Integer) (bFromSweep :type Boolean) (SweepResult :type Hit%20Result%20Structure%20%28by%20ref%29))
  (Utilities|Casting|CastToBP_Pantin OtherActor)
  (Variables|Default|SetentryState true))

(event OnComponentBeginOverlap(ExitTrigger)
  (params (OverlappedComponent :type Primitive%20Component%20Object%20Reference) (OtherActor :type Actor%20Object%20Reference) (OtherComp :type Primitive%20Component%20Object%20Reference) (OtherBodyIndex :type Integer) (bFromSweep :type Boolean) (SweepResult :type Hit%20Result%20Structure%20%28by%20ref%29))
  (Utilities|Casting|CastToBP_Pantin OtherActor)
  (Variables|Default|SetentryState false))

(fn ConstructionScript
  (bind _size (Variables|Default|GetSize))
  (bind _entrytrigger (Variables|Default|GetEntryTrigger))
  (bind _exittrigger (Variables|Default|GetExitTrigger))
  (bind (_x _y _z) (Math|Vector|BreakVector _size))
  (bind _returnvalue (Math|Vector|MakeVector _x 1e+01 _z))
  (Components|Box|SetBoxExtent (Variables|Default|GetTrigger) _size true)
  (Components|Box|SetBoxExtent _entrytrigger _returnvalue true)
  (Transformation|SetRelativeLocation _entrytrigger (Math|Vector|MakeVector 0.0 (+ (* _y -1.0) 5.0) 0.0) false false)
  (Components|Box|SetBoxExtent _exittrigger _returnvalue true)
  (Transformation|SetRelativeLocation _exittrigger (Math|Vector|MakeVector 0.0 (+ _y -5.0) 0.0) false false))