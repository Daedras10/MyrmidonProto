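; BP_Windmill is a rotating windmill with four platforms that stay level while it turns.
; Tick advances an angle by Speed, and SetAngles applies it to the Cylinder, then resets each platform's world rotation to zero.
; The construction script scales both Pale blades by the Lenght variable and applies the starting angle.
; An OnRep function for a replicated angle exists but is empty.
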(event EventTick
  (params (DeltaSeconds :type Float%20%28single-precision%29))
  (Variables|Default|SetAngle (+ (* DeltaSeconds (Variables|Default|GetSpeed)) (Variables|Default|GetAngle)))
  (CallFunction|SetAngles))

(fn ConstructionScript
  (bind _lenght (Variables|Default|GetLenght))
  (bind _returnvalue (Math|Vector|MakeVector 0.2 _lenght 2.0))
  (Transformation|SetRelativeScale3D (Variables|Default|GetPale) _returnvalue)
  (Transformation|SetRelativeScale3D (Variables|Default|GetPale2) _returnvalue)
  (CallFunction|SetAngles))

(fn SetAngles
  (Transformation|SetRelativeRotation (Variables|Default|GetCylinder) (Math|Rotator|MakeRotator 9e+01 (Variables|Default|GetAngle) 9e+01) false false)
  (Transformation|SetWorldRotation (Variables|Default|GetPlatform1) "0, 0, 0" false false)
  (Transformation|SetWorldRotation (Variables|Default|GetPlatform2) "0, 0, 0" false false)
  (Transformation|SetWorldRotation (Variables|Default|GetPlatform3) "0, 0, 0" false false)
  (Transformation|SetWorldRotation (Variables|Default|GetPlatform4) "0, 0, 0" false false))

(fn OnRepReplicatedAngle)