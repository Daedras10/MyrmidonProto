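; Gameplay camera actor that registers with the local player controller and follows the Pantin character.
; Tick eases toward the CurrentRail's position, rotation and FOV, or otherwise a configurable angle and distance, using velocity-based preview offsets and zeroing roll.
; Both modes update depth-of-field focal distance.
; CutToPosition snaps instantly, still supporting obsolete 2D zones that Tick ignores; the CameraTransition timeline is disconnected.
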(event Custom|RailCamInstant
  (bind _camera (Variables|Default|GetCamera))
  (bind _pantin (Variables|Default|GetPantin))
  (bind _returnvalue (Transformation|GetActorTransform _pantin))
  (bind _charactermovement (Variables|/Script/Engine.Character|GetCharacterMovement _pantin))
  ;[1 1 1] Rail Cam Instant
  (bind (_pos _rot _fov) (Default|GetCameraPosandRot (Variables|Default|GetCurrentRail) (Transformation|GetActorTransform) _returnvalue (* (* (/ (Variables|/Script/Engine.MovementComponent|GetVelocity _charactermovement) (Class|MovementComponent|GetMaxSpeed _charactermovement)) "1.000000,1.000000,0.000000") (Variables|Default|GetPreviewDistance))))
  (Transformation|SetActorLocationAndRotation _pos _rot)
  (Utilities|Struct|SetmembersinPostProcessSettings (Variables|/Script/Engine.CameraComponent|GetPostProcessSettings _camera) (Math|Vector|Distance(Vector) _pos (.Location (Math|Transform|BreakTransform _returnvalue))))
  (Camera|SetFieldOfView _camera _fov))

(event Custom|CameraTransition
  (params (Pos :type Vector) (Rot :type Rotator))
  ;[1 1 1] Camera Transition
  (Utilities|FlowControl|DoOnce false))

(event Custom|2DCamInstant
  ;[1 0.3499 0.3001] 2D Cam Instant ( Obsolete )
  (bind _location (Default|GetCameraLocationandRotation (Variables|Default|GetCurrent2DZone) (Variables|Default|GetPantin) 1.0))
  (Transformation|SetActorLocationAndRotation _location (.Rotation (Math|Transform|BreakTransform (Transformation|GetActorTransform)))))

(event Custom|ClassicCamInstant
  (bind _currentdistance (Variables|Default|GetCurrentDistance))
  (bind _currentrot (Variables|Default|GetCurrentRot))
  ;[1 1 1] Classic Cam Instant
  (Transformation|SetActorLocationAndRotation (CallFunction|GetPositionfromRotation (Transformation|GetActorLocation (Variables|Default|GetPantin)) _currentrot _currentdistance) _currentrot)
  (Utilities|Struct|SetmembersinPostProcessSettings (Variables|/Script/Engine.CameraComponent|GetPostProcessSettings (Variables|Default|GetCamera)) _currentdistance))

(event Custom|SetupParameters
  (params (Dist :type Float%20%28double-precision%29) (Preview :type Float%20%28double-precision%29) (Angle :type Rotator))
  ;[1 1 1] Setup Parameters
  (Variables|Default|SetCurrentRot Angle)
  (Variables|Default|SetCurrentDistance Dist)
  (Variables|Default|SetPreviewDistance Preview))

(event Custom|RailCamera
  (params (deltaSeconds :type Float%20%28double-precision%29))
  (bind _returnvalue (Transformation|GetActorTransform))
  (bind _returnvalue_2 (* deltaSeconds 3.0))
  (bind _pantin (Variables|Default|GetPantin))
  (bind _camera (Variables|Default|GetCamera))
  (bind _returnvalue_3 (Transformation|GetActorTransform _pantin))
  (bind (_location _rotation) (Math|Transform|BreakTransform _returnvalue))
  (bind _charactermovement (Variables|/Script/Engine.Character|GetCharacterMovement _pantin))
  ;[1 1 1] Set Camera Pos to Rail
  (bind (_pos _rot _fov) (Default|GetCameraPosandRot (Variables|Default|GetCurrentRail) _returnvalue _returnvalue_3 (* (* (/ (Variables|/Script/Engine.MovementComponent|GetVelocity _charactermovement) (Class|MovementComponent|GetMaxSpeed _charactermovement)) "1.000000,1.000000,0.000000") (Variables|Default|GetPreviewDistance))))
  (Transformation|SetActorLocationAndRotation (Math|Vector|Lerp(Vector) _location _pos _returnvalue_2) (Math|Rotator|Lerp(Rotator) _rotation _rot _returnvalue_2 true))
  (Utilities|Struct|SetmembersinPostProcessSettings (Variables|/Script/Engine.CameraComponent|GetPostProcessSettings _camera) (Math|Vector|Distance(Vector) (Math|Vector|Lerp(Vector) _location _pos _returnvalue_2) (.Location (Math|Transform|BreakTransform _returnvalue_3))))
  (Camera|SetFieldOfView _camera (Math|Float|Lerp (Variables|/Script/Engine.CameraComponent|GetFieldOfView _camera) _fov _returnvalue_2)))

(event Custom|SetCamera
  (params (DeltaSeconds :type Float%20%28double-precision%29))
  (bind _returnvalue (Transformation|GetActorTransform))
  (bind _returnvalue_2 (* DeltaSeconds 3.0))
  (bind _pantin (Variables|Default|GetPantin))
  (bind _currentrot (Variables|Default|GetCurrentRot))
  (bind _currentdistance (Variables|Default|GetCurrentDistance))
  (bind (_location _rotation) (Math|Transform|BreakTransform _returnvalue))
  (bind _charactermovement (Variables|/Script/Engine.Character|GetCharacterMovement _pantin))
  ;[1 1 1] Set Camera
  (Transformation|SetActorLocationAndRotation (Math|Vector|Lerp(Vector) (+ _location (* (* (/ (Variables|/Script/Engine.MovementComponent|GetVelocity _charactermovement) (Class|MovementComponent|GetMaxSpeed _charactermovement)) "1.000000,1.000000,0.000000") (Variables|Default|GetPreviewDistance))) (CallFunction|GetPositionfromRotation (Transformation|GetActorLocation _pantin) _currentrot _currentdistance) _returnvalue_2) (Math|Rotator|Lerp(Rotator) _rotation _currentrot _returnvalue_2 true))
  (Utilities|Struct|SetmembersinPostProcessSettings (Variables|/Script/Engine.CameraComponent|GetPostProcessSettings (Variables|Default|GetCamera)) _currentdistance))

(event Custom|2DCamera
  (params (DeltaSeconds :type Float%20%28double-precision%29))
  (bind _returnvalue (Transformation|GetActorTransform))
  (bind _returnvalue_2 (* DeltaSeconds 3.0))
  (bind (_location _rotation) (Math|Transform|BreakTransform _returnvalue))
  ;[1 0.4226 0.3728] 2D Camera ( obsolete )
  (bind (_location_2 _rotation_2) (Default|GetCameraLocationandRotation (Variables|Default|GetCurrent2DZone) (Variables|Default|GetPantin) DeltaSeconds))
  (Transformation|SetActorLocationAndRotation (Math|Vector|Lerp(Vector) _location _location_2 _returnvalue_2) (Math|Rotator|Lerp(Rotator) _rotation _rotation_2 _returnvalue_2 true)))

(event EventTick
  (params (DeltaSeconds :type Float%20%28single-precision%29))
  (bind _returnvalue (Transformation|GetActorRotation))
  (bind _local_player_controller (Variables|Default|GetLocal%20Player%20Controller))
  (bind (_roll _pitch _yaw) (Math|Rotator|BreakRotator _returnvalue))
  ;[1 1 1] Event Tick
  (Utilities|IsValid _local_player_controller
    (:Is%20Valid
      (if (Variables|/Game/AssetsMyrmidon/Blueprints/GameMode/BP_PlayerController.BP_PlayerController_C|GetisPantin _local_player_controller)
        (Utilities|IsValid (Variables|Default|GetPantin)
          (:Is%20Valid
            (Utilities|IsValid (Variables|Default|GetCurrentRail)
              (:Is%20Valid
                (CallFunction|RailCamera DeltaSeconds))
              (:Is%20Not%20Valid
                (CallFunction|SetCamera DeltaSeconds)))
            (Transformation|SetActorRotation (Math|Rotator|MakeRotator 0.0 _pitch _yaw))))))))

(event EventBeginPlay
  (bind (_playercontroller _castsuccesful) (CallFunction|GetBPLocalPlayerController))
  ;[1 1 1] BeginPlay
  (if _castsuccesful
    (Variables|/Game/AssetsMyrmidon/Blueprints/GameMode/BP_PlayerController.BP_PlayerController_C|SetCam _playercontroller self)
    (Variables|Default|SetLocal%20Player%20Controller _playercontroller)))

(fn ConstructionScript)

(fn GetPositionfromRotation
  (params (Origin :type Vector) (Rot :type Rotator) (Dist :type Float%20%28double-precision%29))
  (return (+ Origin (Math|Vector|RotateVector (Math|Vector|MakeVector (* Dist -1.0) 0.0 0.0) Rot))))

(fn CuttoPosition
  (bind _returnvalue (Transformation|GetActorRotation))
  (bind (_roll _pitch _yaw) (Math|Rotator|BreakRotator _returnvalue))
  (Utilities|IsValid (Variables|Default|GetPantin)
    (:Is%20Valid
      (Utilities|IsValid (Variables|Default|GetCurrentRail)
        (:Is%20Valid
          (CallFunction|RailCamInstant))
        (:Is%20Not%20Valid
          (Utilities|IsValid (Variables|Default|GetCurrent2DZone)
            (:Is%20Valid
              (CallFunction|2DCamInstant))
            (:Is%20Not%20Valid
              (CallFunction|ClassicCamInstant)))))
      (Transformation|SetActorRotation (Math|Rotator|MakeRotator 0.0 _pitch _yaw)))))