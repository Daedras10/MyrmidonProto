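; BP_2DRail is a spline rail that constrains player movement to a path, likely for 2D-style sections.
; GetPlayerPos snaps a world position to a stored distance along the spline.
; GetPlayerMovement advances that distance by input magnitude, signed against the tangent, and returns the new world location.
; ForwardSide flips the rail's direction, and an arrow component marks the current point and tangent, including at construction.
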(fn ConstructionScript
  (CallFunction|SetArrow))

(fn GetPlayerMovement
  (params (Movement :type Vector) (DeltaTime :type Float%20%28double-precision%29))
  (bind (_x _y) (Math|Vector|BreakVector Movement))
  (bind _output_get (Variables|Default|SetPantinPosition (+ (* (Math|Float|SelectFloat 1.0 -1.0 (> (Math|Vector|DotProduct (* (Math|Vector|Normalize (CallFunction|GetTangent)) -1.0) (Math|Vector|MakeVector _x _y 0.0)) 0.0)) (Math|Vector|VectorLength Movement) (Math|Float|SelectFloat -0.2 0.2 (Variables|Default|GetForwardSide)) DeltaTime) (Variables|Default|GetPantinPosition))))
  (CallFunction|SetArrow)
  (return (Spline|GetLocationatDistanceAlongSpline (Variables|Default|GetSpline) _output_get "World")))

(fn GetPlayerPos
  (params (PlayerPos :type Vector))
  (bind _spline (Variables|Default|GetSpline))
  (bind _output_get (Variables|Default|SetPantinPosition (Class|SplineComponent|GetDistanceAlongSplineatLocation _spline PlayerPos "World")))
  (return (Spline|GetLocationatDistanceAlongSpline _spline _output_get "World")))

(fn GetTangent
  (return (* (Spline|GetTangentatDistanceAlongSpline (Variables|Default|GetSpline) (Variables|Default|GetPantinPosition) "World") (Math|Float|SelectFloat 1.0 -1.0 (Variables|Default|GetForwardSide)))))

(fn SetArrow
  (Transformation|SetRelativeLocationAndRotation (Variables|Default|GetArrow) (Spline|GetLocationatDistanceAlongSpline (Variables|Default|GetSpline) (Variables|Default|GetPantinPosition) "Local") (Math|Rotator|FindLookatRotation (Math|Vector|MakeVector 0.0 0.0 0.0) (CallFunction|GetTangent)) false false))