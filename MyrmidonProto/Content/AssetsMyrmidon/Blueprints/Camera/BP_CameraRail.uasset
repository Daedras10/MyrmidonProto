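; Camera rail that supplies position, rotation and FOV for a camera following the player (Pantin) along a spline.
; Curve points keyed by spline distance hold rotation, FOV, target and camera offsets, linearly interpolated between neighbors.
; The camera sits at the spline point nearest the player plus preview and target offset, shifted by its offset, using rail rotation or look-at.
; Construction script draws an arrow per point, clamped to spline length.
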(fn ConstructionScript
  (bind _spline (Variables|Default|GetSpline))
  (bind _arrows (Variables|Default|GetArrows))
  (bind _curvepoints (Variables|Default|GetCurvePoints))
  (for _array_element _arrows
    (Components|DestroyComponent _array_element))
  (Utilities|Array|Clear _arrows)
  (for (_ _array_index) _curvepoints
    (bind _structout (Utilities|Struct|SetmembersinSTRUCT_CurvePoint (Utilities|Array|Get(acopy) _curvepoints _array_index) (Math|Float|Clamp(Float) (.DistanceAlongCurve (Utilities|Struct|BreakSTRUCT_CurvePoint (Utilities|Array|Get(acopy) _curvepoints _array_index))) 0.0 (Spline|GetSplineLength _spline))))
    (AddComponent|AddArrowComponent false (Math|Transform|MakeTransform (Spline|GetLocationatDistanceAlongSpline _spline (.DistanceAlongCurve (Utilities|Struct|BreakSTRUCT_CurvePoint _structout)) "Local") (.Rotation (Utilities|Struct|BreakSTRUCT_CurvePoint _structout))))))

(fn GetCameraPosandRot
  (params (Transform :type Transform) (PantinTransform :type Transform) (Preview :type Vector))
  (bind _location (Math|Transform|BreakTransform PantinTransform))
  (bind _spline (Variables|Default|GetSpline))
  (bind (_rotation _offset _fov _camoffset) (CallFunction|GetCurveInfoatAlpha (Class|SplineComponent|GetDistanceAlongSplineatLocation _spline (+ Preview _location (Variables|Default|GetTargetOffset)) "World")))
  (bind _offset_2 (CallFunction|GetCurveInfoatAlpha (Class|SplineComponent|GetDistanceAlongSplineatLocation _spline _location "World")))
  (Variables|Default|SetTargetOffset _offset_2)
  (return (+ (Math|Transform|TransformDirection Transform _camoffset) (Spline|GetLocationatDistanceAlongSpline _spline (Class|SplineComponent|GetDistanceAlongSplineatLocation _spline (+ Preview _location (Variables|Default|GetTargetOffset)) "World") "World")) (Math|Rotator|SelectRotator (Math|Rotator|FindLookatRotation (.Location (Math|Transform|BreakTransform Transform)) (.Location (Math|Transform|BreakTransform PantinTransform))) (Math|Transform|TransformRotation (Transformation|GetActorTransform) _rotation) (Variables|Default|GetLookAtPlayer)) _fov))

(fn GetCurveInfoatAlpha
  (params (Alpha :type Float%20%28double-precision%29))
  (bind _curvepoints (Variables|Default|GetCurvePoints))
  (bind _index (Utilities|FlowControl|ForLoopwithBreak 1 (Utilities|Array|Length _curvepoints))
    (:LoopBody
      (if (<= Alpha (.DistanceAlongCurve (Utilities|Struct|BreakSTRUCT_CurvePoint (Utilities|Array|Get(acopy) _curvepoints _index))))
        (return (Math|Rotator|Lerp(Rotator) (.Rotation (Utilities|Struct|BreakSTRUCT_CurvePoint (Utilities|Array|Get(acopy) _curvepoints (- _index 1)))) (.Rotation (Utilities|Struct|BreakSTRUCT_CurvePoint (Utilities|Array|Get(acopy) _curvepoints _index))) (/ (- Alpha (.DistanceAlongCurve (Utilities|Struct|BreakSTRUCT_CurvePoint (Utilities|Array|Get(acopy) _curvepoints (- _index 1))))) (- (.DistanceAlongCurve (Utilities|Struct|BreakSTRUCT_CurvePoint (Utilities|Array|Get(acopy) _curvepoints _index))) (.DistanceAlongCurve (Utilities|Struct|BreakSTRUCT_CurvePoint (Utilities|Array|Get(acopy) _curvepoints (- _index 1)))))) true) (Math|Vector|Lerp(Vector) (.Offset (Utilities|Struct|BreakSTRUCT_CurvePoint (Utilities|Array|Get(acopy) _curvepoints (- _index 1)))) (.Offset (Utilities|Struct|BreakSTRUCT_CurvePoint (Utilities|Array|Get(acopy) _curvepoints _index))) (/ (- Alpha (.DistanceAlongCurve (Utilities|Struct|BreakSTRUCT_CurvePoint (Utilities|Array|Get(acopy) _curvepoints (- _index 1))))) (- (.DistanceAlongCurve (Utilities|Struct|BreakSTRUCT_CurvePoint (Utilities|Array|Get(acopy) _curvepoints _index))) (.DistanceAlongCurve (Utilities|Struct|BreakSTRUCT_CurvePoint (Utilities|Array|Get(acopy) _curvepoints (- _index 1))))))) (Math|Float|Lerp (.FOV (Utilities|Struct|BreakSTRUCT_CurvePoint (Utilities|Array|Get(acopy) _curvepoints (- _index 1)))) (.FOV (Utilities|Struct|BreakSTRUCT_CurvePoint (Utilities|Array|Get(acopy) _curvepoints _index))) (/ (- Alpha (.DistanceAlongCurve (Utilities|Struct|BreakSTRUCT_CurvePoint (Utilities|Array|Get(acopy) _curvepoints (- _index 1))))) (- (.DistanceAlongCurve (Utilities|Struct|BreakSTRUCT_CurvePoint (Utilities|Array|Get(acopy) _curvepoints _index))) (.DistanceAlongCurve (Utilities|Struct|BreakSTRUCT_CurvePoint (Utilities|Array|Get(acopy) _curvepoints (- _index 1))))))) (Math|Vector|Lerp(Vector) (.CamOffset (Utilities|Struct|BreakSTRUCT_CurvePoint (Utilities|Array|Get(acopy) _curvepoints (- _index 1)))) (.CamOffset (Utilities|Struct|BreakSTRUCT_CurvePoint (Utilities|Array|Get(acopy) _curvepoints _index))) (/ (- Alpha (.DistanceAlongCurve (Utilities|Struct|BreakSTRUCT_CurvePoint (Utilities|Array|Get(acopy) _curvepoints (- _index 1))))) (- (.DistanceAlongCurve (Utilities|Struct|BreakSTRUCT_CurvePoint (Utilities|Array|Get(acopy) _curvepoints _index))) (.DistanceAlongCurve (Utilities|Struct|BreakSTRUCT_CurvePoint (Utilities|Array|Get(acopy) _curvepoints (- _index 1))))))))))
    (:Completed
      (return "0, 0, 0" "0, 0, 0" 9e+01 "0, 0, 0"))))