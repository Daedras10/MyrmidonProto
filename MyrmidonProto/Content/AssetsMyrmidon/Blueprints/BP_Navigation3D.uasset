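; BP_Navigation3D is a 3D navigation actor that finds paths between points and writes them into its spline.
; GetPath calls FindPath between a given start and end, returning the path; its return sits inside the point loop, so only the first point reaches the spline.
; The go event tests this between Target1 and Target2, offset from the actor's location, printing results and rebuilding the full spline.
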(event Custom|go
  (bind _returnvalue (Transformation|GetActorLocation))
  (bind (_out_path _returnvalue_2) (Class|NavigationVolume3D|FindPath (+ (Variables|Default|GetTarget1) _returnvalue) (+ _returnvalue (Variables|Default|GetTarget2)) (Utilities|Array|MakeArray)))
  (Development|PrintString (Utilities|String|ToString(Boolean) _returnvalue_2))
  (if _returnvalue_2
    (Spline|ClearSplinePoints (Variables|Default|GetSpline) true)
    (for _array_element _out_path
      (Development|PrintString (Utilities|String|ToString(Vector) _array_element) true true "(R=0.000000,G=0.660000,B=1.000000,A=1.000000)" 2e+01)
      (Spline|AddSplinePoint (Variables|Default|GetSpline) _array_element "World" true))))

(event EventBeginPlay)

(event Collision|EventActorBeginOverlap
  (params (OtherActor :type Actor%20Object%20Reference)))

(event EventTick
  (params (DeltaSeconds :type Float%20%28single-precision%29)))

(fn ConstructionScript)

(fn GetPath
  (params (Start :type Vector) (End :type Vector))
  (bind (_out_path _returnvalue) (Class|NavigationVolume3D|FindPath Start End (Utilities|Array|MakeArray)))
  (if _returnvalue
    (Spline|ClearSplinePoints (Variables|Default|GetSpline) true)
    (for _array_element _out_path
      (Spline|AddSplinePoint (Variables|Default|GetSpline) _array_element "World" true)
      (return _out_path))
    (else
      (return _out_path))))