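; BP_RopesMove is a level-art actor, named for ropes, that moves its mesh when something enters its trigger box.
; Box overlap plays a Timeline that drives the mesh's relative location.
; On exit, a retriggerable 1.5-second delay reverses the Timeline only if the IsUnder flag is still false.
; The construction script picks a random mesh from the Meshes array and disables its collision.
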(event OnComponentBeginOverlap(Box)
  (params (OverlappedComponent :type Primitive%20Component%20Object%20Reference) (OtherActor :type Actor%20Object%20Reference) (OtherComp :type Primitive%20Component%20Object%20Reference) (OtherBodyIndex :type Integer) (bFromSweep :type Boolean) (SweepResult :type Hit%20Result%20Structure%20%28by%20ref%29))
  (Variables|Default|SetisUnder true)
  (bind _newtrack_1 (Timeline|Timeline Play)
    (:Update
      (Transformation|SetRelativeLocation (Variables|Default|GetStaticMesh) _newtrack_1 true false))))

(event OnComponentEndOverlap(Box)
  (params (OverlappedComponent :type Primitive%20Component%20Object%20Reference) (OtherActor :type Actor%20Object%20Reference) (OtherComp :type Primitive%20Component%20Object%20Reference) (OtherBodyIndex :type Integer))
  (Variables|Default|SetisUnder false)
  (Utilities|FlowControl|RetriggerableDelay 1.5)
  (if (not (Variables|Default|GetisUnder))
    (bind _newtrack_1 (Timeline|Timeline Reverse)
      (:Update
        (Transformation|SetRelativeLocation (Variables|Default|GetStaticMesh) _newtrack_1 true false)))))

(fn ConstructionScript
  (bind _staticmesh (Variables|Default|GetStaticMesh))
  (bind _meshes (Variables|Default|GetMeshes))
  (Components|StaticMesh|SetStaticMesh _staticmesh (Utilities|Array|Get(acopy) _meshes (Math|Random|RandomInteger (Utilities|Array|Length _meshes))))
  (Collision|SetCollisionEnabled _staticmesh "NoCollision"))