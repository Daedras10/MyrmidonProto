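; BP_Navette is a shuttle ("navette") prop with animated doors, wheels, cog and ropes, driven by three overlap triggers.
; The first opens two doors; the second closes them and starts the machinery; the third reverses the machinery and opens another door, then stops it.
; Timelines rotate the doors and feed a scaled Time parameter to dynamic materials created at construction, faking mechanical motion at differing rates.
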(event OnComponentBeginOverlap(Box)
  (params (OverlappedComponent :type Primitive%20Component%20Object%20Reference) (OtherActor :type Actor%20Object%20Reference) (OtherComp :type Primitive%20Component%20Object%20Reference) (OtherBodyIndex :type Integer) (bFromSweep :type Boolean) (SweepResult :type Hit%20Result%20Structure%20%28by%20ref%29))
  (Utilities|FlowControl|Delay 1.0)
  (bind _trackrotation (Timeline|Timeline Play)
    (:Update
      (Transformation|SetRelativeRotation (Variables|Default|GetSM_NavetteDoor_01) (Math|Rotator|MakeRotator 0.0 0.0 _trackrotation) false false)
      (Utilities|FlowControl|Delay 0.2)
      (Transformation|SetRelativeRotation (Variables|Default|GetSM_NavetteDoor_02) (Class|KismetMathLibrary|NegateRotator (Math|Rotator|MakeRotator 0.0 0.0 _trackrotation)) false false))))

(event OnComponentBeginOverlap(Box1)
  (params (OverlappedComponent :type Primitive%20Component%20Object%20Reference) (OtherActor :type Actor%20Object%20Reference) (OtherComp :type Primitive%20Component%20Object%20Reference) (OtherBodyIndex :type Integer) (bFromSweep :type Boolean) (SweepResult :type Hit%20Result%20Structure%20%28by%20ref%29))
  (Utilities|FlowControl|Sequence
    (:then_0
      (bind _newtrack_0 (Timeline|WheelSpeedControl Play)
        (:Update
          (Rendering|Material|SetScalarParameterValue (Variables|Default|GetWheelMaterial) "Time" (* _newtrack_0 (Variables|Default|GetSpeed)) :!class /Script/Engine.MaterialInstanceDynamic)
          (Rendering|Material|SetScalarParameterValue (Variables|Default|GetSmallWheelMaterial) "Time" (* (* _newtrack_0 (Variables|Default|GetSpeed)) 1.6) :!class /Script/Engine.MaterialInstanceDynamic)
          (Rendering|Material|SetScalarParameterValue (Variables|Default|GetRopeMaterial) "Time" (* (* _newtrack_0 (Variables|Default|GetSpeed)) -0.25) :!class /Script/Engine.MaterialInstanceDynamic))))
    (:then_1
      (Utilities|FlowControl|Delay 1.0)
      (bind _trackrotation (Timeline|Timeline Reverse)
        (:Update
          (Transformation|SetRelativeRotation (Variables|Default|GetSM_NavetteDoor_01) (Math|Rotator|MakeRotator 0.0 0.0 _trackrotation) false false)
          (Utilities|FlowControl|Delay 0.2)
          (Transformation|SetRelativeRotation (Variables|Default|GetSM_NavetteDoor_02) (Class|KismetMathLibrary|NegateRotator (Math|Rotator|MakeRotator 0.0 0.0 _trackrotation)) false false))))))

(event OnComponentBeginOverlap(w)
  (params (OverlappedComponent :type Primitive%20Component%20Object%20Reference) (OtherActor :type Actor%20Object%20Reference) (OtherComp :type Primitive%20Component%20Object%20Reference) (OtherBodyIndex :type Integer) (bFromSweep :type Boolean) (SweepResult :type Hit%20Result%20Structure%20%28by%20ref%29))
  (Utilities|FlowControl|Sequence
    (:then_0
      (bind _newtrack_0 (Timeline|WheelSpeedControl Reverse)
        (:Update
          (Rendering|Material|SetScalarParameterValue (Variables|Default|GetWheelMaterial) "Time" (* _newtrack_0 (Variables|Default|GetSpeed)) :!class /Script/Engine.MaterialInstanceDynamic)
          (Rendering|Material|SetScalarParameterValue (Variables|Default|GetSmallWheelMaterial) "Time" (* (* _newtrack_0 (Variables|Default|GetSpeed)) 1.6) :!class /Script/Engine.MaterialInstanceDynamic)
          (Rendering|Material|SetScalarParameterValue (Variables|Default|GetRopeMaterial) "Time" (* (* _newtrack_0 (Variables|Default|GetSpeed)) -0.25) :!class /Script/Engine.MaterialInstanceDynamic))))
    (:then_1
      (Utilities|FlowControl|Delay 1.0)
      (bind _trackrotation (Timeline|Timeline_0 Play)
        (:Update
          (Transformation|SetRelativeRotation (Variables|Default|GetSM_NavetteDoor_03) (Math|Rotator|MakeRotator 0.0 0.0 (* _trackrotation -1.0)) false false))
        (:Finished
          (Timeline|WheelSpeedControl Stop))))))

(event EventBeginPlay
  (Rendering|Material|SetScalarParameterValue (Variables|Default|GetWheelMaterial) "Speed" 0.0 :!class /Script/Engine.MaterialInstanceDynamic))

(fn ConstructionScript
  (bind _returnvalue (Rendering|Material|CreateDynamicMaterialInstance "/Game/AssetsMyrmidon/Art/Materials/Maquette/Navette/MI_RoueNavette.MI_RoueNavette" "None" "None" :!class /Script/Engine.KismetMaterialLibrary))
  (bind _output_get (Variables|Default|SetSmallWheelMaterial _returnvalue))
  (Rendering|Material|SetMaterial (Variables|Default|GetSM_NavetteCog_02_low) 0 _output_get)
  (bind _returnvalue_2 (Rendering|Material|CreateDynamicMaterialInstance "/Game/AssetsMyrmidon/Art/Materials/Maquette/Navette/MI_RoueNavette.MI_RoueNavette" "None" "None" :!class /Script/Engine.KismetMaterialLibrary))
  (Variables|Default|SetWheelMaterial _returnvalue_2)
  (Rendering|Material|SetMaterial (Variables|Default|GetSM_NavetteCyl_04) 0 _returnvalue_2)
  (bind _returnvalue_3 (Rendering|Material|CreateDynamicMaterialInstance "/Game/AssetsMyrmidon/Art/Materials/Maquette/Navette/M_NavetteRope.M_NavetteRope" "None" "None" :!class /Script/Engine.KismetMaterialLibrary))
  (bind _output_get_2 (Variables|Default|SetRopeMaterial _returnvalue_3))
  (Rendering|Material|SetMaterial (Variables|Default|GetSM_Rope_02) 0 _output_get_2)
  (Rendering|Material|SetScalarParameterValue (Variables|Default|GetWheelMaterial) "Time" 0.0 :!class /Script/Engine.MaterialInstanceDynamic))