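; BP_AnimNotify is an animation notify that plays footstep sounds for the local player's Pantin character.
; On notify it gets the local player controller and proceeds only if that player is a Pantin that is alive and not jumping.
; It plays the Pantin's current footstep sound at its location, scaled by the game instance's SFX volume.
; The notifying mesh is ignored, so the sound always follows the local player's Pantin.
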(fn ReceivedNotify
  (params (MeshComp :type Skeletal%20Mesh%20Component%20Object%20Reference) (Animation :type Anim%20Sequence%20Base%20Object%20Reference) (EventReference :type Anim%20Notify%20Event%20Reference%20Structure%20%28by%20ref%29))
  (bind (_playercontroller _castsuccesful) (CallFunction|GetBPLocalPlayerController))
  (bind _bp_pantin (Variables|/Game/AssetsMyrmidon/Blueprints/GameMode/BP_PlayerController.BP_PlayerController_C|GetBP_Pantin _playercontroller))
  (if _castsuccesful
    (if (Variables|/Game/AssetsMyrmidon/Blueprints/GameMode/BP_PlayerController.BP_PlayerController_C|GetisPantin _playercontroller)
      (if (and (not (Variables|/Game/AssetsMyrmidon/Blueprints/Character/BP_Pantin.BP_Pantin_C|GetIsJumping _bp_pantin)) (Variables|/Script/MyrmidonProto.PantinCharacter|GetIsAlive _bp_pantin))
        (Audio|PlaySoundatLocation (Variables|/Game/AssetsMyrmidon/Blueprints/Character/BP_Pantin.BP_Pantin_C|GetCurrentFootStepSound _bp_pantin) (Transformation|GetActorLocation _bp_pantin) "0, 0, 0" (Default|GetSfxVolume (.GameInstance (CallFunction|GetBPGameInstance))) 1.0 0.0 0 0 0 0)
        (return false)))))