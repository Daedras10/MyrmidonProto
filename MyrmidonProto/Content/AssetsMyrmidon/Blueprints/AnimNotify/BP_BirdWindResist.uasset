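; BP_BirdWindResist is an animation notify that plays the bird's wind-resistance sound.
; It fires only when the local player controller has IsPantin set and the mesh owner is a BP_Bird with ProduceSound enabled.
; The sound plays at the mesh's world location, with volume taken from the game instance's SFX setting.
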(fn ReceivedNotify
  (params (MeshComp :type Skeletal%20Mesh%20Component%20Object%20Reference) (Animation :type Anim%20Sequence%20Base%20Object%20Reference) (EventReference :type Anim%20Notify%20Event%20Reference%20Structure%20%28by%20ref%29))
  (bind (_playercontroller _castsuccesful) (CallFunction|GetBPLocalPlayerController))
  (if _castsuccesful
    (if (Variables|/Game/AssetsMyrmidon/Blueprints/GameMode/BP_PlayerController.BP_PlayerController_C|GetisPantin _playercontroller)
      (bind _asbp_bird (Utilities|Casting|CastToBP_Bird (Components|GetOwner MeshComp)))
      (if (Variables|/Game/AssetsMyrmidon/Blueprints/LDElements/BP_Bird.BP_Bird_C|GetProduceSound _asbp_bird)
        (Audio|PlaySoundatLocation "/Game/AssetsMyrmidon/Sons/Bird/BirdResistWind.BirdResistWind" (Transformation|GetWorldLocation MeshComp) "0, 0, 0" (Default|GetSfxVolume (.GameInstance (CallFunction|GetBPGameInstance))) 1.0 0.0 0 0 0 0)
        (return false)))))