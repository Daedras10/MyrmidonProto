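; BP_CameraRail is a spline camera rail that supplies a camera position and rotation from the "Pantin" target's transform.
; It projects the target's location plus an offset onto the spline to get the camera position.
; Rotation and offset are interpolated between distance-keyed curve points, with the offset feeding back into the projection, and an optional look-at overrides rotation.
; The construction script draws an arrow at each point to preview its rotation.
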(fn ConstructionScript
  (bind _arrows (Variables|Default|GetArrows))
  (for _array_element _arrows
    (Components|DestroyComponent _array_element))
  (Utilities|Array|Clear _arrows)
  (for _array_element_2 (Variables|Default|GetCurvePoints)
    (AddComponent|AddArrowComponent false (Math|Transform|MakeTransform (Spline|GetLocationatDistanceAlongSpline (Variables|Default|GetSpline) (.DistanceAlongCurve (Utilities|Struct|BreakSTRUCT_CurvePoint _array_element_2)) "Local") (.Rotation (Utilities|Struct|BreakSTRUCT_CurvePoint _array_element_2))))))

(fn GetCameraPosandRot
  (params (Transform :type Transform) (PantinTransform :type Transform))
  (bind _spline (Variables|Default|GetSpline))
  (bind (_rotation _offset) (CallFunction|GetCurveInfoatAlpha (Class|SplineComponent|GetDistanceAlongSplineatLocation _spline (+ (.Location (Math|Transform|BreakTransform PantinTransform)) (Variables|Default|GetTargetOffset)) "World")))
  (Variables|Default|SetTargetOffset _offset)
  (return (Spline|GetLocationatDistanceAlongSpline _spline (Class|SplineComponent|GetDistanceAlongSplineatLocation _spline (+ (.Location (Math|Transform|BreakTransform PantinTransform)) (Variables|Default|GetTargetOffset)) "World") "World") (Math|Rotator|SelectRotator (Math|Rotator|FindLookatRotation (.Location (Math|Transform|BreakTransform Transform)) (.Location (Math|Transform|BreakTransform PantinTransform))) _rotation (Variables|Default|GetLookAtPlayer))))

(fn GetCurveInfoatAlpha
  (params (Alpha :type Float%20%28double-precision%29))
  (bind _curvepoints (Variables|Default|GetCurvePoints))
  (bind _index (Utilities|FlowControl|ForLoopwithBreak 1 (Utilities|Array|Length _curvepoints))
    (:LoopBody
      (if (<= Alpha (.DistanceAlongCurve (Utilities|Struct|BreakSTRUCT_CurvePoint (Utilities|Array|Get(acopy) _curvepoints _index))))
        (return (Math|Rotator|Lerp(Rotator) (.Rotation (Utilities|Struct|BreakSTRUCT_CurvePoint (Utilities|Array|Get(acopy) _curvepoints (- _index 1)))) (.Rotation (Utilities|Struct|BreakSTRUCT_CurvePoint (Utilities|Array|Get(acopy) _curvepoints _index))) (/ (- Alpha (.DistanceAlongCurve (Utilities|Struct|BreakSTRUCT_CurvePoint (Utilities|Array|Get(acopy) _curvepoints (- _index 1))))) (- (.DistanceAlongCurve (Utilities|Struct|BreakSTRUCT_CurvePoint (Utilities|Array|Get(acopy) _curvepoints _index))) (.DistanceAlongCurve (Utilities|Struct|BreakSTRUCT_CurvePoint (Utilities|Array|Get(acopy) _curvepoints (- _index 1)))))) true) (Math|Vector|Lerp(Vector) (.Offset (Utilities|Struct|BreakSTRUCT_CurvePoint (Utilities|Array|Get(acopy) _curvepoints (- _index 1)))) (.Offset (Utilities|Struct|BreakSTRUCT_CurvePoint (Utilities|Array|Get(acopy) _curvepoints _index))) (/ (- Alpha (.DistanceAlongCurve (Utilities|Struct|BreakSTRUCT_CurvePoint (Utilities|Array|Get(acopy) _curvepoints (- _index 1))))) (- (.DistanceAlongCurve (Utilities|Struct|BreakSTRUCT_CurvePoint (Utilities|Array|Get(acopy) _curvepoints _index))) (.DistanceAlongCurve (Utilities|Struct|BreakSTRUCT_CurvePoint (Utilities|Array|Get(acopy) _curvepoints (- _index 1))))))))))
    (:Completed
      (return "0, 0, 0" "0, 0, 0"))))