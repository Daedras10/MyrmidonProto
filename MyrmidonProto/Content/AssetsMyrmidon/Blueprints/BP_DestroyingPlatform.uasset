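; Platform that fades out after BP_Pantin steps into its trigger box, then returns after a respawn delay.
; A Tick-driven timer lowers dynamic material opacity on the active view's mesh (PantinCube or AnimSphere), then disables both meshes' collision.
; Only PantinCube's visibility toggles, and respawn resets only its opacity.
; The construction script creates both material instances and sizes meshes and trigger from PlatformScale.
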(event OnComponentBeginOverlap(Box)
  (params (OverlappedComponent :type Primitive%20Component%20Object%20Reference) (OtherActor :type Actor%20Object%20Reference) (OtherComp :type Primitive%20Component%20Object%20Reference) (OtherBodyIndex :type Integer) (bFromSweep :type Boolean) (SweepResult :type Hit%20Result%20Structure%20%28by%20ref%29))
  ;[1 1 1] Overlap
  (Utilities|Casting|CastToBP_Pantin OtherActor)
  (if (Math|Boolean|NORBoolean (Variables|Default|GetShouldDisapear) (Variables|Default|GetShouldRespawn))
    (Variables|Default|SetTimer (Variables|Default|GetDisapearDeleay))
    (Variables|Default|SetShouldDisapear true)))

(event EventTick
  (params (DeltaSeconds :type Float%20%28single-precision%29))
  ;[1 1 1] EveentTick
  (if (or (Variables|Default|GetShouldRespawn) (Variables|Default|GetShouldDisapear))
    (Variables|Default|SetTimer (- (Variables|Default|GetTimer) DeltaSeconds))
    (if (Variables|Default|GetShouldDisapear)
      (if (<= (Variables|Default|GetTimer) 0.0)
        (Rendering|SetVisibility (Variables|Default|GetPantinCube) false false)
        (Variables|Default|SetShouldRespawn true)
        (Variables|Default|SetShouldDisapear false)
        (Variables|Default|SetTimer (Variables|Default|GetRespawnDelay))
        (Collision|SetCollisionEnabled (Variables|Default|GetPantinCube) "NoCollision")
        (Collision|SetCollisionEnabled (Variables|Default|GetAnimSphere) "NoCollision")
        (elif (Variables|Default|GetIsPantinView)
          (Rendering|Material|SetScalarParameterValue (Variables|Default|GetDisapearMatPantin) "Opacity" (/ (Variables|Default|GetTimer) (Variables|Default|GetDisapearDeleay)) :!class /Script/Engine.MaterialInstanceDynamic)
          (else
            (Rendering|Material|SetScalarParameterValue (Variables|Default|GetDisapearMatAnim) "Opacity" (/ (Variables|Default|GetTimer) (Variables|Default|GetDisapearDeleay)) :!class /Script/Engine.MaterialInstanceDynamic))))
      (elif (<= (Variables|Default|GetTimer) 0.0)
        (Rendering|SetVisibility (Variables|Default|GetPantinCube) true false)
        (Variables|Default|SetShouldRespawn false)
        (Collision|SetCollisionEnabled (Variables|Default|GetPantinCube) "QueryAndPhysics")
        (Collision|SetCollisionEnabled (Variables|Default|GetAnimSphere) "QueryAndPhysics")
        (if true
          (Rendering|Material|SetScalarParameterValue (Variables|Default|GetDisapearMatPantin) "Opacity" 1.0 :!class /Script/Engine.MaterialInstanceDynamic)
          (else
            (Rendering|Material|SetScalarParameterValue (Variables|Default|GetDisapearMatAnim) "Opacity" 1.0 :!class /Script/Engine.MaterialInstanceDynamic)))))))

(event EventStartHover
  ;[1 1 1] Hovers (does nothing but override base)
)

(event EventEndHover
  ;[1 1 1] Hovers (does nothing but override base)
)

(fn ConstructionScript
  (bind _platformscale (Variables|Default|GetPlatformScale))
  (bind _returnvalue (* _platformscale 25.0))
  (bind (_x _y) (Math|Vector|BreakVector _returnvalue))
  (|CallParentFunction)
  (bind _returnvalue_2 (Rendering|Material|CreateDynamicMaterialInstance (Variables|Default|GetPantinCube) 0 "/Game/AssetsMyrmidon/Art/Materials/M_DisapearingPlatform.M_DisapearingPlatform" "None" :!class /Script/Engine.PrimitiveComponent))
  (Variables|Default|SetDisapearMatPantin _returnvalue_2)
  (bind _returnvalue_3 (Rendering|Material|CreateDynamicMaterialInstance (Variables|Default|GetAnimSphere) 0 "/Game/AssetsMyrmidon/Art/Materials/M_DisapearingPlatform.M_DisapearingPlatform" "None" :!class /Script/Engine.PrimitiveComponent))
  (Variables|Default|SetDisapearMatAnim _returnvalue_3)
  (Transformation|SetWorldScale3D (Variables|Default|GetAnimSphere) _platformscale)
  (Transformation|SetWorldScale3D (Variables|Default|GetPantinCube) _platformscale)
  (Components|Box|SetBoxExtent (Variables|Default|GetBox) (Math|Vector|MakeVector _x _y 3e+01) true))