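; BP_Merchant is a configurable merchant character with an optional fisherman variant.
; Its construction script selects the body, bag and hat meshes, toggles fishing rod visibility, and maps boolean variations to paired materials, offsetting later slots for merchant model 1.
; At BeginPlay it simulates physics on hat bodies below the Root bone and passes the fisherman flag to ABP_Merchant.
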(event EventBeginPlay
  (Class|SkeletalMeshComponent|SetAllBodiesBelowSimulatePhysics (Variables|Default|GetHat) (Utilities|Name|MakeLiteralName "Root") true false)
  (bind _asabp_merchant (Utilities|Casting|CastToABP_Merchant (Components|SkeletalMesh|GetAnimInstance (Variables|Default|GetSK_Marchand))))
  (Variables|/Game/AssetsMyrmidon/Art/Characters/Merchant/ABP_Merchant.ABP_Merchant_C|SetisFisherman _asabp_merchant (Variables|Customize|GetFisherman)))

(fn ConstructionScript
  (Rendering|SetVisibility (Variables|Default|GetSK_FishingRod) (Variables|Customize|GetFisherman) false)
  (Components|SkeletalMesh|SetSkeletalMeshAsset (Variables|Default|GetSK_Marchand) (Utilities|Array|Get(acopy) (Variables|Arrays|GetMerchantModels) (Variables|Customize|GetMerchantModel)))
  (Components|StaticMesh|SetStaticMesh (Variables|Default|GetBag) (Utilities|Array|Get(acopy) (Variables|Arrays|GetBags) (Variables|Customize|GetCurrentBag)))
  (Components|SkeletalMesh|SetSkeletalMeshAsset (Variables|Default|GetHat) (Utilities|Array|Get(acopy) (Variables|Arrays|GetHats) (Variables|Customize|GetCurrentHat)))
  (for (_array_element _array_index) (Variables|Customize|GetMaterialVariations)
    (Rendering|Material|SetMaterial (Variables|Default|GetSK_Marchand) (+ _array_index 1) (Utilities|Array|Get(acopy) (Variables|Arrays|GetMaterials) (+ (Math|Integer|SelectInt 1 0 _array_element) (+ (* _array_index 2) (Math|Integer|SelectInt 2 0 (and (> _array_index 1) (== (Variables|Customize|GetMerchantModel) 1)))))))))