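; Spline actor that builds a mesh along its editable path in the construction script, with no active runtime logic.
; Each segment gets a collidable spline mesh matching its points and tangents, with configurable forward axis and optional material override.
; Optional cap meshes spawn inside the segment loop, so they duplicate per segment.
; EndMesh sits at the first point and StartMesh at the last, both using the first point's rotation.
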(event EventBeginPlay)

(event Collision|EventActorBeginOverlap
  (params (OtherActor :type Actor%20Object%20Reference)))

(event EventTick
  (params (DeltaSeconds :type Float%20%28single-precision%29)))

(fn ConstructionScript
  (bind _spline (Variables|Default|GetSpline))
  (bind _spline_2 (Variables|Default|GetSpline))
  (for _index (range 0 (- (Spline|GetNumberOfSplinePoints _spline) 2))
    (bind _returnvalue (AddComponent|AddSplineMeshComponent false))
    (Components|StaticMesh|SetStaticMesh _returnvalue (Variables|Default|GetSplineMesh))
    (SplineMesh|SetForwardAxis _returnvalue (Variables|Default|GetMeshForwardAxis) true)
    (Transformation|AttachComponentToComponent _returnvalue _spline "None" "KeepRelative" "KeepRelative" "KeepRelative" true)
    (SplineMesh|SetStartandEnd _returnvalue (Spline|GetLocationatSplinePoint _spline _index "Local") (Spline|GetTangentatSplinePoint _spline _index "Local") (Spline|GetLocationatSplinePoint _spline (+ _index 1) "Local") (Spline|GetTangentatSplinePoint _spline (+ _index 1) "Local") true :!class /Script/Engine.SplineMeshComponent)
    (Collision|SetCollisionEnabled _returnvalue "QueryAndPhysics")
    (if (Variables|Material|GetMaterialOverride)
      (Rendering|Material|SetMaterial _returnvalue 0 (Variables|Material|GetMaterial)))
    (if (Variables|Default|GetUseEndMesh)
      (bind _returnvalue_2 (AddComponent|AddStaticMeshComponent false (Math|Transform|MakeTransform (Spline|GetLocationatSplinePoint _spline_2 0 "Local") (Spline|GetRotationatSplinePoint _spline_2 0 "Local"))))
      (Components|StaticMesh|SetStaticMesh _returnvalue_2 (Variables|Default|GetEndMesh))
      (Collision|SetCollisionEnabled _returnvalue_2 "QueryAndPhysics"))
    (if (Variables|Default|GetUseStartMesh)
      (bind _returnvalue_3 (AddComponent|AddStaticMeshComponent false (Math|Transform|MakeTransform (Spline|GetLocationatSplinePoint _spline_2 (- (Spline|GetNumberOfSplinePoints _spline_2) 1) "Local") (Spline|GetRotationatSplinePoint _spline_2 0 "Local"))))
      (Components|StaticMesh|SetStaticMesh _returnvalue_3 (Variables|Default|GetStartMesh))
      (Collision|SetCollisionEnabled _returnvalue_3 "QueryAndPhysics"))))