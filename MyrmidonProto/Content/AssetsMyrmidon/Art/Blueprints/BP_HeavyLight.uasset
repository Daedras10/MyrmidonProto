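; BP_HeavyLight is a configurable heavy light fixture with switchable on and off states.
; The construction script creates a dynamic emissive material and applies color, intensity, attenuation radius and an open angle that drives both the rect light's barn doors and four mesh panels.
; TurnOn restores that material and ramps light intensity and emissive strength through a timeline.
; TurnOff swaps to an alternate material and zeroes the light immediately.
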(event Custom|TurnOff
  (Rendering|Material|SetMaterial (Variables|Default|GetSM_HeavyLight_01) 1 "/Game/AssetsMyrmidon/Art/Materials/T_AnimateurRoom/Props/MI_Lights02.MI_Lights02")
  (Rendering|Components|Light|SetIntensity (Variables|Default|GetRectLight) 0.0))

(event Custom|TurnOn
  (bind _material (Variables|Default|GetMaterial))
  (Rendering|Material|SetMaterial (Variables|Default|GetSM_HeavyLight_01) 1 _material)
  (bind _intensity (Timeline|Timeline Play)
    (:Update
      (Rendering|Components|Light|SetIntensity (Variables|Default|GetRectLight) (* _intensity (* (Variables|Default|GetLightIntensity) 1e+04)))
      (Audio|Parameter|SetFloatParameter _material "EmissiveStrength" _intensity :!class /Script/AudioExtensions.AudioParameterControllerInterface))))

(fn ConstructionScript
  (bind _openangle (Variables|Default|GetOpenAngle))
  (bind _rectlight (Variables|Default|GetRectLight))
  (bind _returnvalue (Rendering|Material|CreateDynamicMaterialInstance "/Game/AssetsMyrmidon/Art/Materials/T_AnimateurRoom/Props/MI_Lights.MI_Lights" "None" "None" :!class /Script/Engine.KismetMaterialLibrary))
  (Variables|Default|SetMaterial _returnvalue)
  (Rendering|Material|SetMaterial (Variables|Default|GetSM_HeavyLight_01) 1 _returnvalue)
  (Rendering|Material|SetVectorParameterValue _returnvalue "EmissiveTint" (Variables|Default|GetLightColor) :!class /Script/Engine.MaterialInstanceDynamic)
  (Rendering|Components|Light|SetLightColor _rectlight (Variables|Default|GetLightColor) true)
  (Rendering|Lighting|SetAttenuationRadius _rectlight (Variables|Default|GetAttenuationRadius))
  (Rendering|Components|Light|SetIntensity _rectlight (* (Variables|Default|GetLightIntensity) 1e+04))
  (Class|RectLightComponent|SetBarnDoorAngle _rectlight _openangle)
  (for _array_element (Utilities|Array|MakeArray (Variables|Default|GetSM_HeavyLightPanel_02) (Variables|Default|GetSM_HeavyLightPanel_03) (Variables|Default|GetSM_HeavyLightPanel_04) (Variables|Default|GetSM_HeavyLightPanel_01))
    (Transformation|AddRelativeRotation _array_element (Math|Rotator|MakeRotator 0.0 _openangle 0.0) false false)))