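; Spline actor that tiles a chosen static mesh along an editable spline as deformed, collidable spline mesh segments.
; The construction script takes the mesh's largest bounding-box dimension as segment length and fits as many whole segments as the spline length allows, leaving any remainder uncovered.
; Each segment bends using local spline positions and unscaled tangents at its ends, along a configurable forward axis.
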(event EventBeginPlay)

(event Collision|EventActorBeginOverlap
  (params (OtherActor :type Actor%20Object%20Reference)))

(event EventTick
  (params (DeltaSeconds :type Float%20%28single-precision%29)))

(fn ConstructionScript
  (bind _splinemesh (Variables|Default|GetSplineMesh))
  (bind _spline (Variables|Default|GetSpline))
  (bind _returnvalue (StaticMesh|GetBoundingBox _splinemesh))
  (bind (_min _max) (Utilities|Struct|BreakBox _returnvalue))
  (bind _returnvalue_2 (- _max _min))
  (bind (_x _y _z) (Math|Vector|BreakVector _returnvalue_2))
  (bind _returnvalue_3 (Math|Float|Max(Float) _x _y))
  (bind _returnvalue_4 (Math|Float|Max(Float) _returnvalue_3 _z))
  (for _index (range 0 (- (Math|Float|Floor (/ (Spline|GetSplineLength (Variables|Default|GetSpline)) _returnvalue_4)) 1))
    (bind _returnvalue_5 (AddComponent|AddSplineMeshComponent false))
    (Components|StaticMesh|SetStaticMesh _returnvalue_5 (Variables|Default|GetSplineMesh))
    (SplineMesh|SetForwardAxis _returnvalue_5 (Variables|Default|GetMeshForwardAxis) true)
    (Transformation|AttachComponentToComponent _returnvalue_5 _spline "None" "KeepRelative" "KeepRelative" "KeepRelative" true)
    (SplineMesh|SetStartandEnd _returnvalue_5 (Spline|GetLocationatDistanceAlongSpline _spline (* _index _returnvalue_4) "Local") (Spline|GetTangentatDistanceAlongSpline _spline (* _index _returnvalue_4) "Local") (Spline|GetLocationatDistanceAlongSpline _spline (* (+ _index 1) _returnvalue_4) "Local") (Spline|GetTangentatDistanceAlongSpline _spline (* (+ _index 1) _returnvalue_4) "Local") true :!class /Script/Engine.SplineMeshComponent)
    (Collision|SetCollisionEnabled _returnvalue_5 "QueryAndPhysics")))