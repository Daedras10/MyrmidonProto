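; BP_FishFlock04 is a VFX Blueprint that displays a school of fish through its NSFishSchool04 effect component, which appears to be a Niagara system.
; Its construction script pushes the Blueprint's variables for fish count, size, speed and speed range into the effect's matching parameters, with MaxRadius feeding MaxDistance.
; The graph holds no runtime logic, so any flocking motion comes from the effect itself.
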(fn ConstructionScript
  (bind _ns_fishschool04 (Variables|Default|GetNS_FishSchool04))
  (Class|NiagaraComponent|SetVariableInt _ns_fishschool04 "FishCount" (Variables|Default|GetFishCount))
  (Niagara|SetNiagaraVariable(Float) _ns_fishschool04 "MaxDistance" (Variables|Default|GetMaxRadius))
  (Niagara|SetNiagaraVariable(Float) _ns_fishschool04 "FishSize" (Variables|Default|GetFishSize))
  (Niagara|SetNiagaraVariable(Float) _ns_fishschool04 "Speed" (Variables|Default|GetSpeed))
  (Class|NiagaraComponent|SetVariableVec2 _ns_fishschool04 "SpeedRange" (Variables|Default|GetSpeedRange)))