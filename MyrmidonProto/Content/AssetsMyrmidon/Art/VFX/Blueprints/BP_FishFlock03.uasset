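; BP_FishFlock03 is a VFX Blueprint that displays a school of fish through the NSFishSchool03 effect component.
; Its Construction Script copies the Blueprint's fish count, stray amount, fish size, travel speed and speed range into same-named effect parameters.
; The Blueprint acts as a configuration wrapper, with no runtime logic shown and the flocking behavior left to the effect itself.
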(fn ConstructionScript
  (bind _ns_fishschool03 (Variables|Default|GetNS_FishSchool03))
  (Class|NiagaraComponent|SetVariableInt _ns_fishschool03 "FishCount" (Variables|Default|GetFishCount))
  (Niagara|SetNiagaraVariable(Float) _ns_fishschool03 "StrayAmount" (Variables|Default|GetStrayAmount))
  (Niagara|SetNiagaraVariable(Float) _ns_fishschool03 "FishSize" (Variables|Default|GetFishSize))
  (Niagara|SetNiagaraVariable(Float) _ns_fishschool03 "TravelSpeed" (Variables|Default|GetTravelSpeed))
  (Class|NiagaraComponent|SetVariableVec2 _ns_fishschool03 "SpeedRange" (Variables|Default|GetSpeedRange)))