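; Lamp post VFX Blueprint that plays a swinging-pole animation with placement and electrical effects.
; StartAnimation reveals and plays the animated pole with a dynamic material and spawns a bar-placement Niagara system at a socket.
; After short delays, an electrical burst receives arc endpoints from pole sockets, and a timeline drives the material's emissive strength.
; ResetState hides the pole, destroys the burst and clears the Running flag that gates delayed steps.
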(event Custom|SetupVariables
  (params (NS :type Niagara%20Component%20Object%20Reference))
  (Niagara|SetNiagaraVariable(Vector3) NS "ArcStartPos" (Transformation|GetSocketLocation (Variables|Default|GetSM_SwingingPole) "Arc1Start"))
  (Niagara|SetNiagaraVariable(Vector3) NS "ArcEndPos" (Transformation|GetSocketLocation (Variables|Default|GetSM_SwingingPole) "Arc1End"))
  (Niagara|SetNiagaraVariable(Vector3) NS "Arc2StartPos" (Transformation|GetSocketLocation (Variables|Default|GetSM_SwingingPole) "Arc2Start"))
  (Niagara|SetNiagaraVariable(Vector3) NS "Arc2EndPos" (Transformation|GetSocketLocation (Variables|Default|GetSM_SwingingPole) "Arc2End")))

(event Custom|ResetState
  (bind _ns (Variables|Default|GetNS))
  (Variables|Default|SetRunning false)
  (Rendering|SetVisibility (Variables|Default|GetSM_AnimatedSwingingPole) false false)
  (Utilities|IsValid _ns
    (:Is%20Valid
      (Components|DestroyComponent _ns))))

(event Custom|StartAnimation
  (bind _sm_animatedswingingpole (Variables|Default|GetSM_AnimatedSwingingPole))
  (Variables|Default|SetRunning true)
  (Rendering|SetVisibility _sm_animatedswingingpole true false)
  (Components|Timeline|PlayfromStart _sm_animatedswingingpole)
  (Variables|/Script/GeometryCache.GeometryCacheComponent|SetbRunning _sm_animatedswingingpole true)
  (bind _returnvalue (Rendering|Material|CreateDynamicMaterialInstance "/Game/AssetsMyrmidon/Art/Materials/Maquette/Props/M_Swing.M_Swing" "None" "None" :!class /Script/Engine.KismetMaterialLibrary))
  (Rendering|Material|SetMaterial (Variables|Default|GetSM_AnimatedSwingingPole) 0 _returnvalue)
  (Niagara|SpawnSystematLocation "/Game/AssetsMyrmidon/Art/VFX/NiagaraSystems/NS_PlaceBar.NS_PlaceBar" (Transformation|GetSocketLocation (Variables|Default|GetSM_SwingingPole) "StartPos"))
  (Utilities|FlowControl|Delay 0.2)
  (if (Variables|Default|GetRunning)
    (bind _returnvalue_2 (Niagara|SpawnSystematLocation "/Game/AssetsMyrmidon/Art/VFX/NiagaraSystems/NS_ElectricalBurst.NS_ElectricalBurst" "0, 0, 0"))
    (Variables|Default|SetNS _returnvalue_2)
    (Utilities|FlowControl|Sequence
      (:then_0
        (CallFunction|SetupVariables _returnvalue_2)
        (Utilities|FlowControl|Delay 0.5)
        (if (Variables|Default|GetRunning)
          (bind _newtrack_0 (Timeline|Timeline PlayFromStart)
            (:Update
              (Rendering|Material|SetScalarParameterValue _returnvalue "EmissiveStrength" _newtrack_0 :!class /Script/Engine.MaterialInstanceDynamic)))))
      (:then_1
        (Utilities|FlowControl|Delay 0.2)
        (Variables|/Script/GeometryCache.GeometryCacheComponent|SetbRunning (Variables|Default|GetSM_AnimatedSwingingPole) false)))))

(fn ConstructionScript)