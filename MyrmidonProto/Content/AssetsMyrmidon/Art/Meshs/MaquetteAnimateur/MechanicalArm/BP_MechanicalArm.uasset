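; BP_MechanicalArm is an actor whose skeletal mechanical arm tracks a followed actor or a configured target.
; Every tick, it turns the mesh in yaw only toward either ObjectToFollow or the TargetPosition offset, chosen by UseTargetLocation.
; It also passes a relative PinTarget transform to ABP_MechanicalArm.
; When following a BP_Bird, PinTarget always uses the bird's ArmTarget socket, regardless of UseTargetLocation.
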(event Custom|UpdatePosition
  (bind _sk_mechanicalarm (Variables|Default|GetSK_MechanicalArm))
  (bind _sk_mechanicalarm_2 (Variables|Default|GetSK_MechanicalArm))
  (bind _targetposition (Variables|Default|GetTargetPosition))
  (bind _sk_mechanicalarm_3 (Variables|Default|GetSK_MechanicalArm))
  (bind _objecttofollow (Variables|Default|GetObjectToFollow))
  (bind (_location _rotation) (Math|Transform|BreakTransform _targetposition))
  (bind _returnvalue (Transformation|GetWorldRotation _sk_mechanicalarm_2))
  (bind _returnvalue_2 (Transformation|GetWorldTransform _sk_mechanicalarm_3))
  (bind (_roll _pitch) (Math|Rotator|BreakRotator _returnvalue))
  (Transformation|SetWorldRotation (Variables|Default|GetSK_MechanicalArm) (Math|Rotator|MakeRotator _roll _pitch (.Yaw (Math|Rotator|BreakRotator (.Rotation (Math|Transform|BreakTransform (Class|KismetAnimationLibrary|Lookat (Transformation|GetWorldTransform _sk_mechanicalarm) (Math|Vector|SelectVector (+ (.Location (Math|Transform|BreakTransform (Variables|Default|GetTargetPosition))) (Transformation|GetWorldLocation _sk_mechanicalarm)) (Transformation|GetActorLocation (Variables|Default|GetObjectToFollow)) (Variables|Default|GetUseTargetLocation)) "1.000000,0.000000,0.000000" false (Math|Vector|GetUpVector _sk_mechanicalarm) 0.0)))))) false false)
  (bind _asabp_mechanical_arm (Utilities|Casting|CastToABP_MechanicalArm (Components|SkeletalMesh|GetAnimInstance (Variables|Default|GetSK_MechanicalArm))))
  (Utilities|IsValid _objecttofollow
    (:Is%20Valid
      (bind _asbp_bird (Utilities|Casting|CastToBP_Bird _objecttofollow)
        (:then
          (Variables|/Game/AssetsMyrmidon/Art/Meshs/MaquetteAnimateur/MechanicalArm/ABP_MechanicalArm.ABP_MechanicalArm_C|SetPinTarget _asabp_mechanical_arm (Math|Transform|MakeRelativeTransform (Transformation|GetSocketTransform (Variables|/Game/AssetsMyrmidon/Blueprints/LDElements/BP_Bird.BP_Bird_C|GetBird _asbp_bird) "ArmTarget" "RTS_World") (Transformation|GetActorTransform))))
        (:CastFailed
          (Variables|/Game/AssetsMyrmidon/Art/Meshs/MaquetteAnimateur/MechanicalArm/ABP_MechanicalArm.ABP_MechanicalArm_C|SetPinTarget _asabp_mechanical_arm (Math|Transform|SelectTransform (Math|Transform|MakeRelativeTransform (Math|Transform|MakeTransform (+ _location (.Location (Math|Transform|BreakTransform (Transformation|GetWorldTransform (Variables|Default|GetSK_MechanicalArm))))) _rotation) _returnvalue_2) (Math|Transform|MakeRelativeTransform (Transformation|GetActorTransform _objecttofollow) _returnvalue_2) (Variables|Default|GetUseTargetLocation)) :!label _label))))
    (:Is%20Not%20Valid
      (goto _label))))

(event EventTick
  (params (DeltaSeconds :type Float%20%28single-precision%29))
  ;[1 0 0.03369] CHANGER L'EVENT TICK
  (CallFunction|UpdatePosition))

(fn ConstructionScript)